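; Game mode for the Carnage mod in Mordhau that populates the map with bots and registers the mod's weapons at BeginPlay.
; SpawnBots places a deathmatch-AI Mordhau character at each scene component taken from the first CarnageSpawn actor found.
; The hand-wired spawn list uses Scene2 twice and omits Scene5.
; It then appends the Carnage crossbow, longbow, recurve and rock staff to the MordhauSingleton's Equipment list.
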(event EventBeginPlay
  (bind _returnvalue (Class|MordhauUtilityLibrary|GetMordhauSingleton))
  (bind _equipment (Variables|/Script/Mordhau.MordhauSingleton|GetEquipment _returnvalue))
  (|CallParentFunction)
  (Utilities|FlowControl|Sequence
    (:then_0
      ;[1 1 1] Spawn Bots
      (bind _outactors (Actor|GetAllActorsOfClass "/Game/Mordhau/Mods/Carnage/CarnageSpawn.CarnageSpawn_C"))
      (Utilities|SpawnBots (Utilities|Array|MakeArray (Variables|/Game/Mordhau/Mods/Carnage/CarnageSpawn.CarnageSpawn_C|GetScene (Utilities|Array|Get(acopy) _outactors)) (Variables|/Game/Mordhau/Mods/Carnage/CarnageSpawn.CarnageSpawn_C|GetScene1 (Utilities|Array|Get(acopy) _outactors)) (Variables|/Game/Mordhau/Mods/Carnage/CarnageSpawn.CarnageSpawn_C|GetScene2 (Utilities|Array|Get(acopy) _outactors)) (Variables|/Game/Mordhau/Mods/Carnage/CarnageSpawn.CarnageSpawn_C|GetScene2 (Utilities|Array|Get(acopy) _outactors)) (Variables|/Game/Mordhau/Mods/Carnage/CarnageSpawn.CarnageSpawn_C|GetScene3 (Utilities|Array|Get(acopy) _outactors)) (Variables|/Game/Mordhau/Mods/Carnage/CarnageSpawn.CarnageSpawn_C|GetScene4 (Utilities|Array|Get(acopy) _outactors)) (Variables|/Game/Mordhau/Mods/Carnage/CarnageSpawn.CarnageSpawn_C|GetScene6 (Utilities|Array|Get(acopy) _outactors)) (Variables|/Game/Mordhau/Mods/Carnage/CarnageSpawn.CarnageSpawn_C|GetScene7 (Utilities|Array|Get(acopy) _outactors)) (Variables|/Game/Mordhau/Mods/Carnage/CarnageSpawn.CarnageSpawn_C|GetScene8 (Utilities|Array|Get(acopy) _outactors)) (Variables|/Game/Mordhau/Mods/Carnage/CarnageSpawn.CarnageSpawn_C|GetScene9 (Utilities|Array|Get(acopy) _outactors)) (Variables|/Game/Mordhau/Mods/Carnage/CarnageSpawn.CarnageSpawn_C|GetScene10 (Utilities|Array|Get(acopy) _outactors)) (Variables|/Game/Mordhau/Mods/Carnage/CarnageSpawn.CarnageSpawn_C|GetScene11 (Utilities|Array|Get(acopy) _outactors)) (Variables|/Game/Mordhau/Mods/Carnage/CarnageSpawn.CarnageSpawn_C|GetScene12 (Utilities|Array|Get(acopy) _outactors)) (Variables|/Game/Mordhau/Mods/Carnage/CarnageSpawn.CarnageSpawn_C|GetScene13 (Utilities|Array|Get(acopy) _outactors)) (Variables|/Game/Mordhau/Mods/Carnage/CarnageSpawn.CarnageSpawn_C|GetScene14 (Utilities|Array|Get(acopy) _outactors)))))
    (:then_1
      ;[1 1 1] Add Weapons
      (Utilities|Array|Add _equipment "/Game/Mordhau/Mods/Carnage/CarnageCrossbow.CarnageCrossbow_C")
      (Utilities|Array|Add _equipment "/Game/Mordhau/Mods/Carnage/CarnageLongbow.CarnageLongbow_C")
      (Utilities|Array|Add _equipment "/Game/Mordhau/Mods/Carnage/CarnageRecurve.CarnageRecurve_C")
      (Utilities|Array|Add _equipment "/Game/Mordhau/Mods/Carnage/CarnageRockStaff.CarnageRockStaff_C"))))

(fn ConstructionScript
  (|CallParentFunction))