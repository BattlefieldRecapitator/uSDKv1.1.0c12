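; Mordhau player character Blueprint handling death, ragdoll physics, dismemberment, ledge climbing and out-of-bounds warning text.
; Death picks an animation and conditionally ragdolls, with mass-scaled hit impulses offset by pre-death velocity; a Thudder component triggers body-fall sounds and blood decals.
; Climbing uses staged up, forward and down capsule traces, rejecting unsuitable surfaces before sending the target to the server.
; It also spawns the kick weapon and default or Pugilist fists.
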(event OnThud(Thudder)
  (bind _mesh (Variables|Character|GetMesh))
  (bind _thudder (Variables|Default|GetThudder))
  (bind _returnvalue (Transformation|GetSocketLocation _mesh "Neck"))
  (Audio|SpawnSoundAttached "/Game/Mordhau/Audio/Cues/Foley/SC_BodyFall.SC_BodyFall" (Variables|Character|GetMesh) "Hips" "0, 0, 0" "0, 0, 0" "SnapToTarget" true (Math|Float|MapRangeClamped (- (Variables|/Script/Mordhau.ThudderComponent|GetPreviousVelocity _thudder) (Variables|/Script/Mordhau.ThudderComponent|GetCurrentVelocity _thudder)) 75.0 3e+02 0.75 1.0) 1.0 0.0 0 0)
  (if (stale _returnvalue)
    (bind (_outhit _returnvalue_2) (Collision|LineTraceForObjects _returnvalue (+ _returnvalue "0, 0,-200.000000") (Utilities|Array|MakeArray "ObjectTypeQuery1") false 0 "None"))
    (if _returnvalue_2
      (Utilities|IsValid (Class|MordhauUtilityLibrary|SpawnBloodDecalatLocation 0 (Math|Vector|MakeVector 5e+01 1.5e+02 1.5e+02) (.ImpactPoint (Collision|BreakHitResult _outhit)) (Math|Rotator|MakeRotfromX (* (.ImpactNormal (Collision|BreakHitResult _outhit)) -1.0)) 9e+01)
        (:Is%20Valid
          (Rendering|Components|Decal|SetFadeOut (Class|MordhauUtilityLibrary|SpawnBloodDecalatLocation 0 (Math|Vector|MakeVector 5e+01 1.5e+02 1.5e+02) (.ImpactPoint (Collision|BreakHitResult _outhit)) (Math|Rotator|MakeRotfromX (* (.ImpactNormal (Collision|BreakHitResult _outhit)) -1.0)) 9e+01) 9e+01 0.25 false)
          (Class|MordhauUtilityLibrary|SetDecalFadeScreenSize (Class|MordhauUtilityLibrary|SpawnBloodDecalatLocation 0 (Math|Vector|MakeVector 5e+01 1.5e+02 1.5e+02) (.ImpactPoint (Collision|BreakHitResult _outhit)) (Math|Rotator|MakeRotfromX (* (.ImpactNormal (Collision|BreakHitResult _outhit)) -1.0)) 9e+01) 0.085)
          (Class|DecalComponent|SetSortOrder (Class|MordhauUtilityLibrary|SpawnBloodDecalatLocation 0 (Math|Vector|MakeVector 5e+01 1.5e+02 1.5e+02) (.ImpactPoint (Collision|BreakHitResult _outhit)) (Math|Rotator|MakeRotfromX (* (.ImpactNormal (Collision|BreakHitResult _outhit)) -1.0)) 9e+01) 1)
          (bind _returnvalue_3 (Rendering|Material|CreateDynamicMaterialInstance (Class|MordhauUtilityLibrary|SpawnBloodDecalatLocation 0 (Math|Vector|MakeVector 5e+01 1.5e+02 1.5e+02) (.ImpactPoint (Collision|BreakHitResult _outhit)) (Math|Rotator|MakeRotfromX (* (.ImpactNormal (Collision|BreakHitResult _outhit)) -1.0)) 9e+01) :!class /Script/Engine.DecalComponent))
          (Rendering|Material|SetScalarParameterValue _returnvalue_3 "Row" (Math|Conversions|ToFloat(Integer) (Math|Random|RandomIntegerinRange 0 3)) :!class /Script/Engine.MaterialInstanceDynamic)
          (Rendering|Material|SetScalarParameterValue _returnvalue_3 "Column" (Math|Conversions|ToFloat(Integer) (Math|Random|RandomIntegerinRange 0 3)) :!class /Script/Engine.MaterialInstanceDynamic)
          (Rendering|Material|SetScalarParameterValue _returnvalue_3 "StartTime" (Utilities|Time|GetGameTimeinSeconds) :!class /Script/Engine.MaterialInstanceDynamic)
          (Rendering|Material|SetScalarParameterValue _returnvalue_3 "FillDuration" 15.0 :!class /Script/Engine.MaterialInstanceDynamic))))))

(event Custom|ReplicatedTripWithKnockback
  (bind _returnvalue (Class|AdvancedCharacter|Trip))
  (if _returnvalue
    (Class|AdvancedCharacter|Knockback (* (Math|Conversions|ToVector(Vector2D) (Math|Vector2D|Normalize2D (Math|Conversions|ToVector2D(Vector) (Transformation|GetVelocity)))) 1.75e+03))))

(event Custom|ServerSetClimbLocation
  (params (NewParam :type Vector%20Net%20Quantize%20Structure))
  (Variables|Default|SetClimbTargetLocation NewParam))

(event EventOnPostProfileAssigned
  (bind _returnvalue (Math|Transform|MakeTransform "0, 0, 0"))
  (bind _equipmentinventorysize (Variables|Default|GetEquipmentInventorySize))
  (bind _returnvalue_2 (- _equipmentinventorysize 1))
  (|CallParentFunction)
  (Utilities|IsValid (Utilities|Array|Get(acopy) (Variables|Default|GetEquipment) 3)
    (:Is%20Not%20Valid
      (if (stale _returnvalue)
        (bind _returnvalue_3 (Game|SpawnActorfromClass "/Game/Mordhau/Blueprints/Equipment/Weapons/BP_PugilistFistWeapon.BP_PugilistFistWeapon_C" _returnvalue "AlwaysSpawn" 0 0))
        (Class|MordhauCharacter|PickUptoSlot _returnvalue_3 _returnvalue_2)
        (else
          (bind _returnvalue_4 (Game|SpawnActorfromClass "/Game/Mordhau/Blueprints/Equipment/Weapons/BP_FistWeapon.BP_FistWeapon_C" _returnvalue "AlwaysSpawn" 0 0))
          (Class|MordhauCharacter|PickUptoSlot _returnvalue_4 _returnvalue_2))))))

(event EventApplyRagdollForce
  (params (Angle :type Float%20%28single-precision%29) (Type :type EMordhauDamageType%20Enum :default "Generic") (SubType :type Byte :default 0) (bone :type Name%20%28by%20ref%29 :default "None") (Point :type Vector%20%28by%20ref%29 :default "0, 0, 0") (Source :type Actor%20Object%20Reference) (Agent :type Actor%20Object%20Reference))
  (bind _self self)
  (bind _deathsyncedrandom (Variables|Default|GetDeathSyncedRandom))
  (bind _mesh (Variables|Character|GetMesh))
  (bind _movecompvelocitybeforedeath (Variables|Default|GetMoveCompVelocityBeforeDeath))
  (bind (_x _y _z) (Math|Vector|BreakVector _movecompvelocitybeforedeath))
  (bind _returnvalue (Class|SkinnedMeshComponent|GetParentBone _mesh bone))
  (bind _force (CallFunction|ComputeRagdollForce Agent Type SubType _deathsyncedrandom _self _self))
  (bind _returnvalue_2 (Math|Float|Clamp(Float) _z -5e+02 0.0))
  (bind _returnvalue_3 (Math|Vector|VectorLength _force))
  (bind _returnvalue_4 (Math|Vector|MakeVector _x _y _returnvalue_2))
  (bind _returnvalue_5 (* _returnvalue_4 15.0))
  (bind _returnvalue_6 (Math|Vector|DotProduct _returnvalue_4 _force))
  (bind _returnvalue_7 (Math|Vector|ProjectVectorontoVector _returnvalue_5 _force))
  (bind _returnvalue_8 (Class|KismetMathLibrary|DegAcos _returnvalue_6))
  (bind _returnvalue_9 (< _returnvalue_8 9e+01))
  (bind _returnvalue_10 (Math|Conversions|ToFloat(Boolean) _returnvalue_9))
  (bind _returnvalue_11 (* _returnvalue_7 _returnvalue_10))
  (bind _returnvalue_12 (Math|Vector|ClampVectorSize _returnvalue_11 0.0 _returnvalue_3))
  (bind _returnvalue_13 (- _force _returnvalue_12))
  (bind _returnvalue_14 (Math|Vector|ClampVectorSize _returnvalue_13 0.0 1.5e+04))
  (if (Class|SceneComponent|IsAnySimulatingPhysics _mesh)
    (bind _returnvalue_15 (Class|MordhauCharacter|IsBoneDismembered bone))
    (Utilities|FlowControl|Sequence
      (:then_0
        (Class|SkeletalMeshComponent|AddImpulsetoAllBodiesBelow (Variables|Character|GetMesh) _returnvalue_4 "Hips" true true))
      (:then_1
        (if (or _returnvalue_15 (not (Physics|IsSimulatingPhysics _mesh bone)))
          (if (not (Physics|IsSimulatingPhysics _mesh _returnvalue))
            (CallFunction|AddRagdollImpulse _returnvalue_14 Point "Spine1")
            (else
              (CallFunction|AddRagdollImpulse _returnvalue_14 Point _returnvalue)))
          (else
            (CallFunction|AddRagdollImpulse _returnvalue_13 Point bone)))))))

(event EventOnPostDismember
  (params (bone :type Name%20%28by%20ref%29 :default "None") (SeparatedPart :type Separated%20Body%20Part%20Object%20Reference) (Agent :type Actor%20Object%20Reference))
  (bind _returnvalue (Transformation|GetActorRightVector SeparatedPart))
  (bind _mesh (Variables|Character|GetMesh))
  (bind _mesh_2 (Variables|/Script/Mordhau.SeparatedBodyPart|GetMesh SeparatedPart))
  (bind _queueddismemberforcedir (Variables|Default|GetQueuedDismemberForceDir))
  (bind _returnvalue_2 (* _returnvalue -1.0))
  (bind _returnvalue_3 (Math|Rotator|MakeRotfromXZ _queueddismemberforcedir _returnvalue_2))
  (bind _returnvalue_4 (Math|Rotator|CombineRotators "-90.000000, 0,0.000000" _returnvalue_3))
  (bind _returnvalue_5 (Class|KismetMathLibrary|NegateRotator _returnvalue_3))
  (bind _returnvalue_6 (Math|Rotator|CombineRotators _returnvalue_5 _returnvalue_4))
  (bind (_roll _pitch _yaw) (Math|Rotator|BreakRotator _returnvalue_6))
  (|CallParentFunction bone SeparatedPart Agent)
  (Utilities|FlowControl|Sequence
    (:then_0
      (if (Math|Boolean|ANDBoolean (Variables|Default|GetbQueuedDismemberIsPartial) (Utilities|Name|Equal(Name) bone "head") (not (Class|SceneComponent|IsAnySimulatingPhysics _mesh)))
        (Audio|SpawnSoundAttached "/Game/Mordhau/Audio/Cues/Foley/SC_DeathGurgle.SC_DeathGurgle" _mesh "Neck" "0, 0, 0" "0, 0, 0" "SnapToTarget" true 1.0 1.0 0.0 0 0)))
    (:then_1
      (if (not (or (Variables|Default|GetbQueuedDismemberIsPartial) (not (Class|SceneComponent|IsAnySimulatingPhysics _mesh_2))))
        (Physics|AddImpulse _mesh_2 (* _queueddismemberforcedir -1.5e+02) bone true)
        (Class|PrimitiveComponent|AddAngularImpulseinDegrees _mesh_2 (* (Math|Vector|MakeVector _roll _pitch _yaw) 1e+01) bone true)))))

(event EventBeginPlay
  (Components|Tick|SetComponentTickEnabled (Variables|Default|GetThudder) false)
  (bind _returnvalue (Game|SpawnActorfromClass "/Game/Mordhau/Blueprints/Equipment/Weapons/BP_KickWeapon.BP_KickWeapon_C" (Math|Transform|MakeTransform "0, 0, 0") "AlwaysSpawn" 0 0))
  (bind _output_get (Variables|Default|SetKickWeapon _returnvalue))
  (Transformation|AttachActorToActor _output_get self "None" "KeepWorld" "KeepWorld" "KeepWorld" false))

(event EventOnCosmeticHit
  (params (DamageType :type EMordhauDamageType%20Enum :default "Generic") (SubType :type Byte :default 0) (Hit :type Hit%20Result%20Structure%20%28by%20ref%29) (Agent :type Actor%20Object%20Reference))
  (bind (_bblockinghit _binitialoverlap _time _distance _location _impactpoint _normal _impactnormal _physmat _hitactor _hitcomponent _hitbonename) (Collision|BreakHitResult Hit))
  (bind _self self)
  (bind _force (CallFunction|ComputeRagdollForce Agent DamageType SubType 255 _self _self))
  (|CallParentFunction DamageType SubType Hit Agent)
  (if (Class|SceneComponent|IsAnySimulatingPhysics (Variables|Character|GetMesh))
    (bind _returnvalue (Class|MordhauCharacter|IsBoneDismembered _hitbonename))
    (if _returnvalue
      (CallFunction|AddRagdollImpulse (* _force 0.5) _impactpoint "Spine1")
      (else
        (CallFunction|AddRagdollImpulse _force _impactpoint _hitbonename)))))

(event EventBPLODTick
  (params (DeltaTime :type Float%20%28single-precision%29))
  (|CallParentFunction DeltaTime)
  (if (Variables|Default|GetbIsDead)
    (Class|ThudderComponent|DoTick (Variables|Default|GetThudder))))

(event EventOnDied
  (params (Angle :type Float%20%28single-precision%29) (Type :type EMordhauDamageType%20Enum :default "Generic") (SubType :type Byte :default 0) (bone :type Name%20%28by%20ref%29 :default "None") (Point :type Vector%20%28by%20ref%29 :default "0, 0, 0") (Source :type Actor%20Object%20Reference) (Agent :type Actor%20Object%20Reference))
  (|CallParentFunction Angle Type SubType bone Point Source Agent)
  (Utilities|FlowControl|Sequence
    (:then_0
      (bind _asab_mordhau_character_animation (Utilities|Casting|CastToAB_MordhauCharacterAnimation (Components|SkeletalMesh|GetAnimInstance (Variables|Character|GetMesh))))
      (if (Utilities|IsValid (stale _returnvalue))
        (Class|AdvancedCharacter|RequestMeshEnablePhysics (stale _returnvalue) 5.0)
        (Class|AdvancedCharacter|StartRagdollwithBlend 0.0 :!label _label)
        (Class|MordhauCharacter|PlayDeathYell (Variables|Default|GetbForceLongDeathYell))
        (elif (Math|Boolean|ORBoolean (Variables|/Script/Mordhau.AdvancedCharacterAnimInstance|GetbIsAirborne _asab_mordhau_character_animation) (not (Class|MordhauUtilityLibrary|HasBeenReallyRecentlyRendered (Variables|Character|GetMesh))) (< (Class|KismetMathLibrary|PercentByteByte (Variables|Default|GetDeathSyncedRandom) 10) 5) (stale _returnvalue) (and (== Type (Utilities|Enum|LiteralenumEMordhauDamageType "Melee")) (== SubType (Utilities|Enum|LiteralenumEAttackMove "Couch"))) (== Type (Utilities|Enum|LiteralenumEMordhauDamageType "Fall")) (>= (Math|Vector|VectorLength (Variables|Default|GetMoveCompVelocityBeforeDeath)) 1e+02) (Variables|Default|GetbIsRagdollFalling))
          (goto _label)
          (else
            (bind _asmordhau_actor (Utilities|Casting|CastToMordhauActor Agent)
              (:then
                (if (Variables|/Script/Mordhau.MordhauActor|GetbForceRagdollOnDeath _asmordhau_actor)
                  (goto _label)))
              (:CastFailed
                (bind _asadvanced_character (Utilities|Casting|CastToAdvancedCharacter Agent))
                (if (Variables|/Script/Mordhau.AdvancedCharacter|GetbForceRagdollIfDmgAgent _asadvanced_character)
                  (goto _label))))))))
    (:then_1
      (bind _asab_mordhau_character_animation_2 (Utilities|Casting|CastToAB_MordhauCharacterAnimation (Components|SkeletalMesh|GetAnimInstance (Variables|Character|GetMesh))))
      (Default|PickDeathAnim _asab_mordhau_character_animation_2 Angle Agent bone Point Type SubType)
      (Class|MordhauCharacter|PlayDeathYell true) ; Won't do anything if we're already playing one from the node above us
    )))

(fn ConstructionScript
  (|CallParentFunction)
  (Variables|Default|SetMordhauCamera (Variables|Default|GetCamera))
  (Variables|Default|SetBlockCollider (Variables|Default|GetBlockColliderBP))
  (Variables|/Script/Mordhau.ThudderComponent|SetMonitoredComponent (Variables|Default|GetThudder) (Variables|Character|GetMesh)))

(fn FindClimbSpot
  (params (UpwardsCast :type Float%20%28single-precision%29))
  (bind _returnvalue (Math|Vector|MakeVector 0.0 0.0 UpwardsCast))
  (bind _returnvalue_2 (Transformation|GetActorLocation))
  (bind _charactermovement (Variables|Character|GetCharacterMovement))
  (bind _capsulecomponent (Variables|Default|GetCapsuleComponent))
  (bind _returnvalue_3 (Class|CharacterMovementComponent|GetWalkableFloorZ _charactermovement))
  (bind _returnvalue_4 (+ _returnvalue_2 _returnvalue))
  (bind _capsulehalfheight (Variables|/Script/Engine.CapsuleComponent|GetCapsuleHalfHeight _capsulecomponent))
  (bind _capsuleradius (Variables|/Script/Engine.CapsuleComponent|GetCapsuleRadius _capsulecomponent))
  (Utilities|FlowControl|Sequence
    (:then_0
      (bind (_outhit _returnvalue_5) (Class|KismetSystemLibrary|CapsuleTraceSinglebyProfile _returnvalue_2 _returnvalue_4 _capsuleradius _capsulehalfheight "Pawn" false 0 "None" true))
      (if _returnvalue_5
        (bind _output_get (LocalVariables|SetStage1 (.Location (Collision|BreakHitResult _outhit))))
        (if (< (Math|Vector|VectorLength (- _returnvalue_4 _output_get)) 74.0)
          (return false "0, 0, 0"))
        (else
          (LocalVariables|SetStage1 _returnvalue_4))))
    (:then_1
      (bind (_outhit_2 _returnvalue_6) (Class|KismetSystemLibrary|CapsuleTraceSinglebyProfile (LocalVariables|GetStage1) (+ (LocalVariables|GetStage1) (* (Transformation|GetActorForwardVector) (* _capsuleradius 2.0))) _capsuleradius _capsulehalfheight "Pawn" false 0 "None" true))
      (if _returnvalue_6
        (bind _output_get_2 (LocalVariables|SetStage2 (.Location (Collision|BreakHitResult _outhit_2))))
        (if (< (Math|Vector|VectorLength (- (LocalVariables|GetStage1) _output_get_2)) (* _capsuleradius 0.5))
          (return false "0, 0, 0"))
        (else
          (LocalVariables|SetStage2 (+ (LocalVariables|GetStage1) (* (Transformation|GetActorForwardVector) (* _capsuleradius 2.0)))))))
    (:then_2
      (bind (_outhit_3 _returnvalue_7) (Class|KismetSystemLibrary|CapsuleTraceSinglebyProfile (LocalVariables|GetStage2) (+ (LocalVariables|GetStage2) (Math|Vector|MakeVector 0.0 0.0 (* UpwardsCast -1.0))) _capsuleradius _capsulehalfheight "Pawn" false 0 "None" true))
      (if _returnvalue_7
        (bind (_outhit_4 _returnvalue_8) (Class|KismetSystemLibrary|CapsuleTraceSinglebyProfile (LocalVariables|GetStage2) (+ (LocalVariables|GetStage2) (Math|Vector|MakeVector 0.0 0.0 (* UpwardsCast -1.0))) (* _capsuleradius 0.25) _capsulehalfheight "Pawn" false 0 "None" true))
        (if _returnvalue_8
          (bind _output_get_3 (LocalVariables|SetStage3 (.Location (Collision|BreakHitResult _outhit_3))))
          (LocalVariables|SetFinalActorToCheck (.HitActor (Collision|BreakHitResult _outhit_3)))
          (Utilities|IsValid (Transformation|GetAttachParent (.HitComponent (Collision|BreakHitResult _outhit_3)))
            (:Is%20Valid
              (LocalVariables|SetFinalActorToCheck (Components|GetOwner (Transformation|GetAttachParent (.HitComponent (Collision|BreakHitResult _outhit_3))))))
            (:Is%20Not%20Valid
              _))
          (Utilities|Casting|CastToEnvironmentMovable (LocalVariables|GetFinalActorToCheck)
            (:then
              (return false "0, 0,0.000000"))
            (:CastFailed
              (Utilities|Casting|CastToBP_BaseProgressActor (LocalVariables|GetFinalActorToCheck)
                (:then
                  (return false "0, 0,0.000000"))
                (:CastFailed
                  (bind _asmordhau_actor (Utilities|Casting|CastToMordhauActor (LocalVariables|GetFinalActorToCheck))
                    (:then
                      (if (Variables|/Script/Mordhau.MordhauActor|GetbPreventClimbing _asmordhau_actor)
                        (return false "0, 0,0.000000")
                        (else
                          (if (Math|Boolean|ORBoolean (< (- (.Z (Math|Vector|BreakVector _output_get_3)) (.Z (Math|Vector|BreakVector (Transformation|GetActorLocation)))) 74.0) (not (Class|PrimitiveComponent|CanCharacterStepUp (.HitComponent (Collision|BreakHitResult _outhit_3)) self)) (Math|Boolean|ORBoolean (> (- (.Z (Math|Vector|BreakVector (.Location (Collision|BreakHitResult _outhit_3)))) (.Z (Math|Vector|BreakVector (.Location (Collision|BreakHitResult _outhit_4))))) 25.0) (< (.Z (Math|Vector|BreakVector (.ImpactNormal (Collision|BreakHitResult _outhit_3)))) _returnvalue_3) (< (.Z (Math|Vector|BreakVector (.ImpactNormal (Collision|BreakHitResult _outhit_4)))) _returnvalue_3))) :!label _label
                            (return false "0, 0,0.000000")))))
                    (:CastFailed
                      (goto _label)))))))
          (else
            (return false "0, 0,0.000000")))
        (else
          (return false "0, 0,0.000000"))))
    (:then_3
      (return true (LocalVariables|GetStage3)))))

(fn AttemptClimb
  (bind _motion (Variables|Default|GetMotion))
  (bind _righthandequipment (Variables|Default|GetRightHandEquipment))
  (if (or (Variables|Default|GetbIsRagdollFalling) (not (Variables|Default|GetbAllowClimbing)))
    _
    (else
      (Utilities|IsValid _righthandequipment
        (:Is%20Valid
          (if (Variables|/Script/Mordhau.MordhauEquipment|GetbPreventsClimbing _righthandequipment)
            _
            (else
              (Utilities|Casting|CastToClimbingMotion _motion :!label _label
                (:then
                  _)
                (:CastFailed
                  (Utilities|Casting|CastToParryMotion _motion
                    (:then
                      _)
                    (:CastFailed
                      (bind _asattack_motion (Utilities|Casting|CastToAttackMotion _motion)
                        (:then
                          (if (Utilities|Enum|Equal(Enum) (Variables|/Script/Mordhau.AttackMotion|GetStage _asattack_motion) "Recovery")
                            (bind (_succeeded _targetspot) (CallFunction|FindClimbSpot 2e+02 :!label _label_2))
                            (if _succeeded
                              (Variables|Default|SetClimbTargetLocation _targetspot)
                              (CallFunction|ServerSetClimbLocation (Math|Vector|MakeVectorNetQuantize (.X (Math|Vector|BreakVector (Variables|Default|GetClimbTargetLocation))) (.Y (Math|Vector|BreakVector (Variables|Default|GetClimbTargetLocation))) (.Z (Math|Vector|BreakVector (Variables|Default|GetClimbTargetLocation)))) :!label _label_3)
                              (Class|MordhauCharacter|RequestClimb (Variables|Default|GetClimbTargetLocation))
                              (return true)
                              (else
                                (bind (_succeeded_2 _targetspot_2) (CallFunction|FindClimbSpot 1e+02))
                                (if _succeeded_2
                                  (Variables|Default|SetClimbTargetLocation _targetspot_2)
                                  (goto _label_3)
                                  (else
                                    _))))))
                        (:CastFailed
                          (goto _label_2))))))))))
        (:Is%20Not%20Valid
          (goto _label)))))
  (return false))

(fn CalculateLedgeOffsetandNormal
  (params (ClimbingMotion :type Climbing%20Motion%20Object%20Reference))
  (bind _returnvalue (Transformation|GetActorLocation))
  (bind _capsulecomponent (Variables|Default|GetCapsuleComponent))
  (bind _returnvalue_2 (+ _returnvalue "0, 0,50.000000"))
  (bind (_outhit _returnvalue_3) (Class|KismetSystemLibrary|CapsuleTraceSinglebyProfile _returnvalue_2 (+ _returnvalue_2 (* (Transformation|GetActorForwardVector) 105.0)) (Variables|/Script/Engine.CapsuleComponent|GetCapsuleRadius _capsulecomponent) (Variables|/Script/Engine.CapsuleComponent|GetCapsuleHalfHeight _capsulecomponent) "Pawn" false 0 "None" true))
  (if (not _returnvalue_3)
    (return "0, 0, 0" "0, 0, 0" false false "0, 0, 0" "0, 0, 0" "0, 0, 0" "0, 0, 0" "0, 0, 0" "0, 0, 0" "0, 0, 0" "0, 0, 0" "0, 0, 0" "0, 0, 0")))

(fn TryClimbing
  (bind _returnvalue (Class|AdvancedCharacter|IsAirborne))
  (if (or (Character|CanJump) (and _returnvalue (> (.Z (Math|Vector|BreakVector (Transformation|GetVelocity))) -9e+02)))
    (bind _succeeded (CallFunction|AttemptClimb))
    (if _succeeded
      (return true)
      (else
        _)))
  (return false))

(fn AddRagdollImpulse
  (params (Impulse :type Vector) (Location :type Vector) (Bone :type Name))
  (bind _mesh (Variables|Character|GetMesh))
  (Physics|AddImpulseatLocation _mesh (* Impulse (Math|Float|Max(Float) (/ (Class|SkeletalMeshComponent|GetBoneMass _mesh Bone true) 15.0) 0.5)) Location Bone))

(fn GetOutOfBoundsText
  (if (stale _returnvalue)
    (return "Too close to enemy spawn! Fall back!")
    (else
      (return "Get back to the fight, coward!"))))

(fn GetOutOfBoundsSubtext
  (return (Utilities|Text|FormatText "Death in {a} seconds" (Math|Float|Ceil (Class|AdvancedCharacter|GetOutOfBoundsTimeUntilDeath)))))