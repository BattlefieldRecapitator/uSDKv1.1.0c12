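; A display actor that shows equipment pieces from a list one at a time, spinning them in place.
; On a timer it advances through the looping list, destroys the previous piece, spawns the next customized one through the Mordhau singleton and attaches it to its root with the physics proxy removed.
; Tick accumulates a yaw angle from the spin speed and applies it to the current piece's skeletal mesh.
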(event EventBeginPlay
  (Variables|Default|SetNextSwitchTime (+ (Utilities|Time|GetGameTimeinSeconds) (Variables|Default|GetSwitchTime)))
  (Variables|Default|SetCurrentId -1)
  (CallFunction|AdvanceEquipmentinList))

(event EventTick
  (params (DeltaSeconds :type Float%20%28single-precision%29))
  (bind _currentinstance (Variables|Default|GetCurrentInstance))
  (bind _skeletalmeshcomponent (Variables|/Script/Mordhau.MordhauEquipment|GetSkeletalMeshComponent _currentinstance))
  (bind _relativerotation (Variables|/Script/Engine.SceneComponent|GetRelativeRotation _skeletalmeshcomponent))
  (bind (_roll _pitch) (Math|Rotator|BreakRotator _relativerotation))
  (Variables|Default|SetCurrentDegrees (Math|Float|%(Float) (+ (Variables|Default|GetCurrentDegrees) (* (Variables|Default|GetSpinSpeed) DeltaSeconds)) 3.6e+02))
  (if (< (Variables|Default|GetNextSwitchTime) (Utilities|Time|GetGameTimeinSeconds))
    (Variables|Default|SetNextSwitchTime (+ (Utilities|Time|GetGameTimeinSeconds) (Variables|Default|GetSwitchTime)))
    (CallFunction|AdvanceEquipmentinList))
  (Utilities|IsValid _currentinstance
    (:Is%20Valid
      (Transformation|SetRelativeRotation _skeletalmeshcomponent (Math|Rotator|MakeRotator _roll _pitch (Variables|Default|GetCurrentDegrees)) false false))))

(fn ConstructionScript)

(fn AdvanceEquipmentinList
  (bind _equipmentlist (Variables|Default|GetEquipmentList))
  (Variables|Default|SetCurrentId (Math|Integer|%(Integer) (+ (Variables|Default|GetCurrentId) 1) (Utilities|Array|Length _equipmentlist)))
  (if (Utilities|Array|IsValidIndex _equipmentlist (Variables|Default|GetCurrentId))
    (Utilities|IsValid (Variables|Default|GetCurrentInstance)
      (:Is%20Valid
        (Actor|DestroyActor (Variables|Default|GetCurrentInstance)))
      (:Is%20Not%20Valid
        _))
    (bind _returnvalue (Class|MordhauSingleton|SpawnEquipment (Class|MordhauUtilityLibrary|GetMordhauSingleton) (Class|MordhauUtilityLibrary|GetWorldOf self) (Utilities|Array|Get(acopy) (Variables|Default|GetEquipmentList) (Variables|Default|GetCurrentId)) 0 0 0 false false))
    (bind _output_get (Variables|Default|SetCurrentInstance _returnvalue))
    (Transformation|AttachComponentToComponent _output_get (Variables|Default|GetDefaultSceneRoot) "None" "SnapToTarget" "SnapToTarget" "SnapToTarget" false)
    (Class|MordhauEquipment|DestroyPhysicsProxy _output_get)))