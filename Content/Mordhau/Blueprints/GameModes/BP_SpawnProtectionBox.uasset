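; Team spawn protection volume that notifies Mordhau characters when they enter or leave an area reserved for its allowed team.
; Overlap events pass the allowed team to the character, which receives the entered or left team area call.
; When navmesh use is on, the construction script gives the box a team-only nav area class, or the default for other team values.
; Enable and Disable switch the box collision between query-only and none.
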(event EventBeginPlay)

(event Collision|EventActorBeginOverlap
  (params (OtherActor :type Actor%20Object%20Reference))
  (bind _asmordhau_character (Utilities|Casting|CastToMordhauCharacter OtherActor))
  (Class|MordhauCharacter|EnteredTeamArea _asmordhau_character (Variables|Default|GetAllowedTeam)))

(event Collision|EventActorEndOverlap
  (params (OtherActor :type Actor%20Object%20Reference))
  (bind _asmordhau_character (Utilities|Casting|CastToMordhauCharacter OtherActor))
  (Class|MordhauCharacter|LeftTeamArea _asmordhau_character (Variables|Default|GetAllowedTeam)))

(event EventTick
  (params (DeltaSeconds :type Float%20%28single-precision%29)))

(fn ConstructionScript
  (bind _allowedteam (Variables|Default|GetAllowedTeam))
  (if (Variables|Default|GetUsesNavmesh)
    (if (and (>= _allowedteam 0) (< _allowedteam 2))
      (Class|MordhauUtilityLibrary|SetNavAreaClass (Variables|Default|GetBox) (Utilities|Select :Index _allowedteam :Option%200 "/Game/Mordhau/AI/Navigation/BP_NavArea_Team1Only.BP_NavArea_Team1Only_C" :Option%201 "/Game/Mordhau/AI/Navigation/BP_NavArea_Team2Only.BP_NavArea_Team2Only_C"))
      (else
        (Class|MordhauUtilityLibrary|SetNavAreaClass (Variables|Default|GetBox) "/Script/NavigationSystem.NavArea_Default")))))

(fn Enable
  (bind _box (Variables|Default|GetBox))
  (if (Utilities|Enum|NotEqual(Enum) (Collision|GetCollisionEnabled _box) "QueryOnly")
    (Collision|SetCollisionEnabled _box "QueryOnly")))

(fn Disable
  (bind _box (Variables|Default|GetBox))
  (if (Utilities|Enum|NotEqual(Enum) (Collision|GetCollisionEnabled _box) "NoCollision")
    (Collision|SetCollisionEnabled _box "NoCollision")))