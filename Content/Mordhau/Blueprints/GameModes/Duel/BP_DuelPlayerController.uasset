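; Player controller for Duel mode that drives the local player's HUD through matchmade rounds.
; Tick polls the replicated room's round stage for waiting countdowns, HUD updates and tips, has the lobby owner close the matchmaking lobby, and sends customization when no profile is selected.
; RepNotifies announce fights and round results, declare the match at five wins, enable dropping on the duel character, and show a delayed endscreen when new MMR arrives.
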(event Custom|ShowDuelEndscreenDelayed
  (Utilities|FlowControl|Delay 6.5)
  (bind _asbp_duel_hud (Utilities|Casting|CastToBP_DuelHUD (Variables|Default|GetHUD)))
  (Default|ShowDuelEndScreen _asbp_duel_hud))

(event EventBeginPlay
  (|CallParentFunction)
  (bind _asbp_mordhau_game_instance (Utilities|Casting|CastToBP_MordhauGameInstance (Game|GetGameInstance)))
  (Variables|Default|SetGameInstance _asbp_mordhau_game_instance))

(event EventTick
  (params (DeltaSeconds :type Float%20%28single-precision%29))
  (bind _replicatedroomgame (Variables|Default|GetReplicatedRoomGame))
  (bind _roundinfo (Utilities|Struct|BreakST_DuelRoomGame _replicatedroomgame))
  (bind (_stage _winner _starttime) (Utilities|Struct|BreakSTRUCT_DuelRoundInfo _roundinfo))
  (|CallParentFunction DeltaSeconds)
  (if (Pawn|IsLocalPlayerController)
    (Utilities|IsValid (Game|GetGameState)
      (:Is%20Valid
        (Utilities|FlowControl|Sequence
          (:then_0
            (if (and (== (Variables|Default|GetSelectedCharacterProfile) -1) (== (Variables|Default|GetSelectedDefaultProfile) -1))
              (if (Variables|Default|GetbIsInventoryAvailableOnAuthority)
                (Class|MordhauPlayerController|PrepareandSendCustomizationifChanged))))
          (:then_1
            (if (and (Variables|Default|GetHasReplicatedRoomGame) (> (Utilities|Time|GetTimeSeconds) 3.0))
              (switch Utilities|FlowControl|Switch|SwitchonE_DuelRoundStage _stage
                (:NewEnumerator0
                  (Default|ShowAnnouncement (Variables|Default|GetHUD) "Waiting for players" (Utilities|Text|FormatText "-{0}-" (Math|Float|Ceil (Math|Float|Max(Float) (- _starttime (GameState|GetServerWorldTimeSeconds (Game|GetGameState))) 0.0))) 0.1))
                (:NewEnumerator4
                  ;[1 1 1] hacky, assumes roundstart is 3s
                  (Utilities|FlowControl|Sequence
                    (:then_1
                      (if (Math|Boolean|ANDBoolean (Class|MordhauUtilityLibrary|IsValidSteamID (Variables|Default|GetMatchmakingLobbyID)) (Class|MordhauUtilityLibrary|EqualSteamID (Class|MordhauGameInstance|GetMatchmakingLobbyOwner (Variables|Default|GetGameInstance)) (Class|MordhauUtilityLibrary|GetSteamID)) (not (Variables|Default|GetIsMatchmakingLobbyClosed)))
                        (bind _returnvalue (Class|MordhauGameInstance|CloseMatchmakingLobby (Variables|Default|GetGameInstance)))
                        (Variables|Default|SetIsMatchmakingLobbyClosed _returnvalue)))))
                (:NewEnumerator1
                  (Utilities|FlowControl|Sequence
                    (:then_0
                      (Utilities|FlowControl|DoOnce false
                        (:Completed
                          (bind _asbp_duel_hud (Utilities|Casting|CastToBP_DuelHUD (Variables|Default|GetHUD) :!label _label))
                          (Default|Update (Variables|/Game/Mordhau/Blueprints/GameModes/Duel/BP_DuelHUD.BP_DuelHUD_C|GetDuelHUDWidget _asbp_duel_hud))
                          (Class|MordhauPlayerController|ShowTips))))
                    (:then_1
                      (goto _label_2 Reset))))
                (:NewEnumerator2
                  (Variables|Default|SetCountdown 0))
                (:NewEnumerator3
                  (Utilities|FlowControl|DoOnce false :!label _label_2
                    (:Completed
                      (goto _label))))))))))))

(fn ConstructionScript
  (|CallParentFunction))

(fn OnRepReplicatedRoomGame
  (bind _hud (Variables|Default|GetHUD))
  (bind _replicatedroomgame (Variables|Default|GetReplicatedRoomGame))
  (bind _hud_2 (Variables|Default|GetHUD))
  (bind _hud_3 (Variables|Default|GetHUD))
  (bind (_team1wins _team2wins _roundinfo) (Utilities|Struct|BreakST_DuelRoomGame _replicatedroomgame))
  (bind (_stage _winner) (Utilities|Struct|BreakSTRUCT_DuelRoundInfo _roundinfo))
  (bind _returnvalue (== _team1wins 5))
  (bind _returnvalue_2 (== _team2wins 5))
  (bind _returnvalue_3 (or _returnvalue _returnvalue_2))
  (Utilities|FlowControl|Sequence
    (:then_0
      (if (Pawn|IsLocalPlayerController)
        (Variables|Default|SetHasReplicatedRoomGame true)
        (Utilities|FlowControl|Sequence
          (:then_0
            (switch Utilities|FlowControl|Switch|SwitchonE_DuelRoundStage _stage
              (:NewEnumerator1
                (Utilities|IsValid _hud
                  (:Is%20Valid
                    (Utilities|IsValid 0
                      (:Is%20Valid
                        (Default|Hide (Variables|/Game/Mordhau/Blueprints/BP_MordhauHUD.BP_MordhauHUD_C|GetEmoteMenu _hud)))))))
              (:NewEnumerator2
                (Default|ShowAnnouncement _hud_2 "Fight!" "" 2.0)
                (Default|HideMainMenu _hud_2)
                (Audio|PlaySound2D 0 1.0 1.0 0.0 0 0))
              (:NewEnumerator3
                (bind _asmordhau_player_state (Utilities|Casting|CastToMordhauPlayerState (Variables|Default|GetPlayerState)))
                (if (== _winner (Math|Conversions|ToByte(Integer) (Variables|/Script/Mordhau.MordhauPlayerState|GetTeam _asmordhau_player_state)))
                  (if _returnvalue_3
                    (Default|ShowMatchResult _hud_3 true "victory")
                    (else
                      (Default|ShowAnnouncement _hud_3 "Round won" "" 3.0)))
                  (elif _returnvalue_3
                    (Default|ShowMatchResult _hud_3 false "defeat")
                    (else
                      (Default|ShowAnnouncement _hud_3 "Round lost" "" 3.0))))))))))
    (:then_1
      (if (Utilities|Enum|Equal(Enum) _stage "NewEnumerator2")
        (bind _asbp_duel_character (Utilities|Casting|CastToBP_DuelCharacter (Pawn|GetControlledPawn)))
        (Variables|/Script/Mordhau.MordhauCharacter|SetbAllowDrop _asbp_duel_character true)))))

(fn OnRepNewMMR
  (if (Pawn|IsLocalPlayerController)
    (CallFunction|ShowDuelEndscreenDelayed)))

(fn UpdateCountdown
  (params (StartTime :type Float%20%28single-precision%29))
  (bind _returnvalue (Utilities|Time|GetTimeSeconds))
  (bind _hud (Variables|Default|GetHUD))
  (bind _returnvalue_2 (- StartTime _returnvalue))
  (bind _returnvalue_3 (Math|Float|Ceil _returnvalue_2))
  (bind _returnvalue_4 (Math|Integer|Max(Integer) _returnvalue_3))
  (if (!= (Variables|Default|GetCountdown) _returnvalue_4)
    (bind _output_get (Variables|Default|SetCountdown _returnvalue_4))
    (Utilities|FlowControl|Sequence
      (:then_0
        (if (<= _output_get 10)
          (Audio|PlaySound2D 0 1.0 1.0 0.0 0 0)))
      (:then_1
        (if (<= _output_get 5)
          (Default|ShowAnnouncement _hud "Get ready!" (Utilities|Text|FormatText "-{0}-" _output_get) 1.2)
          (else
            (Default|ShowAnnouncement _hud "Match starting" (Utilities|Text|FormatText "-{0}-" _output_get) 1.2)))))))

(fn ComputePlayerRank)