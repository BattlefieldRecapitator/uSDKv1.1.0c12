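; Base Battle Royale item spawn actor that picks a weighted random class from its item list and spawns it on request.
; GetRandomItem renormalizes the weights, then uses roulette wheel selection to feed SpawnRandomItem.
; Mordhau equipment spawns with its armory offset plus a quarter turn and receives random customization.
; When a character is supplied, that character's default customization, if found, and emblem with colors are applied instead.
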(event EventBeginPlay)

(event Collision|EventActorBeginOverlap
  (params (OtherActor :type Actor%20Object%20Reference)))

(event EventTick
  (params (DeltaSeconds :type Float%20%28single-precision%29)))

(fn ConstructionScript)

(fn RenormalizeChances
  (bind _itemlist (Variables|Spawning|GetItemList))
  (if (>= (Utilities|Map|Length _itemlist) 1)
    (bind _keys (Utilities|Map|Keys _itemlist))
    (for _array_element _keys
      (LocalVariables|SetTotalChances (+ (Math|Float|Absolute(Float) (.Value (Utilities|Map|Find _itemlist _array_element))) (LocalVariables|GetTotalChances)))
      (LocalVariables|SetMaxChance (Math|Float|Max(Float) (LocalVariables|GetMaxChance) (Math|Float|Absolute(Float) (.Value (Utilities|Map|Find _itemlist _array_element))))))
    (if (> (LocalVariables|GetMaxChance) 0.0)
      (for _array_element_2 _keys
        (Utilities|Map|Add _itemlist _array_element_2 (/ (.Value (Utilities|Map|Find _itemlist _array_element_2)) (LocalVariables|GetTotalChances)))))))

(fn GetRandomItem
  (bind _itemlist (Variables|Spawning|GetItemList))
  ;[1 1 1] Roulette wheel selection method
  (Spawning|RenormalizeChances)
  (bind _keys (Utilities|Map|Keys _itemlist))
  (LocalVariables|SetRandomNumber (Math|Random|RandomFloat))
  (bind (_array_element _array_index) (Utilities|Array|ForEachLoopwithBreak _keys :!label _label)
    (:LoopBody
      (LocalVariables|SetBestId _array_index)
      (LocalVariables|SetCurrent (+ (.Value (Utilities|Map|Find _itemlist _array_element)) (LocalVariables|GetCurrent)))
      (if (>= (LocalVariables|GetCurrent) (LocalVariables|GetRandomNumber))
        (goto _label Break)))
    (:Completed
      (if (> (Utilities|Array|Length _keys) 0)
        (return (Utilities|Array|Get(acopy) _keys (LocalVariables|GetBestId)))
        (else
          (return 0))))))

(fn SpawnRandomItem
  (params (InSpawnTransform :type Transform) (CustomizeFor :type Mordhau%20Player%20Controller%20Object%20Reference))
  (bind _characterprofile (Variables|/Script/Mordhau.MordhauPlayerController|GetCharacterProfile CustomizeFor))
  (bind _appearancecustomization (Utilities|Struct|BreakCharacterProfile _characterprofile))
  (bind (_emblem _emblemcolors) (Utilities|Struct|BreakAppearanceCustomization _appearancecustomization))
  (bind _founditem (CallFunction|GetRandomItem))
  (if (Utilities|IsValidClass _founditem)
    (LocalVariables|SetSpawnTransform InSpawnTransform)
    (Utilities|FlowControl|Sequence
      (:then_0
        (if (Utilities|ClassIsChildOf _founditem "/Script/Mordhau.MordhauEquipment")
          (bind _asmordhau_equipment (Utilities|Casting|CastToMordhauEquipment (Class|MordhauUtilityLibrary|GetDefaultActor _founditem)))
          (LocalVariables|SetSpawnTransform (Math|Transform|ComposeTransforms (Math|Transform|MakeTransform "0, 0, 0" "90.000000, 0,0.000000") (Math|Transform|ComposeTransforms (Variables|/Script/Mordhau.MordhauEquipment|GetArmoryTransformOffset _asmordhau_equipment) (LocalVariables|GetSpawnTransform))))))
      (:then_1
        (bind _returnvalue (Game|SpawnActorfromClass _founditem (LocalVariables|GetSpawnTransform) "Undefined" 0 0))
        (bind _asmordhau_equipment_2 (Utilities|Casting|CastToMordhauEquipment _returnvalue))
        (bind _returnvalue_2 (Class|MordhauEquipment|GetRandomCustomization _asmordhau_equipment_2 true))
        (LocalVariables|SetCustomizationToApply _returnvalue_2)
        (Utilities|FlowControl|Sequence
          (:then_0
            (Utilities|IsValid CustomizeFor
              (:Is%20Valid
                (LocalVariables|SetEmblem _emblem)
                (LocalVariables|SetEmblemColor1 (Utilities|Array|Get(acopy) _emblemcolors))
                (LocalVariables|SetEmblemColor2 (Utilities|Array|Get(acopy) _emblemcolors 1))
                (bind (_outcustomization _returnvalue_3) (Class|MordhauPlayerController|GetDefaultEquipmentCustomizationfor CustomizeFor (Utilities|GetClass _asmordhau_equipment_2)))
                (if _returnvalue_3
                  (LocalVariables|SetCustomizationToApply _outcustomization)))))
          (:then_1
            (Class|MordhauEquipment|AssignCustomization _asmordhau_equipment_2 (LocalVariables|GetCustomizationToApply) (Math|Conversions|ToByte(Integer) (LocalVariables|GetEmblem)) (LocalVariables|GetEmblemColor1) (LocalVariables|GetEmblemColor2)))))
      (:then_2
        (return _returnvalue)))))