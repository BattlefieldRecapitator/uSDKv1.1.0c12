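; Deathmatch game mode that ends the match on a score limit and records the winner in the game state.
; A score change that reaches ScoreToWin during a match in progress ends it with that player as winner.
; When time runs out, FindWinner gathers team 0 players from the PlayerArray, sorts them and returns the first.
; Both paths write the winner and score into the game state's MatchEndInfo.
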(event EventOnScoreChanged
  (params (State :type Player%20State%20Object%20Reference) (OldValue :type Float%20%28single-precision%29))
  (bind _score (Variables|/Script/Engine.PlayerState|GetScore State))
  (bind _asbp_mordhau_player_state (Utilities|Casting|CastToBP_MordhauPlayerState State))
  (if (and (>= _score (Variables|Default|GetScoreToWin)) (Class|GameMode|IsMatchinProgress))
    (Class|GameMode|EndMatch)
    (bind _asbp_mordhau_game_state (Utilities|Casting|CastToBP_MordhauGameState (Game|GetGameState)))
    (Variables|/Game/Mordhau/Blueprints/GameModes/BP_MordhauGameState.BP_MordhauGameState_C|SetMatchEndInfo _asbp_mordhau_game_state (Utilities|Struct|MakeSTRUCT_MatchEndInfo _asbp_mordhau_player_state 0 _score))))

(event EventMatchTimeRanOut
  (|CallParentFunction)
  (bind _asbp_mordhau_game_state (Utilities|Casting|CastToBP_MordhauGameState (Game|GetGameState)))
  (bind _winner (CallFunction|FindWinner))
  (Variables|/Game/Mordhau/Blueprints/GameModes/BP_MordhauGameState.BP_MordhauGameState_C|SetMatchEndInfo _asbp_mordhau_game_state (Utilities|Struct|MakeSTRUCT_MatchEndInfo _winner 0 (Variables|/Script/Engine.PlayerState|GetScore _winner))))

(event EventTick
  (params (DeltaSeconds :type Float%20%28single-precision%29)))

(fn ConstructionScript
  (|CallParentFunction))

(fn FindWinner
  (bind _returnvalue (Game|GetGameState))
  (bind _sortedplayers (LocalVariables|GetSortedPlayers))
  (Utilities|Casting|CastToBP_MordhauGameState _returnvalue
    (:then
      (for _array_element (Variables|/Script/Engine.GameStateBase|GetPlayerArray _returnvalue)
        (bind _asbp_mordhau_player_state (Utilities|Casting|CastToBP_MordhauPlayerState _array_element))
        (if (== (Variables|/Script/Mordhau.MordhauPlayerState|GetTeam _asbp_mordhau_player_state) 0)
          (Utilities|Array|Add _sortedplayers _asbp_mordhau_player_state)))
      (bind _returnvalue_2 (Class|MordhauUtilityLibrary|SortPlayers _sortedplayers))
      (if (> (Utilities|Array|Length _returnvalue_2) 0)
        (bind _asbp_mordhau_player_state_2 (Utilities|Casting|CastToBP_MordhauPlayerState (Utilities|Array|Get(acopy) _returnvalue_2))
          (:then
            (return _asbp_mordhau_player_state_2))
          (:CastFailed
            _))))
    (:CastFailed
      _))
  (return 0))