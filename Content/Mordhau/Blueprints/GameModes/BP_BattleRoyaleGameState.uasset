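; Battle Royale game state that drives match-phase presentation and rules through Tick, rep notifies and overrides.
; At match start it clears dead characters with authority once, disables chat and scoreboard, then shows a server-time "Get ready" countdown while blocking pawn input.
; Replicated countdown changes trigger announcements and sound until match-end info arrives.
; The local winner gets a victory message and delayed end screen, and remote clients auto-disconnect shortly before map change.
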(event EventHandleMatchEndInfo
  (bind _returnvalue (Game|GetPlayerController 0))
  (|CallParentFunction)
  (bind _asbp_mordhau_hud (Utilities|Casting|CastToBP_MordhauHUD (Class|MordhauUtilityLibrary|GetMordhauHUD)))
  (if (Pawn|IsLocalPlayerController _returnvalue)
    (bind _asmordhau_player_state (Utilities|Casting|CastToMordhauPlayerState (Variables|/Script/Engine.Controller|GetPlayerState _returnvalue)))
    (if (== (.Winner (Utilities|Struct|BreakSTRUCT_MatchEndInfo (Variables|Default|GetMatchEndInfo))) _asmordhau_player_state)
      (Default|ShowMatchResult _asbp_mordhau_hud true "victory")
      (bind _asbp_battle_royale_player_controller (Utilities|Casting|CastToBP_BattleRoyalePlayerController _returnvalue))
      (Default|ShowBREndScreenDelayed _asbp_battle_royale_player_controller))))

(event EventTick
  (params (DeltaSeconds :type Float%20%28single-precision%29))
  (bind _returnvalue (GameState|GetServerWorldTimeSeconds))
  (bind _returnvalue_2 (Game|GetPlayerController 0))
  (bind _roundstartduration (Variables|Default|GetRoundStartDuration))
  (bind _warmupend (Variables|Default|GetWarmupEnd))
  (bind _returnvalue_3 (+ _warmupend _roundstartduration))
  (bind _returnvalue_4 (- _returnvalue_3 _returnvalue))
  (bind _returnvalue_5 (Math|Float|Max(Float) _returnvalue_4 0.0))
  (bind _returnvalue_6 (Math|Float|Ceil _returnvalue_5))
  (|CallParentFunction DeltaSeconds)
  (Utilities|Casting|CastToBP_MordhauPlayerController _returnvalue_2)
  (if (Pawn|IsLocalPlayerController _returnvalue_2)
    (bind _asbp_mordhau_hud (Utilities|Casting|CastToBP_MordhauHUD (HUD|GetHUD _returnvalue_2)))
    (if (Utilities|Name|Equal(Name) (Variables|Default|GetMatchState) "InProgress")
      (Utilities|FlowControl|Sequence
        (:then_0
          (Utilities|FlowControl|DoOnce false
            (:Completed
              (Utilities|FlowControl|Sequence
                (:then_0
                  ;[1 1 1] Destroy ragdoll corpses
                  (bind _outactors (Actor|GetAllActorsOfClass "/Script/Mordhau.AdvancedCharacter"))
                  (for _array_element _outactors
                    (if (and (Ability|HasAuthority _array_element) (Variables|/Script/Mordhau.MordhauCharacter|GetbIsDead _array_element))
                      (Actor|DestroyActor _array_element))))
                (:then_1
                  (Variables|Default|SetbDisableChat true)
                  (Variables|Default|SetbDisableScoreboard true))))))
        (:then_1
          (if (> (+ (Variables|Default|GetWarmupEnd) (Variables|Default|GetRoundStartDuration)) (GameState|GetServerWorldTimeSeconds))
            (if (!= _returnvalue_6 0)
              (Default|ShowAnnouncement _asbp_mordhau_hud "Get ready" (Utilities|Text|FormatText "-{0}-" _returnvalue_6) 0.1)))))
      (elif (Math|Boolean|ANDBoolean (Utilities|Name|Equal(Name) (Variables|Default|GetMatchState) "WaitingPostMatch") (Variables|Default|GetMatchEndInfoReplicated) (> (Variables|Default|GetEndMatchMapChangeEnd) 0.0))
        ;[1 1 1] Auto leave
        (if (< (- (Variables|Default|GetEndMatchMapChangeEnd) (GameState|GetServerWorldTimeSeconds)) 1e+01)
          (Networking|SwitchHasAuthority
            (:Remote
              (Development|ExecuteConsoleCommand "disconnect" (Game|GetPlayerController 0)))))))))

(event EventBeginPlay)

(fn ConstructionScript
  (|CallParentFunction))

(fn ShouldHideSpawnInfoText
  (return true))

(fn ShouldBlockPawnInput
  (bind _returnvalue (|CallParentFunction))
  (return (or _returnvalue (CallFunction|IsinGetReady))))

(fn OnRepCountdown
  (bind _countdown (Variables|Default|GetCountdown))
  (Utilities|FlowControl|Sequence
    (:then_0
      ;[1 1 1] Prevents overriding the match end text if it replicates late
      (if (not (Variables|Default|GetMatchEndInfoReplicated))
        (if (not (== (Variables|Default|GetPreviousCountdown) 0))
          (bind _asbp_mordhau_hud (Utilities|Casting|CastToBP_MordhauHUD (Class|MordhauUtilityLibrary|GetMordhauHUD)))
          (if (and (<= _countdown 20) (> _countdown 1))
            (Default|ShowAnnouncement _asbp_mordhau_hud (Utilities|Text|FormatText "-{a}-" _countdown) "" 2.0)
            (Audio|PlaySound2D "/Game/Mordhau/Audio/Cues/UI/SC_BattleRoyaleCountdown.SC_BattleRoyaleCountdown" 1.0 1.0 0.0 0 0)))))
    (:then_1
      (Variables|Default|SetPreviousCountdown (Variables|Default|GetCountdown)))))

(fn IsinGetReady
  (return (and (> (+ (Variables|Default|GetWarmupEnd) (Variables|Default|GetRoundStartDuration)) (GameState|GetServerWorldTimeSeconds)) (Utilities|Name|Equal(Name) (Variables|Default|GetMatchState) "InProgress"))))