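; Battle royale game mode that runs a single free-for-all round without respawns until one player or none remains.
; Tick closes joining near warmup end, resets and starts the round through the spawn manager, activates the circle after a delay and checks living count.
; Deaths update the Countdown, record placement and grant score and reward drops.
; EndRound declares the survivor or a draw; logins after spawning closes are kicked.
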(event EventPostLogin
  (params (NewPlayer :type Player%20Controller%20Object%20Reference))
  (|CallParentFunction NewPlayer)
  (Utilities|IsValid NewPlayer
    (:Is%20Valid
      (bind _asbp_battle_royale_game_state (Utilities|Casting|CastToBP_BattleRoyaleGameState (Game|GetGameState)))
      (if (not (Variables|/Script/Mordhau.MordhauGameState|GetbAllowSpawning _asbp_battle_royale_game_state))
        (Class|MordhauGameSession|KickPlayer (Class|MordhauUtilityLibrary|GetMordhauGameSession) NewPlayer (Utilities|Text|MakeLiteralText "Took too long to load."))))))

(event EventOnKilled
  (params (Killer :type Controller%20Object%20Reference) (KilledPlayer :type Controller%20Object%20Reference) (KilledPawn :type Pawn%20Object%20Reference) (Type :type EMordhauDamageType%20Enum :default "Generic") (SubType :type Byte :default 0) (DamageSource :type Actor%20Object%20Reference) (DamageAgent :type Actor%20Object%20Reference))
  (bind _playerstate (Variables|/Script/Engine.Controller|GetPlayerState KilledPlayer))
  (Utilities|FlowControl|Sequence
    (:then_0
      (if (Variables|Default|GetInitializedMatch)
        (Utilities|IsValid KilledPlayer
          (:Is%20Valid
            (Utilities|FlowControl|Sequence
              (:then_0
                (Utilities|IsValid _playerstate
                  (:Is%20Valid
                    (bind _asbp_battle_royale_game_state (Utilities|Casting|CastToBP_BattleRoyaleGameState (Game|GetGameState)))
                    (bind _returnvalue (Class|MordhauGameState|GetPlayerCountsPerTeam _asbp_battle_royale_game_state true false))
                    (Utilities|FlowControl|Sequence
                      (:then_0
                        (if (!= (Math|Conversions|ToByte(Integer) (Math|Integer|Max(Integer) (- (Utilities|Array|Get(acopy) _returnvalue) 1))) (Variables|/Game/Mordhau/Blueprints/GameModes/BP_BattleRoyaleGameState.BP_BattleRoyaleGameState_C|GetCountdown _asbp_battle_royale_game_state))
                          (Variables|/Game/Mordhau/Blueprints/GameModes/BP_BattleRoyaleGameState.BP_BattleRoyaleGameState_C|SetCountdown _asbp_battle_royale_game_state (Math|Conversions|ToByte(Integer) (Math|Integer|Max(Integer) (- (Utilities|Array|Get(acopy) _returnvalue) 1))))))
                      (:then_1
                        (bind _asbp_battle_royale_player_controller (Utilities|Casting|CastToBP_BattleRoyalePlayerController KilledPlayer))
                        (Variables|/Game/Mordhau/Blueprints/GameModes/BP_BattleRoyalePlayerController.BP_BattleRoyalePlayerController_C|SetPlacementPosition _asbp_battle_royale_player_controller (+ (Variables|/Game/Mordhau/Blueprints/GameModes/BP_BattleRoyaleGameState.BP_BattleRoyaleGameState_C|GetCountdown _asbp_battle_royale_game_state) 1)))
                      (:then_2
                        ;[1 1 1] Reward drop
                        (bind _asbp_mordhau_player_state (Utilities|Casting|CastToBP_MordhauPlayerState _playerstate))
                        (Class|MordhauPlayerState|AddScore _asbp_mordhau_player_state (* (Math|Conversions|ToInteger(Byte) (+ (Variables|/Game/Mordhau/Blueprints/GameModes/BP_BattleRoyaleGameState.BP_BattleRoyaleGameState_C|GetCountdown _asbp_battle_royale_game_state) 1)) 10000))
                        (Class|MordhauGameSession|TriggerRewardDropforPlayer (Class|MordhauUtilityLibrary|GetMordhauGameSession) _asbp_battle_royale_player_controller))))))
              (:then_1
                (Utilities|Array|Add (Variables|Default|GetAlreadyDiedArray) KilledPlayer)))))))
    (:then_1
      (|CallParentFunction Killer KilledPlayer KilledPawn Type SubType DamageSource DamageAgent))))

(event EventBeginPlay
  (|CallParentFunction)
  (Utilities|FlowControl|Sequence
    (:then_0
      (bind _outactors (Actor|GetAllActorsOfClass "/Game/Mordhau/Blueprints/GameModes/BattleRoyale/BP_BattleRoyaleCircle.BP_BattleRoyaleCircle_C"))
      (if (>= (Utilities|Array|Length _outactors) 1)
        (Variables|Default|SetBattleRoyaleCircle (Utilities|Array|Get(acopy) _outactors))))
    (:then_1
      (bind _outactors_2 (Actor|GetAllActorsOfClass "/Game/Mordhau/Blueprints/GameModes/BattleRoyale/BP_BattleRoyaleSpawnManager.BP_BattleRoyaleSpawnManager_C"))
      (if (>= (Utilities|Array|Length _outactors_2) 0)
        (Variables|Default|SetBattleRoyaleSpawnManager (Utilities|Array|Get(acopy) _outactors_2))))))

(event EventTick
  (params (DeltaSeconds :type Float%20%28single-precision%29))
  (bind _returnvalue (Class|MordhauUtilityLibrary|GetMordhauGameSession))
  (bind _battleroyalecircle (Variables|Default|GetBattleRoyaleCircle))
  (bind _asbp_battle_royale_game_state (Utilities|Casting|CastToBP_BattleRoyaleGameState (Game|GetGameState)))
  (Utilities|FlowControl|Sequence
    (:then_0
      (if (or (== (Variables|/Script/Mordhau.MordhauGameState|GetWarmupEnd _asbp_battle_royale_game_state) -1.0) (< (+ (Utilities|Time|GetTimeSeconds) 3e+01) (Variables|/Script/Mordhau.MordhauGameState|GetWarmupEnd _asbp_battle_royale_game_state)))
        (if (not (stale _returnvalue))
          (Class|MordhauGameSession|AllowJoin _returnvalue true))
        (elif (stale _returnvalue)
          (Class|MordhauGameSession|AllowJoin _returnvalue false))))
    (:then_1
      (if (Class|GameMode|IsMatchinProgress)
        (Utilities|FlowControl|Sequence
          (:then_0
            (Utilities|FlowControl|DoOnce false
              (:Completed
                (Variables|Default|SetInitializedMatch true)
                (Utilities|Array|Clear (Variables|Default|GetAlreadyDiedArray))
                (CallFunction|StartRoundStart)
                (CallFunction|StartRound))))
          (:then_1
            (if (< (+ (Variables|/Script/Mordhau.MordhauGameState|GetWarmupEnd _asbp_battle_royale_game_state) (Variables|/Game/Mordhau/Blueprints/GameModes/BP_BattleRoyaleGameState.BP_BattleRoyaleGameState_C|GetRoundStartDuration _asbp_battle_royale_game_state)) (Utilities|Time|GetTimeSeconds))
              (Utilities|FlowControl|Sequence
                (:then_0
                  (Utilities|FlowControl|DoOnce false
                    (:Completed
                      (Utilities|IsValid _battleroyalecircle
                        (:Is%20Valid
                          (Default|ActivateCircle _battleroyalecircle))))))
                (:then_1
                  (bind _returnvalue_2 (Class|MordhauGameState|GetPlayerCountsPerTeam _asbp_battle_royale_game_state true false))
                  (Utilities|FlowControl|Sequence
                    (:then_0
                      (if (!= (Variables|/Game/Mordhau/Blueprints/GameModes/BP_BattleRoyaleGameState.BP_BattleRoyaleGameState_C|GetCountdown _asbp_battle_royale_game_state) (Math|Conversions|ToByte(Integer) (Utilities|Array|Get(acopy) _returnvalue_2)))
                        (Variables|/Game/Mordhau/Blueprints/GameModes/BP_BattleRoyaleGameState.BP_BattleRoyaleGameState_C|SetCountdown _asbp_battle_royale_game_state (Math|Conversions|ToByte(Integer) (Utilities|Array|Get(acopy) _returnvalue_2)))))
                    (:then_1
                      (if (not (or (Variables|/Script/Mordhau.MordhauGameState|GetbAllowSpawning _asbp_battle_royale_game_state) (> (Utilities|Array|Get(acopy) _returnvalue_2) 1)))
                        (CallFunction|EndRound)))))))))))))

(fn ConstructionScript
  (|CallParentFunction))

(fn StartRoundStart
  (bind _asbp_battle_royale_game_state (Utilities|Casting|CastToBP_BattleRoyaleGameState (Game|GetGameState)))
  (Utilities|FlowControl|Sequence
    (:then_0
      (bind _outactors (Actor|GetAllActorsOfClass "/Script/Mordhau.MordhauEquipment"))
      (for _array_element _outactors
        (if (Variables|/Script/Mordhau.MordhauEquipment|GetbAllowCleanup _array_element)
          (Actor|DestroyActor _array_element)))
      (bind _outactors_2 (Actor|GetAllActorsOfClass "/Script/Mordhau.MordhauProjectile"))
      (for _array_element_2 _outactors_2
        (Actor|DestroyActor _array_element_2)))
    (:then_1
      (Utilities|Array|Clear (Variables|Default|GetAlreadyDiedArray))
      (Variables|/Script/Mordhau.MordhauGameState|SetbAllowSpawning _asbp_battle_royale_game_state true)
      (bind _outactors_3 (Actor|GetAllActorsOfClass "/Script/Engine.Controller"))
      (for _array_element_3 _outactors_3
        (bind _asmordhau_player_state (Utilities|Casting|CastToMordhauPlayerState (Variables|/Script/Engine.Controller|GetPlayerState _array_element_3)))
        (if (>= (Variables|/Script/Mordhau.MordhauPlayerState|GetTeam _asmordhau_player_state) 0)
          (CallFunction|UnpossessandDestroyPawn _array_element_3 true))))))

(fn EndRound
  (bind _returnvalue (Game|GetGameState))
  (Utilities|FlowControl|Sequence
    (:then_0
      (bind _asbp_battle_royale_game_state (Utilities|Casting|CastToBP_BattleRoyaleGameState _returnvalue))
      (bind _array_element (Utilities|Array|ForEachLoopwithBreak (Variables|/Script/Engine.GameStateBase|GetPlayerArray _returnvalue) :!label _label)
        (:LoopBody
          (bind _asbp_mordhau_player_state (Utilities|Casting|CastToBP_MordhauPlayerState _array_element))
          (if (Variables|/Script/Mordhau.MordhauPlayerState|GetbIsAlive _asbp_mordhau_player_state)
            (Class|GameMode|EndMatch)
            (Variables|/Game/Mordhau/Blueprints/GameModes/BP_MordhauGameState.BP_MordhauGameState_C|SetMatchEndInfo _asbp_battle_royale_game_state (Utilities|Struct|MakeSTRUCT_MatchEndInfo _asbp_mordhau_player_state))
            (Utilities|FlowControl|Sequence
              (:then_0
                (bind _asbp_mordhau_player_controller (Utilities|Casting|CastToBP_MordhauPlayerController (Components|GetOwner _asbp_mordhau_player_state)))
                ;[1 1 1] Trigger reward drop
                (Class|MordhauPlayerState|AddScore _asbp_mordhau_player_state 10000)
                (Class|MordhauGameSession|TriggerRewardDropforPlayer (Class|MordhauUtilityLibrary|GetMordhauGameSession) _asbp_mordhau_player_controller))
              (:then_1
                (LocalVariables|SetFoundLiving true)
                (goto _label Break)))))
        (:Completed
          (if (not (LocalVariables|GetFoundLiving))
            (Class|GameMode|EndMatch)
            (Variables|/Game/Mordhau/Blueprints/GameModes/BP_MordhauGameState.BP_MordhauGameState_C|SetMatchEndInfo _asbp_battle_royale_game_state (Utilities|Struct|MakeSTRUCT_MatchEndInfo 0 0 0.0 0.0 true))))))
    (:then_1
      (Variables|Default|SetbIsScoringDisabled true))))

(fn MoreThanOnePlayerAlive
  (bind _asbp_battle_royale_game_state (Utilities|Casting|CastToBP_BattleRoyaleGameState (Game|GetGameState)))
  (if (Variables|/Script/Mordhau.MordhauGameState|GetbAllowSpawning _asbp_battle_royale_game_state)
    (return true)
    (else
      (bind _returnvalue (Class|MordhauGameState|GetPlayerCountsPerTeam _asbp_battle_royale_game_state true false))
      (return (> (Utilities|Array|Get(acopy) _returnvalue) 1)))))

(fn ControllerCanRestart
  (params (Controller :type Controller%20Object%20Reference))
  (bind _returnvalue (|CallParentFunction Controller))
  (return (and _returnvalue (or (not (Utilities|Array|ContainsItem (Variables|Default|GetAlreadyDiedArray) Controller)) (not (Class|GameMode|IsMatchinProgress))))))

(fn StartRound
  (bind _battleroyalespawnmanager (Variables|Default|GetBattleRoyaleSpawnManager))
  (Utilities|FlowControl|Sequence
    (:then_0
      (Utilities|IsValid _battleroyalespawnmanager
        (:Is%20Valid
          (Default|ActivateSpawns _battleroyalespawnmanager))))
    (:then_1
      (Variables|Default|SetbIsScoringDisabled false)
      (bind _asbp_battle_royale_game_state (Utilities|Casting|CastToBP_BattleRoyaleGameState (Game|GetGameState)))
      (Variables|/Script/Mordhau.MordhauGameState|SetbAllowSpawning _asbp_battle_royale_game_state false)
      (Utilities|Array|Clear (Variables|Default|GetAlreadyDiedArray))
      (bind _returnvalue (Class|MordhauGameState|GetPlayerCountsPerTeam _asbp_battle_royale_game_state false false)) ; Don't use living because they'll spawn next frame
      (Variables|/Game/Mordhau/Blueprints/GameModes/BP_BattleRoyaleGameState.BP_BattleRoyaleGameState_C|SetCountdown _asbp_battle_royale_game_state (Math|Conversions|ToByte(Integer) (Utilities|Array|Get(acopy) _returnvalue))))))