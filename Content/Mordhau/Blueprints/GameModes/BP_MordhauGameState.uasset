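; Base Mordhau game state that drives match announcements, post-match screens, scoreboard data, killfeed and player vote kicks.
; Tick runs one-time ammo box and equipment cleanup, then updates the local HUD from MatchState.
; Kills resolve projectiles to their creator and replicate to update killfeed, nemesis counters and a fire bomb stat workaround.
; Vote kicks have cooldown, timed tally, quorum and temporary ban, with RepNotify toggling the vote menu for eligible players.
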(event Custom|ShowScoreboardDelayed
  (bind _returnvalue (Game|GetPlayerController 0))
  (Utilities|FlowControl|Delay 6.5)
  (if (and (Pawn|IsLocalPlayerController _returnvalue) (not (Variables|Default|GetbDisableScoreboard)))
    (bind _asbp_mordhau_player_controller (Utilities|Casting|CastToBP_MordhauPlayerController _returnvalue))
    (Default|ShowScoreboard (Variables|/Game/Mordhau/Blueprints/BP_MordhauPlayerController.BP_MordhauPlayerController_C|GetHUD _asbp_mordhau_player_controller))))

(event Custom|OnRequestedVoteKick
  (params (Initiator :type Mordhau%20Player%20State%20Object%20Reference) (Target :type Mordhau%20Player%20State%20Object%20Reference))
  (bind _returnvalue (Utilities|Time|GetRealTimeSeconds))
  (Utilities|IsValid Target
    (:Is%20Valid
      (bind _asbp_mordhau_player_controller (Utilities|Casting|CastToBP_MordhauPlayerController (Components|GetOwner Target)))
      (bind _asbp_mordhau_player_controller_2 (Utilities|Casting|CastToBP_MordhauPlayerController (Components|GetOwner Initiator)))
      (if (or (== Initiator Target) (Variables|/Script/Mordhau.MordhauPlayerState|GetbIsAdmin Target))
        (Class|MordhauPlayerController|ClientMessageBP _asbp_mordhau_player_controller_2 "Cannot start vote against that player.")
        (elif (Variables|Default|GetIsVoteOngoing)
          (Class|MordhauPlayerController|ClientMessageBP _asbp_mordhau_player_controller_2 "Vote already in progress.")
          (elif (< (+ (Variables|/Game/Mordhau/Blueprints/BP_MordhauPlayerController.BP_MordhauPlayerController_C|GetLastVoteKickStartTime _asbp_mordhau_player_controller_2) 1.8e+02) _returnvalue)
            (Variables|/Game/Mordhau/Blueprints/BP_MordhauPlayerController.BP_MordhauPlayerController_C|SetLastVoteKickStartTime _asbp_mordhau_player_controller_2 _returnvalue)
            (Variables|Default|SetVoteKickInfo (Utilities|Struct|MakeSTRUCT_VoteKickInfo Target Initiator "NewEnumerator4" (select (> (Variables|/Script/Mordhau.MordhauPlayerController|GetTotalMordhauCharacterDamage _asbp_mordhau_player_controller) 1.5e+02) (Math|Conversions|ToByte(Integer) (Math|Float|Round (Math|Float|Clamp(Float) (* (/ (Variables|/Script/Mordhau.MordhauPlayerController|GetTotalMordhauCharacterTeamDamage _asbp_mordhau_player_controller) (Variables|/Script/Mordhau.MordhauPlayerController|GetTotalMordhauCharacterDamage _asbp_mordhau_player_controller)) 1e+02) 0.0 1e+02))) 0)))
            (Variables|Default|SetIsVoteOngoing true)
            (Variables|Default|SetVoteYesVotes 0)
            (Variables|Default|SetVoteNoVotes 0)
            (Utilities|Set|Clear (Variables|Default|GetVoters))
            (CallFunction|TallyVoteKickVotes)
            (else
              (Class|MordhauPlayerController|ClientMessageBP _asbp_mordhau_player_controller_2 "Too soon after last vote."))))))))

(event Custom|TallyVoteKickVotes
  (bind _voteyesvotes (Variables|Default|GetVoteYesVotes))
  (bind _votenovotes (Variables|Default|GetVoteNoVotes))
  (bind _returnvalue (+ _voteyesvotes _votenovotes))
  (Utilities|FlowControl|RetriggerableDelay 3e+01)
  (if (Variables|Default|GetIsVoteOngoing)
    (if (>= _returnvalue (Math|Integer|Max(Integer) (Math|Float|Truncate (* (Utilities|Array|Length (Variables|Default|GetPlayerArray)) (select (Variables|Default|GetbIsTeamMode) 0.2 0.4))) 4))
      (if (> (/ (Math|Conversions|ToFloat(Integer) (Variables|Default|GetVoteYesVotes)) (Math|Conversions|ToFloat(Integer) _returnvalue)) 0.6)
        (Utilities|IsValid (.Target (Utilities|Struct|BreakSTRUCT_VoteKickInfo (Variables|Default|GetVoteKickInfo)))
          (:Is%20Valid
            (CallFunction|FinishVoteKick "NewEnumerator3"))
          (:Is%20Not%20Valid
            (CallFunction|FinishVoteKick "NewEnumerator2" :!label _label)))
        (else
          (goto _label)))
      (else
        (CallFunction|FinishVoteKick "NewEnumerator1")))))

(event Custom|OnRequestedVoteCancel
  (params (Initiator :type Mordhau%20Player%20State%20Object%20Reference))
  (if (Variables|Default|GetIsVoteOngoing)
    (if (or (Variables|/Script/Mordhau.MordhauPlayerState|GetbIsAdmin Initiator) (== Initiator (.Initiator (Utilities|Struct|BreakSTRUCT_VoteKickInfo (Variables|Default|GetVoteKickInfo)))))
      (CallFunction|FinishVoteKick "NewEnumerator0"))))

(event Custom|OnVoteKickVote
  (params (Controller :type Player%20Controller%20Object%20Reference) (VotedYes :type Boolean))
  (bind _voters (Variables|Default|GetVoters))
  (if (Variables|Default|GetIsVoteOngoing)
    (if (not (Utilities|Set|Contains _voters Controller))
      (Utilities|Set|Add _voters Controller)
      (if VotedYes
        (Math|Integer|IncrementInt (Variables|Default|GetVoteYesVotes))
        (else
          (Math|Integer|IncrementInt (Variables|Default|GetVoteNoVotes)))))))

(event Custom|ReplicatedKillNotify
  (params (Killer :type Player%20State%20Object%20Reference) (Killed :type Player%20State%20Object%20Reference) (Weapon :type Actor%20Class%20Reference) (Flags :type Byte))
  (bind _returnvalue (Class|MordhauUtilityLibrary|GetMordhauStats))
  (CallFunction|ReceiveKillNotify Killer Killed Weapon Flags)
  (Utilities|IsValid Killer
    (:Is%20Valid
      (bind _asplayer_controller (Utilities|Casting|CastToPlayerController (Components|GetOwner Killer)))
      ;[1 1 1] Hack to fix fire bomb stat tracking :(
      (if (Pawn|IsLocalPlayerController _asplayer_controller)
        (if (Utilities|ClassIsChildOf Weapon "/Game/Mordhau/Blueprints/Equipment/Thrown/BP_FireBomb.BP_FireBomb_C")
          (Class|MordhauStats|IncrementIntStatValueChecked _returnvalue (Class|MordhauUtilityLibrary|GetWorldOf self) (Variables|/Script/Mordhau.MordhauStats|GetFireKills _returnvalue)))))))

(event EventTick
  (params (DeltaSeconds :type Float%20%28single-precision%29))
  (bind _returnvalue (Game|GetPlayerController 0))
  (bind _returnvalue_2 (GameState|GetServerWorldTimeSeconds))
  (bind _warmupend (Variables|Default|GetWarmupEnd))
  (bind _returnvalue_3 (- _warmupend _returnvalue_2))
  (bind _returnvalue_4 (Math|Float|Max(Float) _returnvalue_3 0.0))
  (bind _returnvalue_5 (Math|Float|Ceil _returnvalue_4))
  (Utilities|FlowControl|Sequence
    (:then_0
      (Utilities|FlowControl|DoOnce false
        (:Completed
          (Utilities|FlowControl|Delay 0.05)
          (Utilities|FlowControl|Sequence
            (:then_0
              (if (Variables|Default|GetNoAmmoBoxes)
                (bind _outactors (Actor|GetAllActorsOfClass "/Game/Mordhau/Blueprints/Interactables/Environment/Specific/BP_AmmoBox.BP_AmmoBox_C"))
                (for _array_element _outactors
                  (Actor|DestroyActor _array_element))))
            (:then_1
              (Networking|SwitchHasAuthority
                (:Authority
                  (if (Variables|Default|GetNoPreplacedEquipment)
                    (bind _outactors_2 (Actor|GetAllActorsOfClass "/Script/Mordhau.MordhauEquipment"))
                    (for _array_element_2 _outactors_2
                      (Actor|DestroyActor _array_element_2))))))))))
    (:then_1
      (bind _asbp_mordhau_player_controller (Utilities|Casting|CastToBP_MordhauPlayerController _returnvalue))
      (if (Pawn|IsLocalPlayerController _returnvalue)
        (bind _asbp_mordhau_hud (Utilities|Casting|CastToBP_MordhauHUD (HUD|GetHUD _returnvalue)))
        (switch name (Variables|Default|GetMatchState)
          (:WaitingToStart
            ;[1 1 1] WaitingToStart
            (Utilities|Casting|CastToAdvancedCharacter (Pawn|GetControlledPawn _returnvalue))
            (if (!= _warmupend -1.0)
              (if (!= _returnvalue_5 0)
                (Default|ShowAnnouncement _asbp_mordhau_hud "Match starting" (Utilities|Text|FormatText "-{0}-" _returnvalue_5) 0.1))
              (else
                (Default|ShowAnnouncement _asbp_mordhau_hud "Waiting for players" "" 0.1))))
          (:WaitingPostMatch
            ;[1 1 1] WaitingPostMatch
            (Utilities|FlowControl|DoOnce (Variables|Default|GetbDoNotGoToNextMapOnMatchEnd)
              (:Completed
                (if (not (Variables|Default|GetbDoNotShowPostMatchScreen))
                  (Utilities|FlowControl|Delay (Variables|Default|GetPostMatchScreenDelay))
                  (Default|HideScoreboard _asbp_mordhau_hud)
                  (bind _asbp_mordhau_hud_2 (Utilities|Casting|CastToBP_MordhauHUD (HUD|GetHUD _asbp_mordhau_player_controller)))
                  (Default|ShowPostMatchScreen _asbp_mordhau_hud_2))))))))))

(fn ConstructionScript)

(fn GetScoreboardTime
  (switch name (Variables|Default|GetMatchState)
    (:Default
      (return (Math|Timespan|MakeTimespan 0)))
    (:InProgress
      (return (CallFunction|GetScoreboardTimeinProgress)))
    (:WaitingPostMatch
      (return (Math|Timespan|FromSeconds (Math|Conversions|ToFloat(Integer) (Math|Float|Ceil (Math|Float|Max(Float) (- (Variables|Default|GetEndMatchMapChangeEnd) (GameState|GetServerWorldTimeSeconds)) 0.0))))))
    (:WaitingToStart
      (return (Math|Timespan|FromSeconds (Math|Conversions|ToFloat(Integer) (Math|Float|Ceil (Math|Float|Max(Float) (- (Variables|Default|GetWarmupEnd) (GameState|GetServerWorldTimeSeconds)) 0.0))))))))

(fn GetScoreboardTimeinProgress
  (bind _matchdurationmax (Variables|Default|GetMatchDurationMax))
  (if (> _matchdurationmax 0)
    (return (Math|Timespan|FromSeconds (Math|Conversions|ToFloat(Integer) (Math|Integer|Max(Integer) (- _matchdurationmax (Variables|Default|GetElapsedTime))))))
    (else
      (return (Math|Timespan|MakeTimespan 200)))))

(fn GetScoreboardObjectiveName
  (return "Score"))

(fn GetScoreboardTeamObjectiveValue
  (params (Team :type Integer))
  (bind _teamscores (Variables|Default|GetTeamScores))
  (if (Utilities|Array|IsValidIndex _teamscores Team)
    (return (Utilities|String|ToString(Integer) (Math|Float|Floor (Utilities|Array|Get(acopy) _teamscores Team))))
    (else
      (return "0"))))

(fn OnRepMatchEndInfo
  (if (not (Variables|Default|GetMatchEndInfoReplicated))
    (Variables|Default|SetMatchEndInfoReplicated true)
    (CallFunction|HandleMatchEndInfo)))

(fn HandleMatchEndInfo
  (bind _returnvalue (Game|GetPlayerController 0))
  (if (Pawn|IsLocalPlayerController _returnvalue)
    (bind _asbp_mordhau_player_controller (Utilities|Casting|CastToBP_MordhauPlayerController _returnvalue))
    (Default|HideSpawnScreen (Variables|/Game/Mordhau/Blueprints/BP_MordhauPlayerController.BP_MordhauPlayerController_C|GetHUD _asbp_mordhau_player_controller))
    (CallFunction|ShowScoreboardDelayed)))

(fn GetKillfeedColor
  (params (PlayerState :type Player%20State%20Object%20Reference))
  (bind _returnvalue (Game|GetPlayerController 0))
  (if (and (Pawn|IsLocalPlayerController _returnvalue) (== (Variables|/Script/Engine.Controller|GetPlayerState _returnvalue) PlayerState))
    (return "(R=1.000000,G=0.874510,B=0.258824,A=1.000000)")
    (else
      (if (Variables|Default|GetbIsTeamMode)
        (bind _asmordhau_player_state (Utilities|Casting|CastToMordhauPlayerState PlayerState)
          (:then
            (switch int (Variables|/Script/Mordhau.MordhauPlayerState|GetTeam _asmordhau_player_state)
              (:Default
                _)
              (:0
                (return "(R=1.000000,G=0.274510,B=0.219608,A=1.000000)"))
              (:1
                (return "(R=0.219608,G=0.494118,B=1.000000,A=1.000000)"))))
          (:CastFailed
            _)))
      (return "(R=0.509804,G=0.454902,B=0.325490,A=1.000000)"))))

(fn GetChatColor
  (params (PlayerState :type Player%20State%20Object%20Reference))
  (bind _returnvalue (Game|GetPlayerController 0))
  (if (and (Pawn|IsLocalPlayerController _returnvalue) (== (Variables|/Script/Engine.Controller|GetPlayerState _returnvalue) PlayerState))
    (return "(R=1.000000,G=0.874510,B=0.258824,A=1.000000)")
    (else
      (if (Variables|Default|GetbIsTeamMode)
        (bind _asmordhau_player_state (Utilities|Casting|CastToMordhauPlayerState PlayerState)
          (:then
            (switch int (Variables|/Script/Mordhau.MordhauPlayerState|GetTeam _asmordhau_player_state)
              (:Default
                _)
              (:0
                (return "(R=1.000000,G=0.274510,B=0.219608,A=1.000000)"))
              (:1
                (return "(R=0.219608,G=0.494118,B=1.000000,A=1.000000)"))))
          (:CastFailed
            _)))
      (return "(R=0.509804,G=0.454902,B=0.325490,A=1.000000)"))))

(fn AddKillNotify
  (params (Killer :type Player%20State%20Object%20Reference) (Killed :type Player%20State%20Object%20Reference) (Weapon :type Actor%20Object%20Reference) (DamageType :type EMordhauDamageType%20Enum :default "Generic"))
  (LocalVariables|SetWeaponToUse Weapon)
  (Utilities|FlowControl|Sequence
    (:then_0
      (bind _asmordhau_projectile (Utilities|Casting|CastToMordhauProjectile Weapon))
      (bind _returnvalue (Class|MordhauProjectile|GetProjectileCreator _asmordhau_projectile))
      (Utilities|IsValid _returnvalue
        (:Is%20Valid
          (LocalVariables|SetWeaponToUse _returnvalue))))
    (:then_1
      (Utilities|IsValid (LocalVariables|GetWeaponToUse)
        (:Is%20Valid
          (LocalVariables|SetWeaponClass (Utilities|GetClass (LocalVariables|GetWeaponToUse))))
        (:Is%20Not%20Valid
          _))
      (Utilities|FlowControl|Sequence
        (:then_0
          (if (Utilities|Enum|Equal(Enum) DamageType "Fall")
            (LocalVariables|SetFlags 2)
            (else
              (Utilities|Casting|CastToKickWeapon (LocalVariables|GetWeaponToUse))
              (LocalVariables|SetFlags 1))))
        (:then_1
          (CallFunction|ReplicatedKillNotify Killer Killed (LocalVariables|GetWeaponClass) (LocalVariables|GetFlags)))))))

(fn ReceiveKillNotify
  (params (Killer :type Player%20State%20Object%20Reference) (Killed :type Player%20State%20Object%20Reference) (Weapon :type Actor%20Class%20Reference) (Flags :type Byte))
  (bind _returnvalue (Class|MordhauUtilityLibrary|GetDefaultActor Weapon))
  (bind _asbp_mordhau_player_controller (Utilities|Casting|CastToBP_MordhauPlayerController (Game|GetPlayerController 0)))
  (if (Pawn|IsLocalPlayerController _asbp_mordhau_player_controller)
    (bind _asmordhau_player_state (Utilities|Casting|CastToMordhauPlayerState (Variables|/Script/Engine.Controller|GetPlayerState _asbp_mordhau_player_controller)))
    (bind _asmordhau_player_state_2 (Utilities|Casting|CastToMordhauPlayerState Killer))
    (bind _asmordhau_player_state_3 (Utilities|Casting|CastToMordhauPlayerState Killed))
    (Utilities|FlowControl|Sequence
      (:then_0
        (switch int (Math|Conversions|ToInteger(Byte) Flags)
          (:Default
            (bind _asmordhau_equipment (Utilities|Casting|CastToMordhauEquipment _returnvalue :!label _label)
              (:then
                (LocalVariables|SetKilledWith (Variables|/Script/Mordhau.MordhauEquipment|GetEquipmentName _asmordhau_equipment)))
              (:CastFailed
                (bind _asmordhau_vehicle (Utilities|Casting|CastToMordhauVehicle _returnvalue)
                  (:then
                    (LocalVariables|SetKilledWith (Variables|/Script/Mordhau.MordhauVehicle|GetVehicleName _asmordhau_vehicle)))
                  (:CastFailed
                    (bind _asmordhau_projectile (Utilities|Casting|CastToMordhauProjectile _returnvalue)
                      (:then
                        (LocalVariables|SetKilledWith (Variables|/Script/Mordhau.MordhauProjectile|GetProjectileName _asmordhau_projectile)))
                      (:CastFailed
                        (LocalVariables|SetKilledWith "RIP"))))))))
          (:0
            (goto _label))
          (:1
            (LocalVariables|SetKilledWith "Kick"))
          (:2
            (LocalVariables|SetKilledWith "Fall"))))
      (:then_1
        (Default|SendMessagetoKillFeed (Variables|/Game/Mordhau/Blueprints/BP_MordhauPlayerController.BP_MordhauPlayerController_C|GetHUD _asbp_mordhau_player_controller) Killer (LocalVariables|GetKilledWith) Killed)
        (if (and (== _asmordhau_player_state _asmordhau_player_state_2) (not (== _asmordhau_player_state _asmordhau_player_state_3)))
          (Variables|/Script/Mordhau.MordhauPlayerState|SetKilledByLocalPlayerCounter _asmordhau_player_state_3 (+ (Variables|/Script/Mordhau.MordhauPlayerState|GetKilledByLocalPlayerCounter _asmordhau_player_state_3) 1))
          (elif (and (== _asmordhau_player_state _asmordhau_player_state_3) (not (== _asmordhau_player_state _asmordhau_player_state_2)))
            (Variables|/Script/Mordhau.MordhauPlayerState|SetKilledLocalPlayerCounter _asmordhau_player_state_2 (+ (Variables|/Script/Mordhau.MordhauPlayerState|GetKilledLocalPlayerCounter _asmordhau_player_state_2) 1))
            (Default|ShowKilledby (Variables|/Game/Mordhau/Blueprints/BP_MordhauPlayerController.BP_MordhauPlayerController_C|GetHUD _asbp_mordhau_player_controller) _asmordhau_player_state_2)))))))

(fn ShouldHideSpawnInfoText
  (return (not (Variables|Default|GetbAllowSpawning))))

(fn OnRepVoteKickInfo
  (bind _returnvalue (Game|GetPlayerController 0))
  (bind _votekickinfo (Variables|Default|GetVoteKickInfo))
  (bind (_target _initiator _result) (Utilities|Struct|BreakSTRUCT_VoteKickInfo _votekickinfo))
  (bind _playerstate (Variables|/Script/Engine.Controller|GetPlayerState _returnvalue))
  (bind _asbp_mordhau_hud (Utilities|Casting|CastToBP_MordhauHUD (Class|MordhauUtilityLibrary|GetMordhauHUD)))
  (if (Utilities|Enum|Equal(Enum) _result "NewEnumerator4")
    (Utilities|IsValid _target
      (:Is%20Valid
        (bind _asbp_mordhau_game_state (Utilities|Casting|CastToBP_MordhauGameState (Game|GetGameState)))
        (bind _asmordhau_player_state (Utilities|Casting|CastToMordhauPlayerState _playerstate))
        (if (and (Math|Boolean|ORBoolean (not (Variables|/Script/Mordhau.MordhauGameState|GetbIsTeamMode _asbp_mordhau_game_state)) (Class|MordhauUtilityLibrary|IsFriendlytoLocalPlayer (Class|MordhauUtilityLibrary|GetWorldOf self) _target) (== _playerstate _target)) (!= (Variables|/Script/Mordhau.MordhauPlayerState|GetTeam _asmordhau_player_state) -1))
          (Default|ShowVoteKickMenu _asbp_mordhau_hud))))
    (else
      (Default|HideVoteKickMenu _asbp_mordhau_hud))))

(fn FinishVoteKick
  (params (Result :type E_VoteKickResult%20Enum :default "NewEnumerator4"))
  (Utilities|FlowControl|Sequence
    (:then_0
      (if (Utilities|Enum|Equal(Enum) Result "NewEnumerator3")
        (Class|MordhauPlayerState|BanPlayer (.Target (Utilities|Struct|BreakSTRUCT_VoteKickInfo (Variables|Default|GetVoteKickInfo))) 10 (Utilities|String|ToString(Text) (Utilities|Text|MakeLiteralText "Vote kick")))))
    (:then_1
      (Variables|Default|SetIsVoteOngoing false)
      (Variables|Default|SetVoteKickInfo (Utilities|Struct|MakeSTRUCT_VoteKickInfo 0 0 Result)))))