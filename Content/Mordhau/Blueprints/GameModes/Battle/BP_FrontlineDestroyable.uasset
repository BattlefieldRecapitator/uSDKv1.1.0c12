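; Destroyable Frontline objective tied to a capture point, reporting weighted progress from lost health.
; Enemy prerequisites toggle damageability and the floating health widget; hits are capped, and owning-team player damage is blocked until objectives complete, except from circle saws.
; Replicated health changes update the widget, award objective score to the last damaging player, and notify the capture point.
; The widget hides once objectives complete or health reaches zero; team tinting is disconnected.
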(event EventBeginPlay
  (bind _mordhauwidget (Variables|Default|GetMordhauWidget))
  (|CallParentFunction)
  (Utilities|IsValid _mordhauwidget
    (:Is%20Valid
      (bind _asbp_destroyable_widget_floater (Utilities|Casting|CastToBP_DestroyableWidgetFloater (UserInterface|GetUserWidgetObject _mordhauwidget)))
      (Default|UpdateHealth _asbp_destroyable_widget_floater (Math|Conversions|ToFloat(Byte) (Variables|Default|GetReplicatedHealth)))
      (CallFunction|UpdateUIWidgets))))

(event Game|Damage|EventAnyDamage
  (params (Damage :type Float%20%28single-precision%29) (DamageType :type Damage%20Type%20Object%20Reference) (InstigatedBy :type Controller%20Object%20Reference) (DamageCauser :type Actor%20Object%20Reference))
  (bind _damagefactor (Variables|Default|GetDamageFactor))
  (bind _capturepoint (Variables|Default|GetCapturePoint))
  (if (Variables|Default|GetbCanBeDamaged)
    (Utilities|FlowControl|Sequence
      (:then_0
        (bind _asmordhau_player_controller (Utilities|Casting|CastToMordhauPlayerController InstigatedBy)
          (:then
            (Variables|Default|SetLastDamagedByPlayerController _asmordhau_player_controller))
          (:CastFailed
            (Variables|Default|SetLastDamagedByPlayerController 0))))
      (:then_1
        (Utilities|IsValid _capturepoint
          (:Is%20Valid
            (if (Variables|/Game/Mordhau/Blueprints/GameModes/Battle/BP_CapturePoint.BP_CapturePoint_C|GetObjectivesCompleted _capturepoint)
              (|CallParentFunction (Math|Float|Min(Float) Damage (select (Math|Float|NearlyEqual(Float) _damagefactor 0.0 1e-06) 0.0 (* (/ 1.0 _damagefactor) (Variables|Default|GetMaxDamagePerHit)))) DamageType InstigatedBy DamageCauser :!label _label)
              (else
                (Utilities|Casting|CastToBP_CircleSawProgressActor DamageCauser
                  (:then
                    (goto _label))
                  (:CastFailed
                    (Utilities|IsValid InstigatedBy
                      (:Is%20Valid
                        (bind _asmordhau_player_state (Utilities|Casting|CastToMordhauPlayerState (Variables|/Script/Engine.Controller|GetPlayerState InstigatedBy))
                          (:then
                            (if (not (== (Variables|/Script/Mordhau.MordhauPlayerState|GetTeam _asmordhau_player_state) (Math|Conversions|ToInteger(Byte) (Variables|/Script/Mordhau.ControlPoint|GetOwningTeam _capturepoint))))
                              (goto _label)))
                          (:CastFailed
                            (goto _label))))
                      (:Is%20Not%20Valid
                        (goto _label))))))))
          (:Is%20Not%20Valid
            (goto _label)))))))

(event EventOnEnemyGainedPrerequisites
  (CallFunction|EnemyGainedPrerequisites))

(event EventOnEnemyLostPrerequisites
  (CallFunction|EnemyLostPrerequisites))

(event EventOnReplicatedHealthChanged
  (bind _capturepoint (Variables|Default|GetCapturePoint))
  (bind _scoreawardedperdestroy (Variables|Default|GetScoreAwardedPerDestroy))
  (bind _lastreplicatedhealth (Variables|Default|GetLastReplicatedHealth))
  (bind _replicatedhealth (Variables|Default|GetReplicatedHealth))
  (bind _scoredamagemultiplier (Variables|Default|GetScoreDamageMultiplier))
  (bind _replicatedhealth_2 (Variables|Default|GetReplicatedHealth))
  (bind _mordhauwidget (Variables|Default|GetMordhauWidget))
  (bind _mordhauwidget_2 (Variables|Default|GetMordhauWidget))
  (bind _lastdamagedbyplayercontroller (Variables|Default|GetLastDamagedByPlayerController))
  (bind _returnvalue (Math|Conversions|ToFloat(Byte) _lastreplicatedhealth))
  (bind _returnvalue_2 (Math|Conversions|ToFloat(Byte) _replicatedhealth))
  (bind _returnvalue_3 (== _replicatedhealth_2 0))
  (bind _returnvalue_4 (- _returnvalue _returnvalue_2))
  (bind _returnvalue_5 (* _returnvalue_4 _scoredamagemultiplier))
  (bind _returnvalue_6 (Math|Float|Truncate _returnvalue_5))
  (Utilities|FlowControl|Sequence
    (:then_0
      (Utilities|IsValid _mordhauwidget_2
        (:Is%20Valid
          (Utilities|FlowControl|Sequence
            (:then_0
              (if _returnvalue_3
                (Variables|/Script/Mordhau.MordhauWidgetComponent|SetbIsSlowHideOverride _mordhauwidget true)
                (Variables|/Script/Mordhau.MordhauWidgetComponent|SetOverrideVisible _mordhauwidget 0)
                (Variables|/Script/Mordhau.MordhauWidgetComponent|SetVisibilityWeightInterpolationSpeed _mordhauwidget 1.0)
                (Utilities|FlowControl|Delay 1.0)
                (Utilities|IsValid _mordhauwidget
                  (:Is%20Valid
                    (Components|DestroyComponent _mordhauwidget)))))
            (:then_1
              (bind _asbp_destroyable_widget_floater (Utilities|Casting|CastToBP_DestroyableWidgetFloater (UserInterface|GetUserWidgetObject _mordhauwidget_2)))
              (Default|UpdateHealth _asbp_destroyable_widget_floater (Math|Conversions|ToFloat(Byte) _replicatedhealth_2)))))))
    (:then_1
      (Utilities|IsValid _lastdamagedbyplayercontroller
        (:Is%20Valid
          (Utilities|FlowControl|Sequence
            (:then_0
              (if (> _returnvalue_6 0)
                (Class|MordhauPlayerController|GiveClientScoreBP _lastdamagedbyplayercontroller "Objective" _returnvalue_6)))
            (:then_1
              (if _returnvalue_3
                (if (> _scoreawardedperdestroy 0)
                  (Class|MordhauPlayerController|GiveClientScoreBP _lastdamagedbyplayercontroller "Objective" _scoreawardedperdestroy))))))))
    (:then_2
      (Utilities|IsValid _capturepoint
        (:Is%20Valid
          (Default|ObjectivesChanged _capturepoint))))
    (:then_3
      (if _returnvalue_3
        (Utilities|IsValid (Variables|Default|GetFinalMeshChangeParticle)
          (:Is%20Valid
            (Variables|Default|SetDamageMeshChangeParticle (Variables|Default|GetFinalMeshChangeParticle))))))))

(event EventOnUpdateUIWidgets
  (CallFunction|UpdateUIWidgets))

(event EventOnInitialize
  (params (Point :type BP%20Capture%20Point%20Object%20Reference))
  (CallFunction|Initialize Point))

(event EventOnAnyObjectiveProgressChanged
  (bind _mordhauwidget (Variables|Default|GetMordhauWidget))
  (bind _capturepoint (Variables|Default|GetCapturePoint))
  (Utilities|IsValid _capturepoint
    (:Is%20Valid
      (if (== (Variables|/Game/Mordhau/Blueprints/GameModes/Battle/BP_CapturePoint.BP_CapturePoint_C|GetObjectiveProgress _capturepoint) 1.0)
        (Variables|Default|SetCapturePointObjectivesCompleted true)
        (Variables|Default|SetScoreAwardedPerDestroy 0)
        (Utilities|IsValid _mordhauwidget
          (:Is%20Valid
            (Variables|/Script/Mordhau.MordhauWidgetComponent|SetOverrideVisible _mordhauwidget 0)))))))

(fn ConstructionScript
  (|CallParentFunction))

(fn Initialize
  (params (InCapturePoint :type BP%20Capture%20Point%20Object%20Reference))
  (Variables|Default|SetCapturePoint InCapturePoint))

(fn EnemyGainedPrerequisites
  (bind _mordhauwidget (Variables|Default|GetMordhauWidget))
  (Utilities|FlowControl|Sequence
    (:then_0
      (Variables|Default|SetbCanBeDamaged true)
      (Utilities|IsValid _mordhauwidget
        (:Is%20Valid
          (if (not (Variables|Default|GetCapturePointObjectivesCompleted))
            (Variables|/Script/Mordhau.MordhauWidgetComponent|SetOverrideVisible _mordhauwidget -1)))))
    (:then_1
      (CallFunction|UpdateUIWidgets))))

(fn EnemyLostPrerequisites
  (bind _mordhauwidget (Variables|Default|GetMordhauWidget))
  (Utilities|FlowControl|Sequence
    (:then_0
      (Variables|Default|SetbCanBeDamaged false)
      (Utilities|IsValid _mordhauwidget
        (:Is%20Valid
          (Variables|/Script/Mordhau.MordhauWidgetComponent|SetOverrideVisible _mordhauwidget 0))))
    (:then_1
      (CallFunction|UpdateUIWidgets))))

(fn UpdateUIWidgets
  (bind _slatebrush (Utilities|Struct|MakeSlateBrush "(X=30.000000,Y=38.000000)" "(Left=0.000000,Top=0.000000,Right=0.000000,Bottom=0.000000)" "(SpecifiedColor=(R=1.000000,G=1.000000,B=1.000000,A=1.000000),ColorUseRule=UseColor_Specified)" "/Game/Mordhau/UI/UIAssets/Textures/ic_strike.ic_strike" "Image" "NoTile" "NoMirror"))
  (bind _slatebrush_2 (Utilities|Struct|MakeSlateBrush "(X=36.000000,Y=40.000000)" "(Left=0.000000,Top=0.000000,Right=0.000000,Bottom=0.000000)" "(SpecifiedColor=(R=1.000000,G=1.000000,B=1.000000,A=1.000000),ColorUseRule=UseColor_Specified)" "/Game/Mordhau/UI/UIAssets/Textures/ic_defence_lvl1.ic_defence_lvl1" "Image" "NoTile" "NoMirror"))
  (bind _capturepoint (Variables|Default|GetCapturePoint))
  (bind _mordhauwidget (Variables|Default|GetMordhauWidget))
  (Utilities|IsValid (Game|GetPlayerController 0)
    (:Is%20Valid
      (Utilities|IsValid _capturepoint
        (:Is%20Valid
          (if (not (== (Variables|/Game/Mordhau/Blueprints/GameModes/Battle/BP_CapturePoint.BP_CapturePoint_C|GetObjectiveProgress _capturepoint) 1.0))
            (Utilities|IsValid _mordhauwidget
              (:Is%20Valid
                (bind _asbp_destroyable_widget_floater (Utilities|Casting|CastToBP_DestroyableWidgetFloater (UserInterface|GetUserWidgetObject _mordhauwidget)))
                (bind _asmordhau_game_state (Utilities|Casting|CastToMordhauGameState (Game|GetGameState)))
                (bind _asmordhau_player_state (Utilities|Casting|CastToMordhauPlayerState (Variables|/Script/Engine.Controller|GetPlayerState (Game|GetPlayerController 0))))
                (if (== (Variables|/Script/Mordhau.ControlPoint|GetOwningTeam _capturepoint) (Math|Conversions|ToByte(Integer) (Variables|/Script/Mordhau.MordhauPlayerState|GetTeam _asmordhau_player_state)))
                  (Variables|/Script/UMG.ProgressBar|SetWidgetStyle (Variables|/Game/Mordhau/Blueprints/GameModes/Battle/BP_DestroyableWidgetFloater.BP_DestroyableWidgetFloater_C|GetProgressBar_0 _asbp_destroyable_widget_floater) (Utilities|Struct|MakeProgressBarStyle (Utilities|Struct|MakeSlateBrush "(X=36.000000,Y=40.000000)" "(Left=0.000000,Top=0.000000,Right=0.000000,Bottom=0.000000)" (Utilities|Struct|MakeSlateColor "(R=0.025187,G=0.025187,B=0.025187,A=1.000000)") "/Game/Mordhau/UI/UIAssets/Textures/ic_defence_lvl1.ic_defence_lvl1" "Image" "NoTile" "NoMirror") _slatebrush_2 _slatebrush_2))
                  (else
                    (Variables|/Script/UMG.ProgressBar|SetWidgetStyle (Variables|/Game/Mordhau/Blueprints/GameModes/Battle/BP_DestroyableWidgetFloater.BP_DestroyableWidgetFloater_C|GetProgressBar_0 _asbp_destroyable_widget_floater) (Utilities|Struct|MakeProgressBarStyle (Utilities|Struct|MakeSlateBrush "(X=30.000000,Y=38.000000)" "(Left=0.000000,Top=0.000000,Right=0.000000,Bottom=0.000000)" (Utilities|Struct|MakeSlateColor "(R=0.025187,G=0.025187,B=0.025187,A=1.000000)") "/Game/Mordhau/UI/UIAssets/Textures/ic_strike.ic_strike" "Image" "NoTile" "NoMirror") _slatebrush _slatebrush))))))))))))

(fn GetObjectiveProgress
  (return (* (- 1.0 (/ (Math|Conversions|ToFloat(Byte) (Variables|Default|GetReplicatedHealth)) 1e+02)) (Variables|Default|GetObjectiveWeight))))