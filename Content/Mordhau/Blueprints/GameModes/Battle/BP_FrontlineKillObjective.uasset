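; Killable Frontline objective character, owned by a capture point's team, that reports lost health as objective progress.
; The server spawns its AI controller, profile and equipment; it takes no damage until the enemy meets prerequisites, when its health floater appears.
; It can then offer itself to owning-team players, split among kill objectives by modulo, possessing candidates who don't decline before the countdown ends.
; Enemy attackers score for damage and the kill.
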(event EventBeginPlay
  (bind _mordhauwidget (Variables|Default|GetMordhauWidget))
  (|CallParentFunction)
  (Utilities|FlowControl|Sequence
    (:then_0
      (Variables|Default|SetContainmentVolumeCounter 0)
      (for _array_element (Collision|GetOverlappingActors (Variables|Default|GetCapsuleComponent) "/Game/Mordhau/Blueprints/GameModes/Battle/BP_KillObjectiveContainmentBox.BP_KillObjectiveContainmentBox_C" :!class /Script/Engine.PrimitiveComponent)
        (bind _asbp_kill_objective_containment_box (Utilities|Casting|CastToBP_KillObjectiveContainmentBox _array_element))
        (if (== (Variables|/Game/Mordhau/Blueprints/GameModes/Battle/BP_KillObjectiveContainmentBox.BP_KillObjectiveContainmentBox_C|GetKillObjectiveToContain _asbp_kill_objective_containment_box) self)
          (Variables|Default|SetContainmentVolumeCounter (+ (Variables|Default|GetContainmentVolumeCounter) 1)))))
    (:then_1
      (Utilities|IsValid _mordhauwidget
        (:Is%20Valid
          (bind _asbp_destroyable_widget_floater (Utilities|Casting|CastToBP_DestroyableWidgetFloater (UserInterface|GetUserWidgetObject _mordhauwidget)))
          (Default|UpdateHealth _asbp_destroyable_widget_floater (Math|Conversions|ToFloat(Byte) (Variables|Default|GetHealth))))))
    (:then_2
      (Networking|SwitchHasAuthority
        (:Authority
          (Variables|Default|SetOriginalReceivedDamageModifier (Variables|Default|GetReceivedDamageModifier))
          (Variables|Default|SetReceivedDamageModifier 0.0)
          (Utilities|FlowControl|Delay 0.2)
          (bind _returnvalue (Game|SpawnActorfromClass "/Game/Mordhau/Blueprints/GameModes/Battle/BP_FrontlineEnemyAIController.BP_FrontlineEnemyAIController_C" (Math|Transform|MakeTransform "0, 0, 0") "Undefined" 0 0))
          (bind _returnvalue_2 (Game|ConstructObjectfromClass (Variables|Default|GetBehaviorProfile) _returnvalue))
          (Variables|/Script/Mordhau.MordhauAIController|SetBehaviorProfile _returnvalue _returnvalue_2)
          (bind _returnvalue_3 (Game|SpawnActorfromClass "/Script/Mordhau.CustomizationReplicationActor" (Math|Transform|MakeTransform "0, 0, 0") "Undefined" 0 0))
          (Class|CustomizationReplicationActor|AssignDatafromProfile _returnvalue_3 (Variables|Default|GetProfileToAssign))
          (bind _output_get (Variables|/Script/Mordhau.MordhauAIController|SetCustomizationReplicationActor _returnvalue _returnvalue_3))
          (Class|MordhauCharacter|SetCustomizationReplicationActor _output_get)
          (Pawn|Possess _returnvalue self)
          (CallFunction|SpawnOurEquipment)
          (Class|MordhauCharacter|OnPostProfileAssigned))))))

(event Collision|EventActorBeginOverlap
  (params (OtherActor :type Actor%20Object%20Reference)))

(event EventBPLODTick
  (params (DeltaTime :type Float%20%28single-precision%29))
  (bind _returnvalue (Pawn|GetController))
  (bind _candidatesforpossess (Variables|Default|GetCandidatesForPossess))
  (bind _candidatesforpossess_2 (Variables|Default|GetCandidatesForPossess))
  (bind _output (Utilities|Array|Get(acopy) _candidatesforpossess_2))
  (|CallParentFunction DeltaTime)
  (Networking|SwitchHasAuthority
    (:Authority
      (if (not (Class|AdvancedCharacter|GetIsDead))
        (if (> (Utilities|Array|Length _candidatesforpossess) 0)
          (if (CallFunction|IsCandidateValidforPossession (Utilities|Array|Get(acopy) _candidatesforpossess))
            (bind _output_get (Variables|Default|SetCandidateTimeToDecline (- (Variables|Default|GetCandidateTimeToDecline) DeltaTime)))
            (if (<= _output_get 0.0)
              (Utilities|IsValid _returnvalue
                (:Is%20Valid
                  (Pawn|UnPossess _returnvalue))
                (:Is%20Not%20Valid
                  _))
              (bind _asbp_mordhau_game_mode (Utilities|Casting|CastToBP_MordhauGameMode (Game|GetGameMode)))
              (Default|UnpossessandDestroyPawn _asbp_mordhau_game_mode _output true)
              (Pawn|Possess _output self)
              (Utilities|Array|Clear _candidatesforpossess_2))
            (else
              (Utilities|Array|RemoveIndex _candidatesforpossess)
              (CallFunction|NotifyCandidateforPossession))))))))

(event EventOnAnyObjectiveProgressChanged
  (bind _point (Variables|Default|GetPoint))
  (if (not (Class|AdvancedCharacter|GetIsDead))
    (Utilities|IsValid _point
      (:Is%20Valid
        (if (== (Variables|/Game/Mordhau/Blueprints/GameModes/Battle/BP_CapturePoint.BP_CapturePoint_C|GetObjectiveProgress _point) 1.0)
          (Variables|Default|SetObjectiveWasCompleted true)
          (Variables|/Script/Mordhau.MordhauWidgetComponent|SetOverrideVisible (Variables|Default|GetMordhauWidget) 0)
          (Variables|Default|SetAwardedKillPoints true))))))

(event EventTick
  (params (DeltaSeconds :type Float%20%28single-precision%29)))

(event EventOnEnemyGainedPrerequisites
  (if (not (Class|AdvancedCharacter|GetIsDead))
    (Variables|Default|SetReceivedDamageModifier (Variables|Default|GetOriginalReceivedDamageModifier))
    (if (not (Variables|Default|GetObjectiveWasCompleted))
      (Variables|/Script/Mordhau.MordhauWidgetComponent|SetOverrideVisible (Variables|Default|GetMordhauWidget) -1)
      (CallFunction|UpdateUIWidgets)
      (Networking|SwitchHasAuthority
        (:Authority
          (if (Variables|Default|GetOfferPlayersToPossess)
            ;[1 1 1] Give time for the announcements to go through..
            (Utilities|FlowControl|Delay 9.0)
            (CallFunction|CompileCandidatesList)
            (CallFunction|NotifyCandidateforPossession)))))))

(event EventOnEnemyLostPrerequisites
  (if (not (Class|AdvancedCharacter|GetIsDead))
    (Variables|Default|SetReceivedDamageModifier 0.0)
    (Variables|/Script/Mordhau.MordhauWidgetComponent|SetOverrideVisible (Variables|Default|GetMordhauWidget) 0)
    (CallFunction|UpdateUIWidgets)))

(event Game|Damage|EventAnyDamage
  (params (Damage :type Float%20%28single-precision%29) (DamageType :type Damage%20Type%20Object%20Reference) (InstigatedBy :type Controller%20Object%20Reference) (DamageCauser :type Actor%20Object%20Reference))
  (Utilities|FlowControl|Sequence
    (:then_0
      (if (and (>= Damage 1.0) (not (Variables|Default|GetAwardedKillPoints)))
        (Utilities|IsValid (Variables|Default|GetPoint)
          (:Is%20Valid
            (Utilities|IsValid InstigatedBy
              (:Is%20Valid
                (bind _asmordhau_player_state (Utilities|Casting|CastToMordhauPlayerState (Variables|/Script/Engine.Controller|GetPlayerState InstigatedBy)))
                (if (not (== (Variables|/Script/Mordhau.MordhauPlayerState|GetTeam _asmordhau_player_state) (Math|Conversions|ToInteger(Byte) (Variables|/Script/Mordhau.ControlPoint|GetOwningTeam (Variables|Default|GetPoint)))))
                  (bind _asmordhau_player_controller (Utilities|Casting|CastToMordhauPlayerController InstigatedBy))
                  (Class|MordhauPlayerController|GiveClientScoreBP _asmordhau_player_controller "Objective" (Math|Float|Truncate (* (Variables|Default|GetScorePerDamageMultiplier) Damage)))
                  (if (Class|AdvancedCharacter|GetIsDead)
                    (Class|MordhauPlayerController|GiveClientScoreBP _asmordhau_player_controller "Objective" (Variables|Default|GetScorePerKill))
                    (Variables|Default|SetAwardedKillPoints true)))))))))
    (:then_1
      (|CallParentFunction Damage DamageType InstigatedBy DamageCauser))))

(event EventOnInitialize
  (params (Point :type BP%20Capture%20Point%20Object%20Reference))
  (bind _output_get (Variables|Default|SetPoint Point))
  (Variables|Default|SetTeam (Variables|/Script/Mordhau.ControlPoint|GetOwningTeam _output_get)))

(event EventOnDied
  (params (Angle :type Float%20%28single-precision%29) (Type :type EMordhauDamageType%20Enum :default "Generic") (SubType :type Byte :default 0) (bone :type Name%20%28by%20ref%29 :default "None") (Point :type Vector%20%28by%20ref%29 :default "0, 0, 0") (Source :type Actor%20Object%20Reference) (Agent :type Actor%20Object%20Reference))
  (bind _mordhauwidget (Variables|Default|GetMordhauWidget))
  (Utilities|FlowControl|Sequence
    (:then_0
      (Variables|/Script/Mordhau.MordhauWidgetComponent|SetOverrideVisible _mordhauwidget 0)
      (Variables|/Script/Mordhau.MordhauWidgetComponent|SetbIsSlowHideOverride _mordhauwidget true)
      (Variables|/Script/Mordhau.MordhauWidgetComponent|SetVisibilityWeightInterpolationSpeed _mordhauwidget 1.0)
      (bind _asbp_destroyable_widget_floater (Utilities|Casting|CastToBP_DestroyableWidgetFloater (UserInterface|GetUserWidgetObject (Variables|Default|GetMordhauWidget))))
      (Default|UpdateHealth _asbp_destroyable_widget_floater 0.0))
    (:then_1
      (|CallParentFunction Angle Type SubType bone Point Source Agent))
    (:then_2
      (Default|ObjectivesChanged (Variables|Default|GetPoint)))))

(event EventOnUpdateUIWidgets
  (CallFunction|UpdateUIWidgets))

(event EventOnHealthChanged
  (bind _mordhauwidget (Variables|Default|GetMordhauWidget))
  (if (not (Class|AdvancedCharacter|GetIsDead))
    (Utilities|FlowControl|Sequence
      (:then_0
        (Utilities|IsValid _mordhauwidget
          (:Is%20Valid
            (bind _asbp_destroyable_widget_floater (Utilities|Casting|CastToBP_DestroyableWidgetFloater (UserInterface|GetUserWidgetObject _mordhauwidget)))
            (Default|UpdateHealth _asbp_destroyable_widget_floater (Math|Conversions|ToFloat(Byte) (Variables|Default|GetHealth))))))
      (:then_1
        (Default|ObjectivesChanged (Variables|Default|GetPoint))))))

(fn ConstructionScript
  (|CallParentFunction))

(fn SpawnOurEquipment
  (for _array_element (Variables|Default|GetEquipmentToSpawn)
    (if (Utilities|IsValidClass _array_element)
      (bind _returnvalue (Game|SpawnActorfromClass _array_element (Math|Transform|MakeTransform "0, 0, 0") "Undefined" 0 0))
      (bind _returnvalue_2 (Class|MordhauEquipment|GetRandomCustomization _returnvalue false))
      (Class|MordhauEquipment|AssignCustomization _returnvalue _returnvalue_2)
      (Class|MordhauCharacter|PickUp _returnvalue))))

(fn UpdateUIWidgets
  (bind _slatebrush (Utilities|Struct|MakeSlateBrush "(X=40.000000,Y=40.000000)" "(Left=0.000000,Top=0.000000,Right=0.000000,Bottom=0.000000)" "(SpecifiedColor=(R=1.000000,G=1.000000,B=1.000000,A=1.000000),ColorUseRule=UseColor_Specified)" 0 "Image" "NoTile" "NoMirror"))
  (bind _slatebrush_2 (Utilities|Struct|MakeSlateBrush "(X=40.000000,Y=40.000000)" "(Left=0.000000,Top=0.000000,Right=0.000000,Bottom=0.000000)" "(SpecifiedColor=(R=1.000000,G=1.000000,B=1.000000,A=1.000000),ColorUseRule=UseColor_Specified)" "/Game/Mordhau/UI/UIAssets/Textures/ic_defence_lvl1.ic_defence_lvl1" "Image" "NoTile" "NoMirror"))
  (bind _mordhauwidget (Variables|Default|GetMordhauWidget))
  (bind _point (Variables|Default|GetPoint))
  (Utilities|IsValid _point
    (:Is%20Valid
      (if (not (== (Variables|/Game/Mordhau/Blueprints/GameModes/Battle/BP_CapturePoint.BP_CapturePoint_C|GetObjectiveProgress _point) 1.0))
        (Utilities|IsValid _mordhauwidget
          (:Is%20Valid
            (bind _asbp_destroyable_widget_floater (Utilities|Casting|CastToBP_DestroyableWidgetFloater (UserInterface|GetUserWidgetObject _mordhauwidget)))
            (bind _asmordhau_game_state (Utilities|Casting|CastToMordhauGameState (Game|GetGameState)))
            (bind _asmordhau_player_state (Utilities|Casting|CastToMordhauPlayerState (Variables|/Script/Engine.Controller|GetPlayerState (Game|GetPlayerController 0))))
            (if (== (Variables|/Script/Mordhau.ControlPoint|GetOwningTeam (Variables|Default|GetPoint)) (Math|Conversions|ToByte(Integer) (Variables|/Script/Mordhau.MordhauPlayerState|GetTeam _asmordhau_player_state)))
              (Variables|/Script/UMG.ProgressBar|SetWidgetStyle (Variables|/Game/Mordhau/Blueprints/GameModes/Battle/BP_DestroyableWidgetFloater.BP_DestroyableWidgetFloater_C|GetProgressBar_0 _asbp_destroyable_widget_floater) (Utilities|Struct|MakeProgressBarStyle (Utilities|Struct|MakeSlateBrush "(X=40.000000,Y=40.000000)" "(Left=0.000000,Top=0.000000,Right=0.000000,Bottom=0.000000)" (Utilities|Struct|MakeSlateColor "(R=0.025187,G=0.025187,B=0.025187,A=1.000000)") "/Game/Mordhau/UI/UIAssets/Textures/ic_defence_lvl1.ic_defence_lvl1" "Image" "NoTile" "NoMirror") _slatebrush_2 _slatebrush_2))
              (else
                (Variables|/Script/UMG.ProgressBar|SetWidgetStyle (Variables|/Game/Mordhau/Blueprints/GameModes/Battle/BP_DestroyableWidgetFloater.BP_DestroyableWidgetFloater_C|GetProgressBar_0 _asbp_destroyable_widget_floater) (Utilities|Struct|MakeProgressBarStyle (Utilities|Struct|MakeSlateBrush "(X=40.000000,Y=40.000000)" "(Left=0.000000,Top=0.000000,Right=0.000000,Bottom=0.000000)" (Utilities|Struct|MakeSlateColor "(R=0.025187,G=0.025187,B=0.025187,A=1.000000)") 0 "Image" "NoTile" "NoMirror") _slatebrush _slatebrush))))))))))

(fn ProcessPossessionCandidates
  (params (NewParam :type Boolean)))

(fn NotifyCandidateforPossession
  (if (> (Utilities|Array|Length (Variables|Default|GetCandidatesForPossess)) 0)
    (Variables|Default|SetCurrentCandidateTimeLeft (Variables|Default|GetCandidateTimeToDecline))
    (Default|NotifyOfferedParticipation (Utilities|Array|Get(acopy) (Variables|Default|GetCandidatesForPossess)))))

(fn IsCandidateValidforPossession
  (params (Candidate :type BP%20Frontline%20Player%20Controller%20Object%20Reference))
  (Utilities|IsValid Candidate
    (:Is%20Valid
      (bind _asmordhau_player_state (Utilities|Casting|CastToMordhauPlayerState (Variables|/Script/Engine.Controller|GetPlayerState Candidate))
        (:then
          (if (and (not (Variables|/Game/Mordhau/Blueprints/GameModes/Battle/BP_FrontlinePlayerController.BP_FrontlinePlayerController_C|GetDeclinedObjectiveParticipation Candidate)) (== (Variables|/Script/Mordhau.MordhauPlayerState|GetTeam _asmordhau_player_state) (Math|Conversions|ToInteger(Byte) (Variables|/Script/Mordhau.ControlPoint|GetOwningTeam (Variables|Default|GetPoint)))))
            (return true)
            (else
              _)))
        (:CastFailed
          _)))
    (:Is%20Not%20Valid
      _))
  (return false))

(fn CompileCandidatesList
  (bind _point (Variables|Default|GetPoint))
  (bind _kill (Variables|/Game/Mordhau/Blueprints/GameModes/Battle/BP_CapturePoint.BP_CapturePoint_C|GetKill _point))
  (Utilities|FlowControl|Sequence
    (:then_0
      (bind _array_element (Utilities|Array|ForEachLoopwithBreak _kill :!label _label)
        (:LoopBody
          (Utilities|IsValid _array_element
            (:Is%20Valid
              (if (== _array_element self)
                (goto _label Break)
                (elif (Variables|BP_FrontlineKillObjective_C|GetOfferPlayersToPossess _array_element)
                  (LocalVariables|SetSkipBias (+ (LocalVariables|GetSkipBias) 1)))))))
        (:Completed
          (for _array_element_2 _kill
            (Utilities|IsValid _array_element_2
              (:Is%20Valid
                (if (Variables|BP_FrontlineKillObjective_C|GetOfferPlayersToPossess _array_element_2)
                  (LocalVariables|SetSkipMod (+ (LocalVariables|GetSkipMod) 1)))))))))
    (:then_1
      (Utilities|Array|Clear (Variables|Default|GetCandidatesForPossess))
      (for _array_element_3 (Variables|/Script/Engine.GameStateBase|GetPlayerArray (Game|GetGameState))
        (bind _asmordhau_player_state (Utilities|Casting|CastToMordhauPlayerState _array_element_3))
        (if (== (Variables|/Script/Mordhau.MordhauPlayerState|GetTeam _asmordhau_player_state) (Math|Conversions|ToInteger(Byte) (Variables|/Script/Mordhau.ControlPoint|GetOwningTeam _point)))
          (Utilities|Array|Add (LocalVariables|GetCandidatePlayerStates) _asmordhau_player_state)))
      (bind _returnvalue (Class|MordhauUtilityLibrary|SortPlayers (LocalVariables|GetCandidatePlayerStates)))
      (for (_array_element_4 _array_index) _returnvalue
        (if (== (Math|Integer|%(Integer) _array_index (LocalVariables|GetSkipMod)) (LocalVariables|GetSkipBias))
          (bind _asbp_frontline_player_controller (Utilities|Casting|CastToBP_FrontlinePlayerController (Components|GetOwner _array_element_4)))
          (Variables|/Game/Mordhau/Blueprints/GameModes/Battle/BP_FrontlinePlayerController.BP_FrontlinePlayerController_C|SetDeclinedObjectiveParticipation _asbp_frontline_player_controller false)
          (if (CallFunction|IsCandidateValidforPossession _asbp_frontline_player_controller)
            (Utilities|Array|Add (Variables|Default|GetCandidatesForPossess) _asbp_frontline_player_controller)))))))

(fn GetObjectiveProgress
  (if (Class|AdvancedCharacter|GetIsDead)
    (return 1.0)
    (else
      (return (- 1.0 (/ (Math|Conversions|ToFloat(Byte) (Variables|Default|GetHealth)) 1e+02))))))