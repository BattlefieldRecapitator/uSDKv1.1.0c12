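; Frontline game mode HUD that shows either a Push or standard Frontline widget, plus team-specific objective text.
; When the game state replicates, it creates the widget matching IsPushMode behind other UI.
; Main menu and minimal/full HUD events toggle that widget's visibility.
; ShowObjectives scans capture points for one the local team can attack or must defend, then displays its objective text or a generic flag-capture message.
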(event EventBeginPlay
  (|CallParentFunction))

(event EventOnGameStateReplicated
  (bind _returnvalue (Game|GetPlayerController 0))
  (|CallParentFunction)
  (bind _asbp_frontline_game_state (Utilities|Casting|CastToBP_FrontlineGameState (Game|GetGameState)))
  (if (Variables|/Game/Mordhau/Blueprints/GameModes/Battle/BP_FrontlineGameState.BP_FrontlineGameState_C|GetIsPushMode _asbp_frontline_game_state)
    (bind _returnvalue_2 (UserInterface|CreateWidget "/Game/Mordhau/Blueprints/GameModes/Push/BP_PushHUDWidget.BP_PushHUDWidget_C" _returnvalue))
    (bind _output_get (Variables|Default|SetPushHUDWidget _returnvalue_2))
    (UserInterface|Viewport|AddtoViewport _output_get -5)
    (if (Variables|Default|GetIsHUDMinimal)
      (Widget|SetVisibility _output_get "Hidden"))
    (else
      (bind _returnvalue_3 (UserInterface|CreateWidget "/Game/Mordhau/Blueprints/GameModes/Battle/BP_FrontlineHUDWidget.BP_FrontlineHUDWidget_C" _returnvalue))
      (bind _output_get_2 (Variables|Default|SetFrontlineHUDWidget _returnvalue_3))
      (UserInterface|Viewport|AddtoViewport _output_get_2 -5)
      (if (Variables|Default|GetIsHUDMinimal)
        (Widget|SetVisibility _output_get_2 "Hidden")))))

(event EventHideMainMenu
  (bind _pushhudwidget (Variables|Default|GetPushHUDWidget))
  (bind _frontlinehudwidget (Variables|Default|GetFrontlineHUDWidget))
  (|CallParentFunction)
  (Utilities|IsValid _frontlinehudwidget
    (:Is%20Valid
      (Widget|SetVisibility _frontlinehudwidget "Visible"))
    (:Is%20Not%20Valid
      (Utilities|IsValid _pushhudwidget
        (:Is%20Valid
          (Widget|SetVisibility _pushhudwidget "Visible"))))))

(event EventShowMainMenu
  (params (ArmoryState :type E_ArmoryStates%20Enum :default "NewEnumerator0"))
  (bind _pushhudwidget (Variables|Default|GetPushHUDWidget))
  (bind _frontlinehudwidget (Variables|Default|GetFrontlineHUDWidget))
  (|CallParentFunction ArmoryState)
  (Utilities|IsValid _frontlinehudwidget
    (:Is%20Valid
      (Widget|SetVisibility _frontlinehudwidget "Hidden"))
    (:Is%20Not%20Valid
      (Utilities|IsValid _pushhudwidget
        (:Is%20Valid
          (Widget|SetVisibility _pushhudwidget "Hidden"))))))

(event EventUseMinimalHUD
  (bind _pushhudwidget (Variables|Default|GetPushHUDWidget))
  (bind _frontlinehudwidget (Variables|Default|GetFrontlineHUDWidget))
  (|CallParentFunction)
  (Utilities|IsValid _frontlinehudwidget
    (:Is%20Valid
      (Widget|SetVisibility _frontlinehudwidget "Hidden"))
    (:Is%20Not%20Valid
      (Utilities|IsValid _pushhudwidget
        (:Is%20Valid
          (Widget|SetVisibility _pushhudwidget "Hidden"))))))

(event EventUseFullHUD
  (bind _pushhudwidget (Variables|Default|GetPushHUDWidget))
  (bind _frontlinehudwidget (Variables|Default|GetFrontlineHUDWidget))
  (|CallParentFunction)
  (Utilities|IsValid _frontlinehudwidget
    (:Is%20Valid
      (Widget|SetVisibility _frontlinehudwidget "Visible"))
    (:Is%20Not%20Valid
      (Utilities|IsValid _pushhudwidget
        (:Is%20Valid
          (Widget|SetVisibility _pushhudwidget "Visible"))))))

(fn ConstructionScript
  (|CallParentFunction))

(fn ShowObjectives
  (bind _objectives (Variables|Default|GetObjectives))
  (bind _asbp_frontline_game_state (Utilities|Casting|CastToBP_FrontlineGameState (Game|GetGameState)))
  (bind _asmordhau_player_controller (Utilities|Casting|CastToMordhauPlayerController (Game|GetPlayerController 0)))
  (bind _asmordhau_player_state (Utilities|Casting|CastToMordhauPlayerState (Variables|/Script/Engine.Controller|GetPlayerState _asmordhau_player_controller)))
  (if (or (== (Variables|/Script/Mordhau.MordhauPlayerState|GetTeam _asmordhau_player_state) 0) (== (Variables|/Script/Mordhau.MordhauPlayerState|GetTeam _asmordhau_player_state) 1))
    (LocalVariables|SetOurTeam (Math|Conversions|ToByte(Integer) (Variables|/Script/Mordhau.MordhauPlayerState|GetTeam _asmordhau_player_state)))
    (LocalVariables|SetEnemyTeam (Math|Conversions|ToByte(Integer) (== (Variables|/Script/Mordhau.MordhauPlayerState|GetTeam _asmordhau_player_state) 0)))
    (bind _array_element (Utilities|Array|ForEachLoopwithBreak (Variables|/Script/Mordhau.MordhauGameState|GetAllCapturePoints _asbp_frontline_game_state) :!label _label)
      (:LoopBody
        (bind _asbp_capture_point (Utilities|Casting|CastToBP_CapturePoint _array_element))
        (if (> (Utilities|Array|Length (Variables|/Game/Mordhau/Blueprints/GameModes/Battle/BP_CapturePoint.BP_CapturePoint_C|GetObjectives _asbp_capture_point)) 0)
          (if (or (Variables|/Script/Mordhau.ControlPoint|GetbIsHiddenPoint _asbp_capture_point) (Variables|/Game/Mordhau/Blueprints/GameModes/Battle/BP_CapturePoint.BP_CapturePoint_C|GetIsPushPoint _asbp_capture_point))
            (if (!= (Variables|/Game/Mordhau/Blueprints/GameModes/Battle/BP_CapturePoint.BP_CapturePoint_C|GetObjectiveProgress _asbp_capture_point) 1.0)
              (if (== (Variables|/Script/Mordhau.ControlPoint|GetOwningTeam _asbp_capture_point) (LocalVariables|GetOurTeam)) :!label _label_2
                (bind _returnvalue (Class|ControlPoint|CanCapture _array_element (LocalVariables|GetEnemyTeam)))
                (if _returnvalue
                  ;[1 1 1] Our objective enemy can do - defend
                  (LocalVariables|SetPointFound _asbp_capture_point)
                  (goto _label Break))
                (else
                  (bind _returnvalue_2 (Class|ControlPoint|CanCapture _array_element (LocalVariables|GetOurTeam)))
                  (if _returnvalue_2
                    ;[1 1 1] Enemy objective we can do - attack
                    (LocalVariables|SetPointFound _asbp_capture_point)
                    (goto _label Break)))))
            (else
              (goto _label_2)))
          (elif (not (== (Variables|/Script/Mordhau.ControlPoint|GetOwningTeam _asbp_capture_point) (LocalVariables|GetOurTeam)))
            (bind _returnvalue_3 (Class|ControlPoint|CanCapture _asbp_capture_point (LocalVariables|GetOurTeam)))
            (if _returnvalue_3
              (LocalVariables|SetPointFound _asbp_capture_point)))))
      (:Completed
        (Utilities|IsValid (LocalVariables|GetPointFound)
          (:Is%20Valid
            (if (> (Utilities|Array|Length (Variables|/Game/Mordhau/Blueprints/GameModes/Battle/BP_CapturePoint.BP_CapturePoint_C|GetObjectives (LocalVariables|GetPointFound))) 0)
              (if (== (Variables|/Script/Mordhau.ControlPoint|GetOwningTeam (LocalVariables|GetPointFound)) (LocalVariables|GetOurTeam))
                (Default|Show _objectives (Variables|/Game/Mordhau/Blueprints/GameModes/Battle/BP_CapturePoint.BP_CapturePoint_C|GetObjectiveDefend (LocalVariables|GetPointFound)))
                (else
                  (Default|Show _objectives (Variables|/Game/Mordhau/Blueprints/GameModes/Battle/BP_CapturePoint.BP_CapturePoint_C|GetObjectiveAttack (LocalVariables|GetPointFound)))))
              (else
                (bind _output_get (LocalVariables|SetTextToShow (Utilities|Text|FormatText "Capture the enemy flags and defend your own!")))
                (Default|Show _objectives _output_get)))))))))