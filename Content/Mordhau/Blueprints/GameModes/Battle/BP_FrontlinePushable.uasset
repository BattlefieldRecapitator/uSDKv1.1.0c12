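; Frontline pushable objective that reports weighted progress to its linked capture point.
; Enemy prerequisite events toggle pushing, area decal and floating widget, with pushing disabled once the point's objectives complete.
; Progress updates notify the point and widget; full progress hides widget and decal and fires an empty PushableArrivedAtDestination event.
; The widget icon depends on whether the local player's team owns the point; team-colored progress bar logic is disconnected.
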(event Custom|PushableArrivedAtDestination)

(event EventBeginPlay
  (|CallParentFunction) ; This node is disabled and will not be called.\nDrag off pins to build functionality.
)

(event Collision|EventActorBeginOverlap
  (params (OtherActor :type Actor%20Object%20Reference))
  (|CallParentFunction OtherActor) ; This node is disabled and will not be called.\nDrag off pins to build functionality.
)

(event EventTick
  (params (DeltaSeconds :type Float%20%28single-precision%29))
  (|CallParentFunction DeltaSeconds) ; This node is disabled and will not be called.\nDrag off pins to build functionality.
)

(event EventOnProgressUpdated
  (params (OldProgress :type Float%20%28single-precision%29))
  (bind _mordhauwidget (Variables|Default|GetMordhauWidget))
  (bind _progress (Variables|Default|GetProgress))
  (bind _returnvalue (== _progress 1.0))
  (|CallParentFunction OldProgress)
  (Utilities|FlowControl|Sequence
    (:then_0
      (Default|ObjectivesChanged (Variables|Default|GetCapturePoint))
      (if _returnvalue
        (Variables|/Script/Mordhau.MordhauWidgetComponent|SetOverrideVisible _mordhauwidget 0)
        (Rendering|SetVisibility (Variables|Default|GetAreaDecal) false false))
      (bind _asbp_pushable_widget_floater (Utilities|Casting|CastToBP_PushableWidgetFloater (UserInterface|GetUserWidgetObject _mordhauwidget)))
      (Default|UpdateProgress _asbp_pushable_widget_floater _progress))
    (:then_1
      (if _returnvalue
        (CallFunction|PushableArrivedatDestination)))))

(event EventOnInitialize
  (params (Point :type BP%20Capture%20Point%20Object%20Reference))
  (CallFunction|Initialize Point))

(event EventOnEnemyLostPrerequisites
  (CallFunction|EnemyLostPrerequisites)
  (CallFunction|UpdateUIWidgets))

(event EventOnEnemyGainedPrerequisites
  (CallFunction|EnemyGainedPrerequisites)
  (CallFunction|UpdateUIWidgets))

(event EventOnUpdateUIWidgets
  (CallFunction|UpdateUIWidgets))

(event EventOnAnyObjectiveProgressChanged
  (bind _capturepoint (Variables|Default|GetCapturePoint))
  (Utilities|IsValid _capturepoint
    (:Is%20Valid
      (if (== (Variables|/Game/Mordhau/Blueprints/GameModes/Battle/BP_CapturePoint.BP_CapturePoint_C|GetObjectiveProgress _capturepoint) 1.0)
        (CallFunction|EnemyLostPrerequisites)))))

(fn ConstructionScript
  (|CallParentFunction))

(fn Initialize
  (params (CapturePoint :type BP%20Capture%20Point%20Object%20Reference))
  (Variables|Default|SetCapturePoint CapturePoint))

(fn EnemyGainedPrerequisites
  (bind _capturepoint (Variables|Default|GetCapturePoint))
  (Utilities|IsValid _capturepoint
    (:Is%20Valid
      (if (not (== (Variables|/Game/Mordhau/Blueprints/GameModes/Battle/BP_CapturePoint.BP_CapturePoint_C|GetObjectiveProgress _capturepoint) 1.0))
        (Variables|Default|SetbIsPushingAllowed true)
        (if (not (== (Variables|Default|GetProgress) 1.0))
          (Variables|/Script/Mordhau.MordhauWidgetComponent|SetOverrideVisible (Variables|Default|GetMordhauWidget) -1)
          (Rendering|SetVisibility (Variables|Default|GetAreaDecal) true false))))))

(fn EnemyLostPrerequisites
  (Variables|Default|SetbIsPushingAllowed false)
  (Variables|/Script/Mordhau.MordhauWidgetComponent|SetOverrideVisible (Variables|Default|GetMordhauWidget) 0)
  (Rendering|SetVisibility (Variables|Default|GetAreaDecal) false false))

(fn UpdateUIWidgets
  (bind _capturepoint (Variables|Default|GetCapturePoint))
  (bind _mordhauwidget (Variables|Default|GetMordhauWidget))
  (Utilities|IsValid (Game|GetPlayerController 0)
    (:Is%20Valid
      (Utilities|IsValid _capturepoint
        (:Is%20Valid
          (if (not (== (Variables|/Game/Mordhau/Blueprints/GameModes/Battle/BP_CapturePoint.BP_CapturePoint_C|GetObjectiveProgress _capturepoint) 1.0))
            (Utilities|IsValid _mordhauwidget
              (:Is%20Valid
                (bind _asbp_pushable_widget_floater (Utilities|Casting|CastToBP_PushableWidgetFloater (UserInterface|GetUserWidgetObject _mordhauwidget)))
                (bind _asmordhau_game_state (Utilities|Casting|CastToMordhauGameState (Game|GetGameState)))
                (bind _asmordhau_player_state (Utilities|Casting|CastToMordhauPlayerState (Variables|/Script/Engine.Controller|GetPlayerState (Game|GetPlayerController 0))))
                (if (== (Variables|/Script/Mordhau.ControlPoint|GetOwningTeam _capturepoint) (Math|Conversions|ToByte(Integer) (Variables|/Script/Mordhau.MordhauPlayerState|GetTeam _asmordhau_player_state)))
                  (Class|Image|SetBrush (Variables|/Game/Mordhau/Blueprints/GameModes/Battle/BP_PushableWidgetFloater.BP_PushableWidgetFloater_C|GetIcon _asbp_pushable_widget_floater) (Utilities|Struct|MakeSlateBrush "(X=36.000000,Y=40.000000)" "(Left=0.000000,Top=0.000000,Right=0.000000,Bottom=0.000000)" (Utilities|Struct|MakeSlateColor "(R=0.848958,G=0.848958,B=0.848958,A=1.000000)") "/Game/Mordhau/UI/UIAssets/Textures/ic_defence_lvl1.ic_defence_lvl1" "Image" "NoTile" "NoMirror"))
                  (else
                    (Class|Image|SetBrush (Variables|/Game/Mordhau/Blueprints/GameModes/Battle/BP_PushableWidgetFloater.BP_PushableWidgetFloater_C|GetIcon _asbp_pushable_widget_floater) (Utilities|Struct|MakeSlateBrush "(X=32.000000,Y=32.000000)" "(Left=0.000000,Top=0.000000,Right=0.000000,Bottom=0.000000)" "(SpecifiedColor=(R=1.000000,G=1.000000,B=1.000000,A=1.000000),ColorUseRule=UseColor_Specified)" 0 "Image" "NoTile" "NoMirror"))))))))))))

(fn GetObjectiveProgress
  (return (* (Variables|Default|GetProgress) (Variables|Default|GetObjectiveWeight))))