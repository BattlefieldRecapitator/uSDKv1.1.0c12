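; Deathmatch game state that shows the local player a victory or defeat screen when the match ends.
; It extends the parent's match-end handling, comparing the winner to the first player controller's player state and sending the result to the Mordhau HUD.
; Victory shows if that player won or has team -1; otherwise defeat shows with the winner's name.
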(event EventHandleMatchEndInfo
  (bind _matchendinfo (Variables|Default|GetMatchEndInfo))
  (bind _winner (Utilities|Struct|BreakSTRUCT_MatchEndInfo _matchendinfo))
  (|CallParentFunction)
  (bind _asbp_mordhau_hud (Utilities|Casting|CastToBP_MordhauHUD (Class|MordhauUtilityLibrary|GetMordhauHUD)))
  (bind _asmordhau_player_state (Utilities|Casting|CastToMordhauPlayerState (Variables|/Script/Engine.Controller|GetPlayerState (Game|GetPlayerController 0))))
  (if (or (== _winner _asmordhau_player_state) (== (Variables|/Script/Mordhau.MordhauPlayerState|GetTeam _asmordhau_player_state) -1))
    (Default|ShowMatchResult _asbp_mordhau_hud true "victory")
    (else
      (Default|ShowMatchResult _asbp_mordhau_hud false "defeat" (Utilities|Text|FormatText "{a} wins the match!" (Utilities|Text|ToText(String) (PlayerState|GetPlayerName _winner)))))))

(event EventBeginPlay)

(event EventTick
  (params (DeltaSeconds :type Float%20%28single-precision%29)))

(fn ConstructionScript
  (|CallParentFunction))