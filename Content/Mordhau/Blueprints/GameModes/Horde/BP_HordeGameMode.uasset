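; Game mode for Horde, running cooperative waves of AI enemies and ending in victory after the last wave or defeat when no living players remain and spawning is closed.
; At BeginPlay it pre-spawns a pool of AI controllers sized to the largest wave and shared customization actors per enemy variant.
; Tick drives waves: random variants spawn in grids at shuffled spawn points, and clearing one awards coins, heals survivors and respawns dead players.
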(event EventOnKilled
  (params (Killer :type Controller%20Object%20Reference) (KilledPlayer :type Controller%20Object%20Reference) (KilledPawn :type Pawn%20Object%20Reference) (Type :type EMordhauDamageType%20Enum :default "Generic") (SubType :type Byte :default 0) (DamageSource :type Actor%20Object%20Reference) (DamageAgent :type Actor%20Object%20Reference))
  (Utilities|FlowControl|Sequence
    (:then_0
      (if (!= Killer KilledPlayer)
        (bind _asmordhau_player_controller (Utilities|Casting|CastToMordhauPlayerController Killer))
        (bind _asbp_horde_player_state (Utilities|Casting|CastToBP_HordePlayerState (Variables|/Script/Engine.Controller|GetPlayerState _asmordhau_player_controller)))
        (bind _asbp_horde_enemy (Utilities|Casting|CastToBP_HordeEnemy KilledPawn)
          (:then
            (Class|MordhauPlayerController|GiveClientScoreBP _asmordhau_player_controller "Kill" (Math|Float|Truncate (Variables|Default|GetKillScoreChange)))
            (Class|MordhauPlayerState|AddKills _asbp_horde_player_state 1)
            (Variables|/Game/Mordhau/Blueprints/GameModes/Horde/BP_HordePlayerState.BP_HordePlayerState_C|SetCoins _asbp_horde_player_state (+ (Variables|/Game/Mordhau/Blueprints/GameModes/Horde/BP_HordePlayerState.BP_HordePlayerState_C|GetCoins _asbp_horde_player_state) (Variables|/Game/Mordhau/Blueprints/GameModes/Horde/BP_HordeEnemy.BP_HordeEnemy_C|GetKillReward _asbp_horde_enemy))))
          (:CastFailed
            ;[1 1 1] Team kill
            (Utilities|Casting|CastToPlayerController KilledPlayer)
            (Variables|/Game/Mordhau/Blueprints/GameModes/Horde/BP_HordePlayerState.BP_HordePlayerState_C|SetCoins _asbp_horde_player_state (Math|Integer|Max(Integer) (+ (Variables|/Game/Mordhau/Blueprints/GameModes/Horde/BP_HordePlayerState.BP_HordePlayerState_C|GetCoins _asbp_horde_player_state) (Variables|Default|GetTeamKillCoinPunishment))))))))
    (:then_1
      (|CallParentFunction Killer KilledPlayer KilledPawn Type SubType DamageSource DamageAgent))))

(event EventBeginPlay
  (|CallParentFunction)
  (Utilities|FlowControl|Sequence
    (:then_0
      (bind _outactors (Actor|GetAllActorsOfClass "/Game/Mordhau/Blueprints/GameModes/Horde/BP_HordeGameConfiguration.BP_HordeGameConfiguration_C"))
      (if (> (Utilities|Array|Length _outactors) 0)
        (bind _output_get (Variables|Default|SetHordeGameConfiguration (Utilities|Array|Get(acopy) _outactors)))
        (Variables|Default|SetKillObjectiveCached (Variables|/Game/Mordhau/Blueprints/GameModes/Horde/BP_HordeGameConfiguration.BP_HordeGameConfiguration_C|GetKillObjective _output_get))))
    (:then_1
      (bind _outactors_2 (Actor|GetAllActorsOfClass "/Game/Mordhau/Blueprints/GameModes/Horde/Objectives/BP_HordeTask.BP_HordeTask_C"))
      (Variables|Default|SetHordeTasks _outactors_2))
    (:then_2
      (bind _outactors_3 (Actor|GetAllActorsOfClass "/Game/Mordhau/Blueprints/GameModes/Horde/BP_HordeSpawn.BP_HordeSpawn_C"))
      (Variables|Default|SetHordeSpawns _outactors_3)
      (Utilities|FlowControl|Sequence
        (:then_0
          (CallFunction|PrepareAIControllers))
        (:then_1
          (CallFunction|SetupCustomizationReplicationActors))))))

(event EventTick
  (params (DeltaSeconds :type Float%20%28single-precision%29))
  (|CallParentFunction DeltaSeconds)
  (bind _asbp_horde_game_state (Utilities|Casting|CastToBP_HordeGameState (Game|GetGameState)))
  (if (Class|GameMode|IsMatchinProgress)
    (if (Variables|Default|GetHasStarted)
      (bind _returnvalue (Class|MordhauGameState|GetPlayerCountsPerTeam _asbp_horde_game_state true false))
      (if (and (== (Utilities|Array|Get(acopy) _returnvalue) 0) (not (Variables|/Script/Mordhau.MordhauGameState|GetbAllowSpawning _asbp_horde_game_state)))
        ;[1 1 1] No players alive, end the match if spawning is over
        (CallFunction|TriggerDefeat)
        (elif (Variables|Default|GetWaveHasSpawned)
          (Variables|Default|SetEnemiesRemaining 0)
          (for _array_element (Variables|Default|GetSpawnedEnemies)
            (Utilities|IsValid _array_element
              (:Is%20Valid
                (if (not (Class|AdvancedCharacter|GetIsDead _array_element))
                  (Variables|Default|SetEnemiesRemaining (+ (Variables|Default|GetEnemiesRemaining) 1))))))
          (Variables|/Game/Mordhau/Blueprints/GameModes/Horde/BP_HordeGameState.BP_HordeGameState_C|SetReplicatedHordeMatchInfo _asbp_horde_game_state (Utilities|Struct|MakeSTRUCT_HordeMatchInfo (.Wave (Utilities|Struct|BreakSTRUCT_HordeMatchInfo (Variables|/Game/Mordhau/Blueprints/GameModes/Horde/BP_HordeGameState.BP_HordeGameState_C|GetReplicatedHordeMatchInfo _asbp_horde_game_state))) (Math|Conversions|ToByte(Integer) (Math|Integer|Clamp(Integer) (Variables|Default|GetEnemiesRemaining) 0 255)) (.NextWaveStartTime (Utilities|Struct|BreakSTRUCT_HordeMatchInfo (Variables|/Game/Mordhau/Blueprints/GameModes/Horde/BP_HordeGameState.BP_HordeGameState_C|GetReplicatedHordeMatchInfo _asbp_horde_game_state)))))
          (if (== (Variables|Default|GetEnemiesRemaining) 0)
            (CallFunction|ProgressWave))
          (elif (< (+ (Variables|Default|GetWaveStartTime) (Variables|Default|GetWaveEnemySpawnOffset)) (Utilities|Time|GetTimeSeconds))
            (Variables|/Script/Mordhau.MordhauGameState|SetbAllowSpawning _asbp_horde_game_state false)
            (bind _outactors (Actor|GetAllActorsOfClass "/Script/Mordhau.MordhauPlayerController"))
            (for _array_element_2 _outactors
              (bind _asbp_horde_character (Utilities|Casting|CastToBP_HordeCharacter (Pawn|GetControlledPawn _array_element_2)))
              (Variables|/Script/Mordhau.AdvancedCharacter|SetReceivedDamageModifier _asbp_horde_character (Math|Curves|GetFloatValue (Variables|Default|GetReceivedDamageByPlayerNum) (Math|Conversions|ToFloat(Integer) (Utilities|Array|Get(acopy) _returnvalue)))))
            (CallFunction|SpawnWave))))
      (else
        (bind _returnvalue_2 (Class|MordhauGameState|GetPlayerCountsPerTeam _asbp_horde_game_state false true))
        (if (> (Utilities|Array|Get(acopy) _returnvalue_2) 0)
          ;[1 1 1] Players present, start the match
          (CallFunction|StartHordeMatch))))))

(fn ConstructionScript
  (|CallParentFunction))

(fn SpawnWave
  (bind _waves (Variables|Default|GetWaves))
  (bind _spawnedperspawner (LocalVariables|GetSpawnedPerSpawner))
  (bind _hordespawns (Variables|Default|GetHordeSpawns))
  (bind _hordespawns_2 (Variables|Default|GetHordeSpawns))
  (bind _wave (Variables|Default|GetWave))
  (bind _output (Utilities|Array|Get(acopy) _waves _wave))
  (bind _wavevariants (Utilities|Struct|BreakSTRUCT_HordeWaveInfo _output))
  (bind _asbp_horde_game_state (Utilities|Casting|CastToBP_HordeGameState (Game|GetGameState)))
  (Utilities|FlowControl|Sequence
    (:then_0
      (Variables|Default|SetWaveHasSpawned true)
      (Utilities|Array|Shuffle _hordespawns)
      (for _array_element _hordespawns
        (Utilities|Array|Add (LocalVariables|GetSpawnedPerSpawner) 0))
      (bind _output_get (LocalVariables|SetChosenWaveVariant (Math|Random|RandomInteger (Utilities|Array|Length _wavevariants))))
      (bind _keys (Utilities|Map|Keys (Utilities|Struct|BreakSTRUCT_HordeEnemyArray (Utilities|Array|Get(acopy) _wavevariants _output_get))))
      (for _array_element_2 _keys
        (LocalVariables|SetTotalToSpawnInWave (+ (LocalVariables|GetTotalToSpawnInWave) (.Value (Utilities|Map|Find (Utilities|Struct|BreakSTRUCT_HordeEnemyArray (Utilities|Array|Get(acopy) _wavevariants _output_get)) _array_element_2)))))
      (for _array_element_3 _keys
        (for _index (range 0 (- (.Value (Utilities|Map|Find (Utilities|Struct|BreakSTRUCT_HordeEnemyArray (Utilities|Array|Get(acopy) _wavevariants _output_get)) _array_element_3)) 1))
          (bind _returnvalue (Game|ConstructObjectfromClass (.Behavior (Utilities|Struct|BreakSTRUCT_HordeEnemyInfo (.Value (Utilities|Map|Find (Variables|Default|GetEnemyDatabase) _array_element_3)))) (Utilities|Array|Get(acopy) (Variables|Default|GetAIControllers) (LocalVariables|GetTotalSpawned))))
          (Variables|/Script/Mordhau.MordhauAIController|SetBehaviorProfile (Utilities|Array|Get(acopy) (Variables|Default|GetAIControllers) (LocalVariables|GetTotalSpawned)) _returnvalue)
          (bind _ascustomization_replication_actor (Utilities|Casting|CastToCustomizationReplicationActor (Utilities|Array|Get(acopy) (Utilities|Struct|BreakArrayOfActor (.Value (Utilities|Map|Find (Variables|Default|GetEnemyVariantCustomizationActor) _array_element_3))) (Math|Random|RandomIntegerinRange 0 (- (Utilities|Array|Length (Utilities|Struct|BreakArrayOfActor (.Value (Utilities|Map|Find (Variables|Default|GetEnemyVariantCustomizationActor) _array_element_3)))) 1)))))
          (bind _output_get_2 (Variables|/Script/Mordhau.MordhauAIController|SetCustomizationReplicationActor (Utilities|Array|Get(acopy) (Variables|Default|GetAIControllers) (LocalVariables|GetTotalSpawned)) _ascustomization_replication_actor))
          (bind _output_get_3 (LocalVariables|SetRandomChoice (Math|Random|RandomIntegerinRange 0 (- (Math|Integer|Min(Integer) (Utilities|Array|Length _hordespawns_2) (+ (/ (LocalVariables|GetTotalToSpawnInWave) 11) 1)) 1))))
          (bind _returnvalue_2 (Game|SpawnActorfromClass (.CharacterType (Utilities|Struct|BreakSTRUCT_HordeEnemyInfo (.Value (Utilities|Map|Find (Variables|Default|GetEnemyDatabase) _array_element_3)))) (Math|Transform|MakeTransform (Math|Transform|TransformLocation (Transformation|GetActorTransform (Utilities|Array|Get(acopy) _hordespawns_2 _output_get_3)) (Math|Vector|MakeVector (* (/ (Utilities|Array|Get(acopy) _spawnedperspawner _output_get_3) 6) 1.3e+02) (* (Math|Integer|%(Integer) (Utilities|Array|Get(acopy) _spawnedperspawner _output_get_3) 6) 1.3e+02) 0.0)) (.Rotation (Math|Transform|BreakTransform (Transformation|GetActorTransform (Utilities|Array|Get(acopy) _hordespawns_2 _output_get_3))))) "Undefined" 0 0))
          (Utilities|Array|SetArrayElem _spawnedperspawner _output_get_3 (+ (Utilities|Array|Get(acopy) _spawnedperspawner _output_get_3) 1))
          (Utilities|Array|Add (Variables|Default|GetSpawnedEnemies) _returnvalue_2)
          (Variables|/Script/Mordhau.AdvancedCharacter|SetTeam _returnvalue_2 1)
          (Class|MordhauCharacter|SetCustomizationReplicationActor _returnvalue_2 _output_get_2)
          (Pawn|Possess (Utilities|Array|Get(acopy) (Variables|Default|GetAIControllers) (LocalVariables|GetTotalSpawned)) _returnvalue_2)
          (CallFunction|SpawnEquipmentfor (.Equipment (Utilities|Struct|BreakSTRUCT_HordeEnemyInfo (.Value (Utilities|Map|Find (Variables|Default|GetEnemyDatabase) _array_element_3)))) _returnvalue_2)
          (CallFunction|SpawnEquipmentfor (.SecondaryEquipment (Utilities|Struct|BreakSTRUCT_HordeEnemyInfo (.Value (Utilities|Map|Find (Variables|Default|GetEnemyDatabase) _array_element_3)))) _returnvalue_2)
          (Class|MordhauCharacter|OnPostProfileAssigned _returnvalue_2)
          (LocalVariables|SetTotalSpawned (+ (LocalVariables|GetTotalSpawned) 1)))
        (for (_array_element_4 _array_index) (LocalVariables|GetSpawnedPerSpawner)
          (if (> _array_element_4 0)
            (Variables|/Game/Mordhau/Blueprints/GameModes/Horde/BP_HordeSpawn.BP_HordeSpawn_C|SetSpawnActivatedCounter (Utilities|Array|Get(acopy) (Variables|Default|GetHordeSpawns) _array_index) (+ (Variables|/Game/Mordhau/Blueprints/GameModes/Horde/BP_HordeSpawn.BP_HordeSpawn_C|GetSpawnActivatedCounter (Utilities|Array|Get(acopy) (Variables|Default|GetHordeSpawns) _array_index)) 1))))))
    (:then_1
      (Variables|/Game/Mordhau/Blueprints/GameModes/Horde/BP_HordeGameState.BP_HordeGameState_C|SetReplicatedHordeMatchInfo _asbp_horde_game_state (Utilities|Struct|MakeSTRUCT_HordeMatchInfo (Math|Conversions|ToByte(Integer) _wave) (Math|Conversions|ToByte(Integer) (Math|Integer|Clamp(Integer) (LocalVariables|GetTotalSpawned) 0 255)) 0.0)))))

(fn StartHordeMatch
  (Variables|Default|SetHasStarted true)
  (CallFunction|ProgressWave))

(fn ProgressWave
  (bind _waves (Variables|Default|GetWaves))
  (Utilities|Array|Clear (Variables|Default|GetSpawnedEnemies))
  (bind _asbp_horde_game_state (Utilities|Casting|CastToBP_HordeGameState (Game|GetGameState)))
  (bind _outactors (Actor|GetAllActorsOfClass "/Script/Mordhau.MordhauPlayerController"))
  (Utilities|FlowControl|Sequence
    (:then_0
      ;[1 1 1] Award points for completion, heal them up
      (if (Utilities|Array|IsValidIndex _waves (Variables|Default|GetWave))
        (for _array_element _outactors
          (LocalVariables|SetConsideredChar 0)
          (Utilities|IsValid _array_element
            (:Is%20Valid
              (Utilities|FlowControl|Sequence
                (:then_0
                  (bind _asmordhau_vehicle (Utilities|Casting|CastToMordhauVehicle (Pawn|GetControlledPawn _array_element))
                    (:then
                      (LocalVariables|SetConsideredChar (Variables|/Script/Mordhau.MordhauVehicle|GetDriver _asmordhau_vehicle)))
                    (:CastFailed
                      (bind _asmordhau_character (Utilities|Casting|CastToMordhauCharacter (Pawn|GetControlledPawn _array_element)))
                      (LocalVariables|SetConsideredChar _asmordhau_character))))
                (:then_1
                  (Utilities|IsValid (LocalVariables|GetConsideredChar)
                    (:Is%20Valid
                      (Class|AdvancedCharacter|OffsetHealth (LocalVariables|GetConsideredChar) 100 false)
                      (Class|MordhauPlayerController|GiveClientScoreBP _array_element "WaveCleared" (.CompletionReward (Utilities|Struct|BreakSTRUCT_HordeWaveInfo (Utilities|Array|Get(acopy) (Variables|Default|GetWaves) (Variables|Default|GetWave)))))
                      (LocalVariables|SetCoinAward (.CompletionReward (Utilities|Struct|BreakSTRUCT_HordeWaveInfo (Utilities|Array|Get(acopy) (Variables|Default|GetWaves) (Variables|Default|GetWave))))))
                    (:Is%20Not%20Valid
                      (Class|MordhauPlayerController|GiveClientScoreBP _array_element "WaveCleared" (Math|Float|Truncate (* (Math|Conversions|ToFloat(Integer) (.CompletionReward (Utilities|Struct|BreakSTRUCT_HordeWaveInfo (Utilities|Array|Get(acopy) (Variables|Default|GetWaves) (Variables|Default|GetWave))))) (Variables|Default|GetDeadWaveCompletionMultiplier))))
                      (LocalVariables|SetCoinAward (Math|Float|Truncate (* (Math|Conversions|ToFloat(Integer) (.CompletionReward (Utilities|Struct|BreakSTRUCT_HordeWaveInfo (Utilities|Array|Get(acopy) (Variables|Default|GetWaves) (Variables|Default|GetWave))))) (Variables|Default|GetDeadWaveCompletionMultiplier))))))
                  (bind _asbp_horde_player_state (Utilities|Casting|CastToBP_HordePlayerState (Variables|/Script/Engine.Controller|GetPlayerState _array_element)))
                  (Variables|/Game/Mordhau/Blueprints/GameModes/Horde/BP_HordePlayerState.BP_HordePlayerState_C|SetCoins _asbp_horde_player_state (+ (Variables|/Game/Mordhau/Blueprints/GameModes/Horde/BP_HordePlayerState.BP_HordePlayerState_C|GetCoins _asbp_horde_player_state) (LocalVariables|GetCoinAward))))))))))
    (:then_1
      (bind _output_get (Variables|Default|SetWave (+ (Variables|Default|GetWave) 1)))
      (if (Utilities|Array|IsValidIndex _waves _output_get)
        (Variables|/Script/Mordhau.MordhauGameState|SetbAllowSpawning _asbp_horde_game_state true)
        (bind _output_get_2 (Variables|Default|SetWaveStartTime (Utilities|Time|GetTimeSeconds)))
        (Variables|/Game/Mordhau/Blueprints/GameModes/Horde/BP_HordeGameState.BP_HordeGameState_C|SetReplicatedHordeMatchInfo _asbp_horde_game_state (Utilities|Struct|MakeSTRUCT_HordeMatchInfo (.Wave (Utilities|Struct|BreakSTRUCT_HordeMatchInfo (Variables|/Game/Mordhau/Blueprints/GameModes/Horde/BP_HordeGameState.BP_HordeGameState_C|GetReplicatedHordeMatchInfo _asbp_horde_game_state))) (.EnemiesRemaining (Utilities|Struct|BreakSTRUCT_HordeMatchInfo (Variables|/Game/Mordhau/Blueprints/GameModes/Horde/BP_HordeGameState.BP_HordeGameState_C|GetReplicatedHordeMatchInfo _asbp_horde_game_state))) (+ _output_get_2 (Variables|Default|GetWaveEnemySpawnOffset))))
        (Variables|Default|SetWaveHasSpawned false)
        (Utilities|FlowControl|Sequence
          (:then_0
            (for _array_element_2 _outactors
              (Utilities|IsValid _array_element_2
                (:Is%20Valid
                  (Utilities|Casting|CastToAdvancedCharacter (Pawn|GetControlledPawn _array_element_2)
                    (:CastFailed
                      (if (Variables|/Script/Mordhau.MordhauPlayerController|GetbReceivedValidProfileFromClient _array_element_2)
                        (bind _asmordhau_player_state (Utilities|Casting|CastToMordhauPlayerState (Variables|/Script/Engine.Controller|GetPlayerState _array_element_2)))
                        (if (== (Variables|/Script/Mordhau.MordhauPlayerState|GetTeam _asmordhau_player_state) 0)
                          (CallFunction|UnpossessandDestroyPawn _array_element_2 true))))))))))
        (else
          (Class|GameMode|EndMatch)
          (Variables|/Game/Mordhau/Blueprints/GameModes/BP_MordhauGameState.BP_MordhauGameState_C|SetMatchEndInfo _asbp_horde_game_state (Utilities|Struct|MakeSTRUCT_MatchEndInfo 0 0 1.0)))))))

(fn SetupCustomizationReplicationActors
  (bind _enemydatabase (Variables|Default|GetEnemyDatabase))
  (bind _keys (Utilities|Map|Keys _enemydatabase))
  (for _array_element _keys
    (Utilities|Array|Clear (LocalVariables|GetTemp))
    (for _array_element_2 (.CustomizationVariants (Utilities|Struct|BreakSTRUCT_HordeEnemyInfo (.Value (Utilities|Map|Find _enemydatabase _array_element))))
      (bind _returnvalue (Game|SpawnActorfromClass "/Script/Mordhau.CustomizationReplicationActor" (Math|Transform|MakeTransform "0, 0, 0") "Undefined" 0 0))
      (Utilities|Array|Add (LocalVariables|GetTemp) _returnvalue)
      (Class|CustomizationReplicationActor|AssignDatafromProfile _returnvalue _array_element_2))
    (Utilities|Map|Add (Variables|Default|GetEnemyVariantCustomizationActor) _array_element (Utilities|Struct|MakeArrayOfActor (LocalVariables|GetTemp)))))

(fn PrepareAIControllers
  (for _array_element (Variables|Default|GetWaves)
    (for _array_element_2 (.WaveVariants (Utilities|Struct|BreakSTRUCT_HordeWaveInfo _array_element))
      (bind _values (Utilities|Map|Values (Utilities|Struct|BreakSTRUCT_HordeEnemyArray _array_element_2)))
      (LocalVariables|SetCandidate 0)
      (for _array_element_3 _values
        (LocalVariables|SetCandidate (+ (LocalVariables|GetCandidate) _array_element_3)))
      (LocalVariables|SetMaxWaveEnemies (Math|Integer|Max(Integer) (LocalVariables|GetMaxWaveEnemies) (LocalVariables|GetCandidate)))))
  (for _index (range 0 (- (LocalVariables|GetMaxWaveEnemies) 1))
    (bind _returnvalue (Game|SpawnActorfromClass "/Game/Mordhau/AI/BP_HordeAIController.BP_HordeAIController_C" (Math|Transform|MakeTransform "0, 0, 0") "Undefined" 0 0))
    (Utilities|Array|Add (Variables|Default|GetAIControllers) _returnvalue)))

(fn SpawnEquipmentfor
  (params (EquipList :type Array%20of%20Mordhau%20Equipment%20Class%20References) (Char :type Mordhau%20Character%20Object%20Reference))
  (bind _returnvalue (Utilities|Array|Length EquipList))
  (if (> _returnvalue 0)
    (bind _output_get (LocalVariables|SetChosenClass (Utilities|Array|Get(acopy) EquipList (Math|Random|RandomIntegerinRange 0 (- _returnvalue 1)))))
    (if (Utilities|IsValidClass _output_get)
      (bind _returnvalue_2 (Game|SpawnActorfromClass _output_get (Math|Transform|MakeTransform "0, 0, 0") "Undefined" 0 0))
      (bind _returnvalue_3 (Class|MordhauEquipment|GetRandomCustomization _returnvalue_2 false))
      (Class|MordhauEquipment|AssignCustomization _returnvalue_2 _returnvalue_3)
      (Class|MordhauCharacter|PickUp Char _returnvalue_2))))

(fn TriggerDefeat
  (bind _asbp_horde_game_state (Utilities|Casting|CastToBP_HordeGameState (Game|GetGameState)))
  (Class|GameMode|EndMatch)
  (Variables|/Game/Mordhau/Blueprints/GameModes/BP_MordhauGameState.BP_MordhauGameState_C|SetMatchEndInfo _asbp_horde_game_state (Utilities|Struct|MakeSTRUCT_MatchEndInfo 0 1 1.0)))