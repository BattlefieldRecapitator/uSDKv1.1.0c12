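; Horde mode variant of the recurve bow that switches to fire arrows based on the wielder's skill.
; When the loaded state changes, it runs the parent logic, then, if the bow is loaded, casts the parent character to BP_HordeCharacter.
; It enables fire arrows if a specific skill level is above zero and disables them otherwise, so the choice is re-evaluated on every load.
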(event EventBeginPlay
  (|CallParentFunction) ; This node is disabled and will not be called.\nDrag off pins to build functionality.
)

(event Collision|EventActorBeginOverlap
  (params (OtherActor :type Actor%20Object%20Reference))
  (|CallParentFunction OtherActor) ; This node is disabled and will not be called.\nDrag off pins to build functionality.
)

(event EventTick
  (params (DeltaSeconds :type Float%20%28single-precision%29))
  (|CallParentFunction DeltaSeconds) ; This node is disabled and will not be called.\nDrag off pins to build functionality.
)

(event EventOnLoadedChanged
  (|CallParentFunction)
  (if (Variables|Default|GetbIsLoaded)
    (bind _asbp_horde_character (Utilities|Casting|CastToBP_HordeCharacter (Class|MordhauEquipment|GetParentCharacter)))
    (Class|MordhauEquipment|SetUseFireArrows (> (Default|GetSkill _asbp_horde_character "NewEnumerator35") 0))))

(fn ConstructionScript
  (|CallParentFunction))