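; Recurve bow arrow projectile for Horde mode that hooks the Fletcher restock and Scatter Shot effects on the owning player.
; When fired and not locally predicted, it passes itself to the owning Horde player controller to try a scatter shot.
; On hitting a SurfaceType1 surface, it asks that controller to try a Fletcher restock.
; Both events run the parent projectile logic first and leave the effect logic to the controller.
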(event EventBeginPlay
  (|CallParentFunction) ; This node is disabled and will not be called.\nDrag off pins to build functionality.
)

(event Collision|EventActorBeginOverlap
  (params (OtherActor :type Actor%20Object%20Reference))
  (|CallParentFunction OtherActor) ; This node is disabled and will not be called.\nDrag off pins to build functionality.
)

(event EventTick
  (params (DeltaSeconds :type Float%20%28single-precision%29))
  (|CallParentFunction DeltaSeconds) ; This node is disabled and will not be called.\nDrag off pins to build functionality.
)

(event EventOnProjectileHit
  (params (HitLocation :type Vector%20%28by%20ref%29 :default "0, 0, 0") (HitNormal :type Vector%20%28by%20ref%29 :default "0, 0, 0") (BounceForce :type Float%20%28single-precision%29) (Surface :type Byte :default 0) (bHasHitWorld :type Boolean) (bHasStopped :type Boolean))
  (|CallParentFunction HitLocation HitNormal BounceForce Surface bHasHitWorld bHasStopped)
  (if (== Surface (Utilities|Enum|LiteralenumEPhysicalSurface "SurfaceType1"))
    (bind _returnvalue (Class|MordhauProjectile|GetProjectileOwningController))
    (bind _asbp_horde_player_controller (Utilities|Casting|CastToBP_HordePlayerController _returnvalue))
    (Default|TryFletcherRestock _asbp_horde_player_controller)))

(event EventOnProjectileFired
  (|CallParentFunction)
  (if (not (Variables|Default|GetbIsLocallyPredicted))
    (bind _returnvalue (Class|MordhauProjectile|GetProjectileOwningController))
    (bind _asbp_horde_player_controller (Utilities|Casting|CastToBP_HordePlayerController _returnvalue))
    (Default|TryScatterShot _asbp_horde_player_controller self)))

(fn ConstructionScript
  (|CallParentFunction))