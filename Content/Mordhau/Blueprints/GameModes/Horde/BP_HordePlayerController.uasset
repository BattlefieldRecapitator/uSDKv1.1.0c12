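; Horde mode player controller that holds the player's skill levels and carries loadout and skills onto the possessed BP_HordeCharacter.
; The server validates upgrades against prerequisites and a level cap, then copies the replicated skill array to the character.
; On a character's first possession it restores saved armor, equipment and ammo, applying weapon customization.
; It also implements bow skills: chance-based arrow restock, recursion-guarded scatter shot and fire arrows.
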(event EventBeginPlay
  (|CallParentFunction)
  (Networking|SwitchHasAuthority
    (:Authority
      (for _index (range 0 (- (Math|Conversions|ToInteger(Byte) (Utilities|Enum|LiteralenumE_HordeSkill "NewEnumerator4")) 1))
        (Utilities|Array|Add (Variables|Default|GetReplicatedSkills) 0)))))

(event EventTick
  (params (DeltaSeconds :type Float%20%28single-precision%29))
  (|CallParentFunction DeltaSeconds) ; This node is disabled and will not be called.\nDrag off pins to build functionality.
)

(event EventOnAfterPossess
  (params (APawn :type Pawn%20Object%20Reference))
  (bind _lastheadarmor (Variables|Default|GetLastHeadArmor))
  (bind _lastchestarmor (Variables|Default|GetLastChestArmor))
  (bind _lastlegarmor (Variables|Default|GetLastLegArmor))
  (Utilities|FlowControl|Sequence
    (:then_0
      (bind _asbp_horde_character (Utilities|Casting|CastToBP_HordeCharacter APawn))
      (if (not (Variables|/Game/Mordhau/Blueprints/Characters/BP_HordeCharacter.BP_HordeCharacter_C|GetAlreadyGaveDefaults _asbp_horde_character))
        (Variables|/Game/Mordhau/Blueprints/Characters/BP_HordeCharacter.BP_HordeCharacter_C|SetAlreadyGaveDefaults _asbp_horde_character true)
        (Networking|SwitchHasAuthority
          (:Authority
            (Utilities|FlowControl|Sequence
              (:then_0
                (Variables|/Game/Mordhau/Blueprints/Characters/BP_HordeCharacter.BP_HordeCharacter_C|SetReplicatedSkills _asbp_horde_character (Variables|Default|GetReplicatedSkills))
                (Utilities|FlowControl|Sequence
                  (:then_0
                    (if (> (CallFunction|GetSkillLevel "NewEnumerator3") 0)
                      (Variables|/Script/Mordhau.AdvancedCharacter|SetbHasLastChance _asbp_horde_character true)))))
              (:then_1
                (if (Utilities|IsValidClass _lastheadarmor)
                  (Variables|/Game/Mordhau/Blueprints/Characters/BP_BattleRoyaleCharacter.BP_BattleRoyaleCharacter_C|SetHeadArmor _asbp_horde_character _lastheadarmor)))
              (:then_2
                (if (Utilities|IsValidClass _lastchestarmor)
                  (Variables|/Game/Mordhau/Blueprints/Characters/BP_BattleRoyaleCharacter.BP_BattleRoyaleCharacter_C|SetChestArmor _asbp_horde_character _lastchestarmor)))
              (:then_3
                (if (Utilities|IsValidClass _lastlegarmor)
                  (Variables|/Game/Mordhau/Blueprints/Characters/BP_BattleRoyaleCharacter.BP_BattleRoyaleCharacter_C|SetLegArmor _asbp_horde_character _lastlegarmor)))
              (:then_4
                (for (_array_element _array_index) (Variables|Default|GetLastEquipment)
                  (if (Utilities|IsValidClass _array_element)
                    (bind _returnvalue (Game|SpawnActorfromClass _array_element (Math|Transform|MakeTransform "0, 0, 0") "Undefined" 0 0))
                    (Utilities|FlowControl|Sequence
                      (:then_0
                        (CallFunction|CustomizeEquipment _returnvalue))
                      (:then_1
                        (Class|MordhauCharacter|PickUptoSlot _asbp_horde_character _returnvalue (Math|Conversions|ToByte(Integer) _array_index))
                        (if (!= (Utilities|Array|Get(acopy) (Variables|Default|GetLastEquipmentAmmo) _array_index) (Class|MordhauEquipment|GetAmmo _returnvalue))
                          (Class|MordhauEquipment|SetAmmo _returnvalue (Utilities|Array|Get(acopy) (Variables|Default|GetLastEquipmentAmmo) _array_index)))))))))))))
    (:then_1
      (|CallParentFunction APawn))))

(fn ConstructionScript
  (|CallParentFunction))

(fn OnRepPurchaseTrigger
  (Networking|CanExecuteCosmeticEvents
    (:True
      (Audio|PlaySound2D "/Game/Mordhau/Audio/Cues/UI/SC_HordePurchase.SC_HordePurchase" 1.0 1.0 0.0 0 0))))

(fn CustomizeEquipment
  (params (Equipment :type Mordhau%20Equipment%20Object%20Reference))
  (bind _characterprofile (Variables|Default|GetCharacterProfile))
  (bind _appearancecustomization (Utilities|Struct|BreakCharacterProfile _characterprofile))
  (bind (_emblem _emblemcolors) (Utilities|Struct|BreakAppearanceCustomization _appearancecustomization))
  (bind _returnvalue (Class|MordhauEquipment|GetRandomCustomization Equipment true))
  (LocalVariables|SetCustomization _returnvalue)
  (Utilities|FlowControl|Sequence
    (:then_0
      (LocalVariables|SetEmblem _emblem)
      (LocalVariables|SetEmblemColor1 (Utilities|Array|Get(acopy) _emblemcolors))
      (LocalVariables|SetEmblemColor2 (Utilities|Array|Get(acopy) _emblemcolors 1))
      (bind (_outcustomization _returnvalue_2) (Class|MordhauPlayerController|GetDefaultEquipmentCustomizationfor (Utilities|GetClass Equipment)))
      (if _returnvalue_2
        (LocalVariables|SetCustomization _outcustomization)))
    (:then_1
      (Class|MordhauEquipment|AssignCustomization Equipment (LocalVariables|GetCustomization) (Math|Conversions|ToByte(Integer) (LocalVariables|GetEmblem)) (LocalVariables|GetEmblemColor1) (LocalVariables|GetEmblemColor2)))))

(fn OnRepReplicatedSkills
  (CallFunction|SkillsUpdated))

(fn UpgradeSkill
  (params (Skill :type E_HordeSkill%20Enum :default "NewEnumerator0"))
  (bind _returnvalue (Math|Conversions|ToInteger(Byte) Skill))
  (bind _replicatedskills (Variables|Default|GetReplicatedSkills))
  (bind _output (Utilities|Array|Get(acopy) _replicatedskills _returnvalue))
  (Networking|SwitchHasAuthority
    (:Authority
      (if (Utilities|Array|IsValidIndex _replicatedskills _returnvalue)
        (if (CallFunction|HasPrerequisite Skill)
          (if (< _output 5)
            (Utilities|Array|SetArrayElem _replicatedskills _returnvalue (+ _output 1))
            (CallFunction|SkillsUpdated)
            (return true)
            (else
              _)))))
    (:Remote
      _))
  (return false))

(fn GetSkillLevel
  (params (Skill :type E_HordeSkill%20Enum :default "NewEnumerator0"))
  (bind _returnvalue (Math|Conversions|ToInteger(Byte) Skill))
  (bind _replicatedskills (Variables|Default|GetReplicatedSkills))
  (if (Utilities|Array|IsValidIndex _replicatedskills _returnvalue)
    (return (Utilities|Array|Get(acopy) _replicatedskills _returnvalue))
    (else
      (return 0))))

(fn HasPrerequisite
  (params (Skill :type E_HordeSkill%20Enum :default "NewEnumerator0"))
  (bind _skillprerequisites (Variables|Default|GetSkillPrerequisites))
  (bind (_value _returnvalue) (Utilities|Map|Find _skillprerequisites Skill))
  (if _returnvalue
    (if (> (CallFunction|GetSkillLevel _value) 0)
      _
      (else
        (return false))))
  (return true))

(fn SkillsUpdated
  (Networking|SwitchHasAuthority
    (:Authority
      (bind _asbp_horde_character (Utilities|Casting|CastToBP_HordeCharacter (Pawn|GetControlledPawn)))
      (Variables|/Game/Mordhau/Blueprints/Characters/BP_HordeCharacter.BP_HordeCharacter_C|SetReplicatedSkills _asbp_horde_character (Variables|Default|GetReplicatedSkills)))))

(fn GetSkillLevelFloat
  (params (Skill :type E_HordeSkill%20Enum :default "NewEnumerator0"))
  (return (Math|Conversions|ToFloat(Byte) (CallFunction|GetSkillLevel Skill))))

(fn TryFletcherRestock
  (Networking|SwitchHasAuthority
    (:Authority
      (if (<= (Math|Random|RandomFloat) (* (CallFunction|GetSkillLevelFloat "NewEnumerator33") 0.2))
        (bind _returnvalue (Class|MordhauPlayerController|GetLastControlledCharacter))
        (Utilities|IsValid _returnvalue
          (:Is%20Valid
            (if (Class|AdvancedCharacter|GetIsDead _returnvalue)
              (bind _asbp_bow (Utilities|Casting|CastToBP_Bow (Variables|/Script/Mordhau.MordhauCharacter|GetLeftHandEquipment _returnvalue)))
              (Class|MordhauEquipment|SetAmmo _asbp_bow (Class|KismetMathLibrary|BMin (+ (Class|MordhauEquipment|GetAmmo _asbp_bow) 1) (Class|MordhauEquipment|GetCurrentMaxAmmo _asbp_bow))))))))))

(fn TryScatterShot
  (params (SourceProjectile :type Mordhau%20Projectile%20Object%20Reference))
  (bind _returnvalue (Utilities|GetClass SourceProjectile))
  (bind _returnvalue_2 (Transformation|GetActorTransform SourceProjectile))
  (bind (_location _rotation _scale) (Math|Transform|BreakTransform _returnvalue_2))
  (bind (_roll _pitch _yaw) (Math|Rotator|BreakRotator _rotation))
  (bind (_roll_2 _pitch_2 _yaw_2) (Math|Rotator|BreakRotator _rotation))
  (Networking|SwitchHasAuthority
    (:Authority
      (if (not (Variables|Default|GetAvoidScattershotRecursion))
        (Variables|Default|SetAvoidScattershotRecursion true)
        (Utilities|FlowControl|Sequence
          (:then_0
            (if (<= (Math|Random|RandomFloat) (* (CallFunction|GetSkillLevelFloat "NewEnumerator34") 0.1))
              (bind _returnvalue_3 (Class|MordhauPlayerController|GetLastControlledCharacter))
              (Utilities|IsValid _returnvalue_3
                (:Is%20Valid
                  (Utilities|FlowControl|Sequence
                    (:then_0
                      (bind _returnvalue_4 (Game|SpawnActorfromClass _returnvalue (Math|Transform|MakeTransform (Math|Transform|TransformLocation _returnvalue_2 "50.000000,10.000000, 0") (Math|Rotator|MakeRotator _roll _pitch (+ _yaw 2.5)) _scale) "Undefined" 0 0))
                      (Variables|/Script/Mordhau.MordhauProjectile|SetbUsesLocalProjectileBlending _returnvalue_4 false)
                      (CallFunction|AssignFireArrowValues _returnvalue_4)
                      (Class|MordhauProjectile|InitializeProjectile _returnvalue_4 self false _returnvalue_3)
                      (Class|MordhauProjectile|Fire _returnvalue_4))
                    (:then_1
                      (bind _returnvalue_5 (Game|SpawnActorfromClass _returnvalue (Math|Transform|MakeTransform (Math|Transform|TransformLocation _returnvalue_2 "50.000000,-10.000000, 0") (Math|Rotator|MakeRotator _roll_2 _pitch_2 (+ _yaw_2 -2.5)) _scale) "Undefined" 0 0))
                      (Variables|/Script/Mordhau.MordhauProjectile|SetbUsesLocalProjectileBlending _returnvalue_5 false)
                      (CallFunction|AssignFireArrowValues _returnvalue_5)
                      (Class|MordhauProjectile|InitializeProjectile _returnvalue_5 self false _returnvalue_3)
                      (Class|MordhauProjectile|Fire _returnvalue_5)))))))
          (:then_1
            (Variables|Default|SetAvoidScattershotRecursion false)))))))

(fn AssignFireArrowValues
  (params (Arrow :type Actor%20Object%20Reference))
  (bind _asbp_arrow_projectile (Utilities|Casting|CastToBP_ArrowProjectile Arrow))
  (if (> (CallFunction|GetSkillLevel "NewEnumerator35") 0)
    (Variables|/Game/Mordhau/Blueprints/Equipment/Ranged/BP_ArrowProjectile.BP_ArrowProjectile_C|SetFireDamage _asbp_arrow_projectile 1e+01)
    (Variables|/Game/Mordhau/Blueprints/Equipment/Ranged/BP_ArrowProjectile.BP_ArrowProjectile_C|SetFireDuration _asbp_arrow_projectile (* (CallFunction|GetSkillLevelFloat "NewEnumerator35") 0.5))
    (Variables|/Game/Mordhau/Blueprints/Equipment/Ranged/BP_ArrowProjectile.BP_ArrowProjectile_C|SetFireTick _asbp_arrow_projectile 0.5)))