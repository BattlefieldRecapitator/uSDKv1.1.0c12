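; Horde-mode shop item that players buy with coins, either as new equipment or wearable upgrade, or as ammo restock for equipment they carry.
; Registers with the Horde game state; interaction deducts cost, spawns or restocks, and bumps the controller's PurchaseTrigger.
; InitializeDisplay copies equipment meshes from a briefly spawned actor, or uses the quiver mesh for ammo.
; UpdateVisuals initializes lazily, tracks local affordability and toggles the widget by camera distance with hysteresis.
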(event EventBeginPlay
  (|CallParentFunction)
  (Networking|CanExecuteCosmeticEvents
    (:True
      (bind _asbp_horde_game_state (Utilities|Casting|CastToBP_HordeGameState (Game|GetGameState)))
      (Utilities|Array|AddUnique (Variables|/Game/Mordhau/Blueprints/GameModes/Horde/BP_HordeGameState.BP_HordeGameState_C|GetPurchasables _asbp_horde_game_state) self))))

(event Collision|EventActorBeginOverlap
  (params (OtherActor :type Actor%20Object%20Reference))
  (|CallParentFunction OtherActor) ; This node is disabled and will not be called.\nDrag off pins to build functionality.
)

(event EventOnInteractionStart
  (params (Character :type Mordhau%20Character%20Object%20Reference))
  (bind _cost (Variables|Default|GetCost))
  (Utilities|IsValid Character
    (:Is%20Valid
      (bind _asbp_horde_player_state (Utilities|Casting|CastToBP_HordePlayerState (Variables|/Script/Engine.Pawn|GetPlayerState Character)))
      (if (>= (Variables|/Game/Mordhau/Blueprints/GameModes/Horde/BP_HordePlayerState.BP_HordePlayerState_C|GetCoins _asbp_horde_player_state) _cost)
        (Variables|/Game/Mordhau/Blueprints/GameModes/Horde/BP_HordePlayerState.BP_HordePlayerState_C|SetCoins _asbp_horde_player_state (- (Variables|/Game/Mordhau/Blueprints/GameModes/Horde/BP_HordePlayerState.BP_HordePlayerState_C|GetCoins _asbp_horde_player_state) _cost))
        (bind _asbp_battle_royale_character (Utilities|Casting|CastToBP_BattleRoyaleCharacter Character))
        (Utilities|FlowControl|Sequence
          (:then_0
            (if (Variables|Default|GetIsAmmoRestock)
              (bind _asmordhau_equipment (Utilities|Casting|CastToMordhauEquipmentClass (Variables|Default|GetPurchasableClass)))
              (bind _returnvalue (Class|MordhauCharacter|FindEquipmenttoRestock _asbp_battle_royale_character (Utilities|Array|MakeArray _asmordhau_equipment)))
              (Utilities|IsValid _returnvalue
                (:Is%20Valid
                  (Class|MordhauEquipment|SetAmmo _returnvalue (Class|KismetMathLibrary|BMin (+ (Class|MordhauEquipment|GetAmmo _returnvalue) (Math|Conversions|ToByte(Integer) (Variables|Default|GetAmmoRestockAmount))) (Class|MordhauEquipment|GetCurrentMaxAmmo _returnvalue)))))
              (else
                (CallFunction|SpawnItem _asbp_battle_royale_character))))
          (:then_1
            (bind _asbp_horde_player_controller (Utilities|Casting|CastToBP_HordePlayerController (Pawn|GetController _asbp_battle_royale_character)))
            (Variables|/Game/Mordhau/Blueprints/GameModes/Horde/BP_HordePlayerController.BP_HordePlayerController_C|SetPurchaseTrigger _asbp_horde_player_controller (+ (Variables|/Game/Mordhau/Blueprints/GameModes/Horde/BP_HordePlayerController.BP_HordePlayerController_C|GetPurchaseTrigger _asbp_horde_player_controller) 1))))))))

(fn ConstructionScript
  (|CallParentFunction))

(fn CanInteract
  (params (Character :type Mordhau%20Character%20Object%20Reference))
  (Utilities|IsValid Character
    (:Is%20Valid
      (bind _asbp_horde_player_state (Utilities|Casting|CastToBP_HordePlayerState (Variables|/Script/Engine.Pawn|GetPlayerState Character))
        (:then
          (if (>= (Variables|/Game/Mordhau/Blueprints/GameModes/Horde/BP_HordePlayerState.BP_HordePlayerState_C|GetCoins _asbp_horde_player_state) (Variables|Default|GetCost))
            (if (Variables|Default|GetIsAmmoRestock) :!label _label
              (bind _asmordhau_equipment (Utilities|Casting|CastToMordhauEquipmentClass (Variables|Default|GetPurchasableClass))
                (:then
                  (bind _returnvalue (Class|MordhauCharacter|FindEquipmenttoRestock Character (Utilities|Array|MakeArray _asmordhau_equipment)))
                  (Utilities|IsValid _returnvalue
                    (:Is%20Valid
                      _)
                    (:Is%20Not%20Valid
                      (return false))))
                (:CastFailed
                  (return false))))
            (else
              (return false))))
        (:CastFailed
          (goto _label))))
    (:Is%20Not%20Valid
      _))
  (return (stale _returnvalue)))

(fn SetAvailability
  (params (NewAvailable :type Boolean))
  (Variables|Default|SetIsAvailable NewAvailable))

(fn SpawnItem
  (params (ForCharacter :type BP%20Battle%20Royale%20Character%20Object%20Reference))
  (bind _purchasableclass (Variables|Default|GetPurchasableClass))
  (if (Utilities|IsValidClass _purchasableclass)
    (bind _returnvalue (Game|SpawnActorfromClass _purchasableclass (Transformation|GetActorTransform) "Undefined" 0 0))
    (bind _asmordhau_equipment (Utilities|Casting|CastToMordhauEquipment _returnvalue)
      (:then
        (bind _returnvalue_2 (Class|MordhauEquipment|GetRandomCustomization _asmordhau_equipment true))
        (LocalVariables|SetCustomization _returnvalue_2)
        (Utilities|FlowControl|Sequence
          (:then_0
            (bind _asmordhau_player_controller (Utilities|Casting|CastToMordhauPlayerController (Pawn|GetController ForCharacter)))
            (LocalVariables|SetEmblem (.Emblem (Utilities|Struct|BreakAppearanceCustomization (.AppearanceCustomization (Utilities|Struct|BreakCharacterProfile (Variables|/Script/Mordhau.MordhauPlayerController|GetCharacterProfile _asmordhau_player_controller))))))
            (LocalVariables|SetEmblemColor1 (Utilities|Array|Get(acopy) (.EmblemColors (Utilities|Struct|BreakAppearanceCustomization (.AppearanceCustomization (Utilities|Struct|BreakCharacterProfile (Variables|/Script/Mordhau.MordhauPlayerController|GetCharacterProfile _asmordhau_player_controller)))))))
            (LocalVariables|SetEmblemColor2 (Utilities|Array|Get(acopy) (.EmblemColors (Utilities|Struct|BreakAppearanceCustomization (.AppearanceCustomization (Utilities|Struct|BreakCharacterProfile (Variables|/Script/Mordhau.MordhauPlayerController|GetCharacterProfile _asmordhau_player_controller))))) 1))
            (bind (_outcustomization _returnvalue_3) (Class|MordhauPlayerController|GetDefaultEquipmentCustomizationfor _asmordhau_player_controller (Utilities|GetClass _asmordhau_equipment)))
            (if _returnvalue_3
              (LocalVariables|SetCustomization _outcustomization)))
          (:then_1
            (Class|MordhauEquipment|AssignCustomization _asmordhau_equipment (LocalVariables|GetCustomization) (Math|Conversions|ToByte(Integer) (LocalVariables|GetEmblem)) (LocalVariables|GetEmblemColor1) (LocalVariables|GetEmblemColor2))
            (Class|MordhauEquipment|RestockOtherEquipmentonCharacter _asmordhau_equipment ForCharacter)
            (if (not (and (Variables|/Script/Mordhau.MordhauEquipment|GetbDestroyIfNoAmmo _asmordhau_equipment) (== (Class|MordhauEquipment|GetAmmo _asmordhau_equipment) 0)))
              (bind _returnvalue_4 (Class|MordhauCharacter|PickUp ForCharacter _asmordhau_equipment))
              (if _returnvalue_4
                (Class|MordhauCharacter|SwitchEquipment ForCharacter _asmordhau_equipment)
                (else
                  (Variables|/Script/Mordhau.MordhauEquipment|SetbCanRagdoll _asmordhau_equipment true)
                  (Class|MordhauEquipment|UpdateEquipmentState _asmordhau_equipment)))))))
      (:CastFailed
        (bind _asbp_wearable_pickup (Utilities|Casting|CastToBP_WearablePickup _returnvalue))
        (Default|EquipifUpgrade _asbp_wearable_pickup ForCharacter)))))

(fn InitializeDisplay
  (bind _lodskeletalmesh (Variables|Default|GetLODSkeletalMesh))
  (bind _staticmesh (Variables|Default|GetStaticMesh))
  (bind _purchasableclass (Variables|Default|GetPurchasableClass))
  (Utilities|FlowControl|Sequence
    (:then_0
      (if (Variables|Default|GetIsAmmoRestock)
        (Class|SkinnedMeshComponent|SetSkeletalMesh (Variables|Default|GetLODSkeletalMesh) 0 true)
        (bind _asmordhau_equipment (Utilities|Casting|CastToMordhauEquipmentClass _purchasableclass))
        (bind _asmordhau_equipment_2 (Utilities|Casting|CastToMordhauEquipment (Class|MordhauUtilityLibrary|GetDefaultActor _asmordhau_equipment)))
        (Variables|Default|SetName (Utilities|Text|FormatText "{a} Ammo" (Variables|/Script/Mordhau.MordhauEquipment|GetEquipmentName _asmordhau_equipment_2)))
        (bind _asquiver (Utilities|Casting|CastToQuiver (Class|MordhauUtilityLibrary|GetDefaultObject (Variables|/Script/Mordhau.MordhauEquipment|GetQuiver _asmordhau_equipment_2))))
        (Components|StaticMesh|SetStaticMesh _staticmesh (Utilities|Array|Get(acopy) (Variables|/Script/Mordhau.Quiver|GetQuiverMeshes _asquiver) (- (Utilities|Array|Length (Variables|/Script/Mordhau.Quiver|GetQuiverMeshes _asquiver)) 1)))
        (for _index (range 0 (- (Rendering|Material|GetNumMaterials _staticmesh) 1))
          (bind _returnvalue (Rendering|Material|CreateDynamicMaterialInstance _staticmesh _index 0 "None" :!class /Script/Engine.PrimitiveComponent))
          (Rendering|Material|SetScalarParameterValue _returnvalue "ShineIntensity" 1.0 :!class /Script/Engine.MaterialInstanceDynamic))
        (else
          (Components|StaticMesh|SetStaticMesh (Variables|Default|GetStaticMesh) 0)
          (Utilities|FlowControl|Sequence
            (:then_0
              (bind _returnvalue_2 (Game|SpawnActorfromClass _purchasableclass (Transformation|GetActorTransform) "Undefined" 0 0))
              (bind _asmordhau_equipment_3 (Utilities|Casting|CastToMordhauEquipment _returnvalue_2)
                (:then
                  (Variables|Default|SetName (Variables|/Script/Mordhau.MordhauEquipment|GetEquipmentName _asmordhau_equipment_3))
                  (Variables|/Script/Mordhau.MordhauEquipment|SetbForceInstantMeshUpdate _asmordhau_equipment_3 true)
                  (bind _returnvalue_3 (Class|MordhauEquipment|GetRandomCustomization _asmordhau_equipment_3 true))
                  (Class|MordhauEquipment|AssignCustomization _asmordhau_equipment_3 _returnvalue_3)
                  (Class|SkinnedMeshComponent|SetSkeletalMesh _lodskeletalmesh (Variables|/Script/Engine.SkinnedMeshComponent|GetSkeletalMesh (Variables|/Script/Mordhau.MordhauEquipment|GetSkeletalMeshComponent _asmordhau_equipment_3)) true)
                  (Components|SkinnedMesh|SetPhysicsAsset _lodskeletalmesh (Variables|/Script/Mordhau.MordhauEquipment|GetPhysicsAsset _asmordhau_equipment_3) false)
                  (for _index_2 (range 0 (- (Rendering|Material|GetNumMaterials (Variables|/Script/Mordhau.MordhauEquipment|GetSkeletalMeshComponent _asmordhau_equipment_3)) 1))
                    (Rendering|Material|SetMaterial _lodskeletalmesh _index_2 (Rendering|Material|GetMaterial (Variables|/Script/Mordhau.MordhauEquipment|GetSkeletalMeshComponent _asmordhau_equipment_3) _index_2))
                    (bind _asmaterial_instance_dynamic (Utilities|Casting|CastToMaterialInstanceDynamic (Rendering|Material|GetMaterial (Variables|/Script/Mordhau.MordhauEquipment|GetSkeletalMeshComponent _asmordhau_equipment_3) _index_2)))
                    (Rendering|Material|SetScalarParameterValue _asmaterial_instance_dynamic "ShineIntensity" 1.0 :!class /Script/Engine.MaterialInstanceDynamic)))
                (:CastFailed
                  (bind _asbp_wearable_pickup (Utilities|Casting|CastToBP_WearablePickup _returnvalue_2)))))
            (:then_1
              (Actor|DestroyActor _returnvalue_2))))))
    (:then_1
      (bind _returnvalue_4 (AddComponent|AddMordhauWidgetComponent false (Math|Transform|MakeTransform (Class|MordhauUtilityLibrary|GetComponentsBoundingBoxinActorSpace self))))
      (Variables|Default|SetWidget _returnvalue_4))
    (:then_2
      (CallFunction|SetAvailability false)
      (Variables|Default|SetInitialized true))))

(fn UpdateVisuals
  (bind _returnvalue (Math|Float|MakeLiteralFloat 8e+02))
  (bind _returnvalue_2 (Game|GetPlayerCameraManager 0))
  (bind _returnvalue_3 (Transformation|GetActorLocation))
  (bind _returnvalue_4 (Game|GetPlayerController 0))
  (bind _isavailable (Variables|Default|GetIsAvailable))
  (bind _returnvalue_5 (Camera|GetCameraLocation _returnvalue_2))
  (bind _returnvalue_6 (- _returnvalue_3 _returnvalue_5))
  (bind _returnvalue_7 (Math|Vector|VectorLength _returnvalue_6))
  (if (Utilities|IsValidClass (Variables|Default|GetPurchasableClass))
    (Utilities|FlowControl|Sequence
      (:then_0
        (if (not (Variables|Default|GetInitialized))
          (CallFunction|InitializeDisplay)))
      (:then_1
        (Utilities|IsValid _returnvalue_4
          (:Is%20Valid
            (if (Pawn|IsLocalPlayerController _returnvalue_4)
              (Utilities|FlowControl|Sequence
                (:then_0
                  (bind _asbp_horde_player_state (Utilities|Casting|CastToBP_HordePlayerState (Variables|/Script/Engine.Controller|GetPlayerState _returnvalue_4)))
                  (if (not (Math|Boolean|Equal(Boolean) _isavailable (>= (Variables|/Game/Mordhau/Blueprints/GameModes/Horde/BP_HordePlayerState.BP_HordePlayerState_C|GetCoins _asbp_horde_player_state) (Variables|Default|GetCost))))
                    (CallFunction|SetAvailability (not _isavailable))))
                (:then_1
                  (Utilities|FlowControl|Sequence
                    (:then_0
                      (Variables|Default|SetIsValid true)
                      (if (Variables|Default|GetIsAmmoRestock)
                        (bind _asmordhau_equipment (Utilities|Casting|CastToMordhauEquipmentClass (Variables|Default|GetPurchasableClass)))
                        (bind _asbp_horde_character (Utilities|Casting|CastToBP_HordeCharacter (Pawn|GetControlledPawn _returnvalue_4))
                          (:then
                            (bind _returnvalue_8 (Class|MordhauCharacter|FindEquipmenttoRestock _asbp_horde_character (Utilities|Array|MakeArray _asmordhau_equipment)))
                            (Utilities|IsValid _returnvalue_8
                              (:Is%20Not%20Valid
                                _)))
                          (:CastFailed
                            _))
                        (Variables|Default|SetIsValid false)))
                    (:then_1
                      (if (!= (Variables|/Script/Mordhau.MordhauWidgetComponent|GetOverrideVisible (Variables|Default|GetWidget)) 0)
                        (if (not (< _returnvalue_7 (+ _returnvalue 25.0)))
                          (Variables|/Script/Mordhau.MordhauWidgetComponent|SetOverrideVisible (Variables|Default|GetWidget) 0))
                        (elif (< _returnvalue_7 _returnvalue)
                          (Variables|/Script/Mordhau.MordhauWidgetComponent|SetOverrideVisible (Variables|Default|GetWidget) -1))))))))))))))