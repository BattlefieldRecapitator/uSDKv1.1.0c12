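; Base Horde mode chest that players buy with coins, deducting the cost on interaction and calling BreakChest with the buyer's controller.
; CanInteract refuses players who cannot afford it.
; On cosmetic-capable instances it registers in the Horde game state's Purchasables list.
; UpdateVisuals syncs availability to the local player's coins and toggles the widget by destroyed state and camera distance, with hysteresis against flicker.
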(event EventBeginPlay
  (|CallParentFunction)
  (Networking|CanExecuteCosmeticEvents
    (:True
      (CallFunction|SetAvailability false)
      (bind _asbp_horde_game_state (Utilities|Casting|CastToBP_HordeGameState (Game|GetGameState)))
      (Utilities|Array|AddUnique (Variables|/Game/Mordhau/Blueprints/GameModes/Horde/BP_HordeGameState.BP_HordeGameState_C|GetPurchasables _asbp_horde_game_state) self))))

(event Collision|EventActorBeginOverlap
  (params (OtherActor :type Actor%20Object%20Reference))
  (|CallParentFunction OtherActor) ; This node is disabled and will not be called.\nDrag off pins to build functionality.
)

(event EventOnInteractionStart
  (params (Character :type Mordhau%20Character%20Object%20Reference))
  (bind _cost (Variables|Default|GetCost))
  (Utilities|IsValid Character
    (:Is%20Valid
      (bind _asbp_horde_player_state (Utilities|Casting|CastToBP_HordePlayerState (Variables|/Script/Engine.Pawn|GetPlayerState Character)))
      (if (>= (Variables|/Game/Mordhau/Blueprints/GameModes/Horde/BP_HordePlayerState.BP_HordePlayerState_C|GetCoins _asbp_horde_player_state) _cost)
        (Variables|/Game/Mordhau/Blueprints/GameModes/Horde/BP_HordePlayerState.BP_HordePlayerState_C|SetCoins _asbp_horde_player_state (- (Variables|/Game/Mordhau/Blueprints/GameModes/Horde/BP_HordePlayerState.BP_HordePlayerState_C|GetCoins _asbp_horde_player_state) _cost))
        (bind _asbp_horde_player_controller (Utilities|Casting|CastToBP_HordePlayerController (Pawn|GetController Character))
          (:then
            (CallFunction|BreakChest _asbp_horde_player_controller))
          (:CastFailed
            (CallFunction|BreakChest)))))))

(event Game|Damage|EventAnyDamage
  (params (Damage :type Float%20%28single-precision%29) (DamageType :type Damage%20Type%20Object%20Reference) (InstigatedBy :type Controller%20Object%20Reference) (DamageCauser :type Actor%20Object%20Reference)))

(fn ConstructionScript
  (|CallParentFunction))

(fn CanInteract
  (params (Character :type Mordhau%20Character%20Object%20Reference))
  (Utilities|IsValid Character
    (:Is%20Valid
      (bind _asbp_horde_player_state (Utilities|Casting|CastToBP_HordePlayerState (Variables|/Script/Engine.Pawn|GetPlayerState Character))
        (:then
          (if (>= (Variables|/Game/Mordhau/Blueprints/GameModes/Horde/BP_HordePlayerState.BP_HordePlayerState_C|GetCoins _asbp_horde_player_state) (Variables|Default|GetCost))
            _
            (else
              (return false))))
        (:CastFailed
          _)))
    (:Is%20Not%20Valid
      _))
  (return (|CallParentFunction Character)))

(fn SetAvailability
  (params (NewAvailable :type Boolean))
  (Variables|Default|SetIsAvailable NewAvailable))

(fn UpdateVisuals
  (bind _returnvalue (Game|GetPlayerCameraManager 0))
  (bind _returnvalue_2 (Math|Float|MakeLiteralFloat 8e+02))
  (bind _returnvalue_3 (Transformation|GetActorLocation))
  (bind _returnvalue_4 (Game|GetPlayerController 0))
  (bind _isavailable (Variables|Default|GetIsAvailable))
  (bind _mordhauwidget (Variables|Default|GetMordhauWidget))
  (bind _returnvalue_5 (Camera|GetCameraLocation _returnvalue))
  (bind _returnvalue_6 (- _returnvalue_5 _returnvalue_3))
  (bind _returnvalue_7 (Math|Vector|VectorLength _returnvalue_6))
  (Utilities|IsValid _returnvalue_4
    (:Is%20Valid
      (if (Pawn|IsLocalPlayerController _returnvalue_4)
        (bind _asbp_horde_player_state (Utilities|Casting|CastToBP_HordePlayerState (Variables|/Script/Engine.Controller|GetPlayerState _returnvalue_4)))
        (if (Variables|Default|GetChestDestroyed)
          (Variables|/Script/Mordhau.MordhauWidgetComponent|SetOverrideVisible (Variables|Default|GetMordhauWidget) 0)
          (else
            (Utilities|FlowControl|Sequence
              (:then_0
                (if (not (Math|Boolean|Equal(Boolean) _isavailable (>= (Variables|/Game/Mordhau/Blueprints/GameModes/Horde/BP_HordePlayerState.BP_HordePlayerState_C|GetCoins _asbp_horde_player_state) (Variables|Default|GetCost))))
                  (CallFunction|SetAvailability (not _isavailable))))
              (:then_1
                (if (!= (Variables|/Script/Mordhau.MordhauWidgetComponent|GetOverrideVisible _mordhauwidget) 0)
                  (if (not (< _returnvalue_7 (+ _returnvalue_2 25.0)))
                    (Variables|/Script/Mordhau.MordhauWidgetComponent|SetOverrideVisible _mordhauwidget 0))
                  (elif (< _returnvalue_7 _returnvalue_2)
                    (Variables|/Script/Mordhau.MordhauWidgetComponent|SetOverrideVisible _mordhauwidget -1)))))))))))