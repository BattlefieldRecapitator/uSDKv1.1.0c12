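; Horde mode game state that handles client-facing match feedback and decides when spawn info text is hidden.
; On cosmetic-capable instances it gathers purchasables and chests at BeginPlay, then round-robins a few visual updates per tick to spread the cost.
; Replicated match info changes override surviving enemies' widget visibility when few remain and play sounds as the enemy count leaves or reaches zero.
; Match end shows victory, or defeat with the wave reached.
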(event EventHandleMatchEndInfo
  (|CallParentFunction)
  (bind _asbp_mordhau_hud (Utilities|Casting|CastToBP_MordhauHUD (Class|MordhauUtilityLibrary|GetMordhauHUD)))
  (if (== (.WinnerTeam (Utilities|Struct|BreakSTRUCT_MatchEndInfo (Variables|Default|GetMatchEndInfo))) 0)
    (Default|ShowMatchResult _asbp_mordhau_hud true "victory")
    (else
      (Default|ShowMatchResult _asbp_mordhau_hud false "defeat" (Utilities|Text|FormatText "Reached Wave {a}" (+ (.Wave (Utilities|Struct|BreakSTRUCT_HordeMatchInfo (Variables|Default|GetReplicatedHordeMatchInfo))) 1))))))

(event EventBeginPlay
  (|CallParentFunction)
  (Networking|CanExecuteCosmeticEvents
    (:True
      (bind _outactors (Actor|GetAllActorsOfClass "/Game/Mordhau/Blueprints/GameModes/Horde/BP_HordePurchasable.BP_HordePurchasable_C"))
      (Variables|Default|SetPurchasables _outactors)
      (bind _outactors_2 (Actor|GetAllActorsOfClass "/Game/Mordhau/Blueprints/GameModes/Horde/BP_HordeChestBase.BP_HordeChestBase_C"))
      (Utilities|Array|AppendArray (Variables|Default|GetPurchasables) _outactors_2))))

(event EventTick
  (params (DeltaSeconds :type Float%20%28single-precision%29))
  (|CallParentFunction DeltaSeconds)
  (Networking|CanExecuteCosmeticEvents
    (:True
      (if (> (Utilities|Array|Length (Variables|Default|GetPurchasables)) 0)
        (for _index (range 1 3)
          (CallFunction|UpdateNextPurchasableVisuals))))))

(fn ConstructionScript
  (|CallParentFunction))

(fn UpdateNextPurchasableVisuals
  (bind _purchasables (Variables|Default|GetPurchasables))
  (Utilities|FlowControl|Sequence
    (:then_0
      (if (not (Utilities|Array|IsValidIndex _purchasables (Variables|Default|GetPurchasableIndex)))
        (Variables|Default|SetPurchasableIndex 0)))
    (:then_1
      (bind _asbp_horde_purchasable (Utilities|Casting|CastToBP_HordePurchasable (Utilities|Array|Get(acopy) _purchasables (Variables|Default|GetPurchasableIndex)))
        (:then
          (Default|UpdateVisuals _asbp_horde_purchasable))
        (:CastFailed
          (bind _asbp_horde_chest_base (Utilities|Casting|CastToBP_HordeChestBase (Utilities|Array|Get(acopy) _purchasables (Variables|Default|GetPurchasableIndex))))
          (Default|UpdateVisuals _asbp_horde_chest_base))))
    (:then_2
      (Variables|Default|SetPurchasableIndex (+ (Variables|Default|GetPurchasableIndex) 1)))))

(fn OnRepReplicatedHordeMatchInfo
  (bind _replicatedhordematchinfo (Variables|Default|GetReplicatedHordeMatchInfo))
  (bind _enemiesremaining (Utilities|Struct|BreakSTRUCT_HordeMatchInfo _replicatedhordematchinfo))
  (Utilities|FlowControl|Sequence
    (:then_0
      (if (and (or (> (Variables|Default|GetLastReplicatedEnemiesRemaining) 3) (== (Variables|Default|GetLastReplicatedEnemiesRemaining) 0)) (and (<= _enemiesremaining 3) (> _enemiesremaining 0)))
        (bind _outactors (Actor|GetAllActorsOfClass "/Game/Mordhau/Blueprints/GameModes/Horde/BP_HordeEnemy.BP_HordeEnemy_C"))
        (for _array_element _outactors
          (if (not (Class|AdvancedCharacter|GetIsDead _array_element))
            (Variables|/Script/Mordhau.MordhauWidgetComponent|SetOverrideVisible (Variables|/Game/Mordhau/Blueprints/GameModes/Horde/BP_HordeEnemy.BP_HordeEnemy_C|GetMordhauWidget _array_element) -1)))))
    (:then_1
      (if (> (Utilities|Time|GetTimeSeconds) 2.0)
        (if (and (== (Variables|Default|GetLastReplicatedEnemiesRemaining) 0) (!= _enemiesremaining 0))
          (Audio|PlaySound2D "/Game/Mordhau/UI/UIAssets/Sounds/EnemyCapped.EnemyCapped" 1.0 1.0 0.0 0 0)
          (elif (and (!= (Variables|Default|GetLastReplicatedEnemiesRemaining) 0) (== _enemiesremaining 0))
            (Audio|PlaySound2D "/Game/Mordhau/UI/UIAssets/Sounds/FriendlyCapped.FriendlyCapped" 1.0 1.0 0.0 0 0)))))
    (:then_2
      (Variables|Default|SetLastReplicatedEnemiesRemaining _enemiesremaining))))

(fn ShouldHideSpawnInfoText
  (if (Math|Boolean|ORBoolean (not (Class|GameStateBase|HasMatchStarted)) (Variables|Default|GetMatchEndInfoReplicated) (== (.EnemiesRemaining (Utilities|Struct|BreakSTRUCT_HordeMatchInfo (Variables|Default|GetReplicatedHordeMatchInfo))) 0))
    (return true)
    (else
      (return false))))