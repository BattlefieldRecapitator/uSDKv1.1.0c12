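; BP_ScenarioPlayerController is the player controller for Scenario game modes, letting the mode override the player's character customization.
; After the parent validates a new profile from the client, it casts the game mode to BP_ScenarioGameMode.
; If that mode's override flag is set, it replaces the pending character profile with the mode's default player profile.
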(event EventBeginPlay
  (|CallParentFunction) ; This node is disabled and will not be called.\nDrag off pins to build functionality.
)

(event EventTick
  (params (DeltaSeconds :type Float%20%28single-precision%29))
  (|CallParentFunction DeltaSeconds) ; This node is disabled and will not be called.\nDrag off pins to build functionality.
)

(event EventOnNewProfilefromClientPostValidation
  (|CallParentFunction)
  (bind _asbp_scenario_game_mode (Utilities|Casting|CastToBP_ScenarioGameMode (Game|GetGameMode)))
  (if (Variables|/Game/Mordhau/Blueprints/GameModes/Scenario/BP_ScenarioGameMode.BP_ScenarioGameMode_C|GetOverrideDefaultPlayerCustomization _asbp_scenario_game_mode)
    (Variables|Default|SetPendingCharacterProfile (Variables|/Game/Mordhau/Blueprints/GameModes/Scenario/BP_ScenarioGameMode.BP_ScenarioGameMode_C|GetOverrideDefaultPlayerProfile _asbp_scenario_game_mode))))

(fn ConstructionScript
  (|CallParentFunction))