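; Environmental hazard volume that kills living players and horses moving fast enough into it along its local negative X axis, then impales their bodies.
; On Tick, the authority checks box overlaps and applies lethal damage with the volume as agent.
; The kill event cosmetically ragdolls the victim and pins its spine or neck bone to the box's -X face with a new physics handle.
; Tick also removes handles without a valid grabbed component.
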(event EventOnUsedtoKillOther
  (params (Character :type Advanced%20Character%20Object%20Reference) (Type :type EMordhauDamageType%20Enum :default "Generic") (SubType :type Byte :default 0) (bone :type Name%20%28by%20ref%29 :default "None") (Point :type Vector%20%28by%20ref%29 :default "0, 0, 0") (Source :type Actor%20Object%20Reference))
  (Networking|CanExecuteCosmeticEvents
    (:True
      (CallFunction|StickyCharacter Character))))

(event EventTick
  (params (DeltaSeconds :type Float%20%28single-precision%29))
  (Utilities|FlowControl|Sequence
    (:then_0
      (Networking|SwitchHasAuthority
        (:Authority
          (CallFunction|CheckVolume))))
    (:then_1
      (Utilities|Array|Clear (Variables|Default|GetPhysicsHandlesToRemove))
      (for _array_element (Variables|Default|GetPhysicsHandles)
        (Utilities|IsValid _array_element
          (:Is%20Valid
            (Utilities|IsValid (Class|PhysicsHandleComponent|GetGrabbedComponent _array_element)
              (:Is%20Not%20Valid
                _)))
          (:Is%20Not%20Valid
            _))
        (Utilities|Array|Add (Variables|Default|GetPhysicsHandlesToRemove) _array_element))
      (for _array_element_2 (Variables|Default|GetPhysicsHandlesToRemove)
        (Utilities|IsValid _array_element_2
          (:Is%20Valid
            (Components|DestroyComponent _array_element_2))
          (:Is%20Not%20Valid
            _))
        (Utilities|Array|RemoveItem (Variables|Default|GetPhysicsHandles) _array_element_2)))))

(fn ConstructionScript)

(fn CheckVolume
  (bind _output_get (LocalVariables|SetOverlappingActors (Collision|GetOverlappingActors (Variables|Default|GetBox) "/Script/Mordhau.AdvancedCharacter" :!class /Script/Engine.PrimitiveComponent)))
  (for _array_element _output_get
    (bind _asadvanced_character (Utilities|Casting|CastToAdvancedCharacter _array_element))
    (if (not (Class|AdvancedCharacter|GetIsDead _asadvanced_character))
      (Utilities|Casting|CastToMordhauCharacter _asadvanced_character
        (:then
          _)
        (:CastFailed
          (Utilities|Casting|CastToHorse _asadvanced_character)))
      (if (<= (.X (Math|Vector|BreakVector (Math|Vector|UnrotateVector (Transformation|GetVelocity _asadvanced_character) (Transformation|GetWorldRotation (Variables|Default|GetBox))))) (* (Variables|Default|GetVelocityToKill) -1.0))
        (Class|AdvancedCharacter|MordhauTakeDamage _asadvanced_character 1e+03 (Collision|MakeHitResult false false 0.0 0.0 "0, 0, 0" "0, 0, 0" "0,0,1" "0,0,1" 0 0) "Generic" 0 _asadvanced_character self)))))

(fn StickyCharacter
  (params (Character :type Advanced%20Character%20Object%20Reference))
  (bind _box (Variables|Default|GetBox))
  (bind _box_2 (Variables|Default|GetBox))
  (bind _mesh (Variables|/Script/Engine.Character|GetMesh Character))
  (bind _returnvalue (Transformation|GetWorldTransform _box_2))
  (bind _returnvalue_2 (Components|Box|GetUnscaledBoxExtent _box))
  (bind (_x _y _z) (Math|Vector|BreakVector _returnvalue_2))
  (Utilities|FlowControl|Sequence
    (:then_0
      (Utilities|Casting|CastToMordhauCharacter Character
        (:then
          (LocalVariables|SetBoneToSticky "Spine1"))
        (:CastFailed
          (Utilities|Casting|CastToHorse Character
            (:then
              (LocalVariables|SetBoneToSticky "Neck2"))
            (:CastFailed
              (return))))))
    (:then_1
      (bind _returnvalue_3 (AddComponent|AddPhysicsHandleComponent))
      (Utilities|Array|Add (Variables|Default|GetPhysicsHandles) _returnvalue_3)
      (Class|AdvancedCharacter|StartRagdoll Character)
      (Physics|Components|PhysicsHandle|GrabComponentatLocationwithRotation _returnvalue_3 _mesh (LocalVariables|GetBoneToSticky) (Transformation|GetSocketLocation _mesh (LocalVariables|GetBoneToSticky)) (Transformation|GetSocketRotation _mesh (LocalVariables|GetBoneToSticky)))
      (Physics|Components|PhysicsHandle|SetTargetLocation _returnvalue_3 (Math|Transform|TransformLocation _returnvalue (Math|Vector|MakeVector (* _x -1.0) (Math|Float|Clamp(Float) (.Y (Math|Vector|BreakVector (Math|Transform|InverseTransformLocation _returnvalue (Transformation|GetSocketLocation _mesh (LocalVariables|GetBoneToSticky))))) (* _y -1.0) _y) (Math|Float|Clamp(Float) (.Z (Math|Vector|BreakVector (Math|Transform|InverseTransformLocation _returnvalue (Transformation|GetSocketLocation _mesh (LocalVariables|GetBoneToSticky))))) (* _z -1.0) _z)))))))