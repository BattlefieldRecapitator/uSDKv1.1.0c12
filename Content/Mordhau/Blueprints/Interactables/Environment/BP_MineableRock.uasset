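; BP_MineableRock is an interactable environment rock that yields steel ingots when mined with a pickaxe.
; On AnyDamage it checks that the damage causer is a Mordhau character in an attack motion, making a left or right strike with BP_Pickaxe.
; A hit counter gates production, though its current threshold yields an item on every valid hit.
; ProduceItem spawns the ingot at SpawnPoint and assigns it a zeroed equipment customization.
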(event EventBeginPlay
  (|CallParentFunction) ; This node is disabled and will not be called.\nDrag off pins to build functionality.
)

(event Collision|EventActorBeginOverlap
  (params (OtherActor :type Actor%20Object%20Reference))
  (|CallParentFunction OtherActor) ; This node is disabled and will not be called.\nDrag off pins to build functionality.
)

(event EventTick
  (params (DeltaSeconds :type Float%20%28single-precision%29))
  (|CallParentFunction DeltaSeconds) ; This node is disabled and will not be called.\nDrag off pins to build functionality.
)

(event Game|Damage|EventAnyDamage
  (params (Damage :type Float%20%28single-precision%29) (DamageType :type Damage%20Type%20Object%20Reference) (InstigatedBy :type Controller%20Object%20Reference) (DamageCauser :type Actor%20Object%20Reference))
  (bind _asmordhau_character (Utilities|Casting|CastToMordhauCharacter DamageCauser))
  (bind _asattack_motion (Utilities|Casting|CastToAttackMotion (Variables|/Script/Mordhau.MordhauCharacter|GetMotion _asmordhau_character)))
  (if (or (Utilities|Enum|Equal(Enum) (Variables|/Script/Mordhau.AttackMotion|GetMove _asattack_motion) "RightStrike") (Utilities|Enum|Equal(Enum) (Variables|/Script/Mordhau.AttackMotion|GetMove _asattack_motion) "LeftStrike"))
    (if (== (Utilities|GetClass (Variables|/Script/Mordhau.AttackMotion|GetWeapon _asattack_motion)) "/Game/Mordhau/Blueprints/Equipment/Weapons/Specific/Makeshift/BP_Pickaxe.BP_Pickaxe_C")
      (bind _output_get (Variables|Default|SetTotalHits (+ (Variables|Default|GetTotalHits) 1)))
      (if (>= _output_get 1)
        (CallFunction|ProduceItem "/Game/Mordhau/Blueprints/Equipment/Ranged/BP_SteelIngot.BP_SteelIngot_C")
        (Variables|Default|SetTotalHits 0)))))

(fn ConstructionScript
  (|CallParentFunction))

(fn ProduceItem
  (params (Type :type Mordhau%20Equipment%20Class%20Reference))
  (bind _returnvalue (Game|SpawnActorfromClass Type (Transformation|GetWorldTransform (Variables|Default|GetSpawnPoint)) "Undefined" 0 0))
  (Utilities|IsValid _returnvalue
    (:Is%20Valid
      (Class|MordhauEquipment|AssignCustomization _returnvalue (Utilities|Struct|MakeEquipmentCustomization 0 (Utilities|Array|MakeArray 0 0 0) (Utilities|Array|MakeArray 0 0 0))))))