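; Deployable spike wall that hurts characters and horses running into it and impales those it kills.
; On server hits, damage scales with speed into the wall, drops during certain combat motions, and is capped for planter friendlies; survivors are knocked back.
; Cosmetic kill handling ragdolls the victim and pins a spine or neck bone to the impale point with a physics handle.
; Low health disables box collision.
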(event OnComponentHit(Box)
  (params (HitComponent :type Primitive%20Component%20Object%20Reference) (OtherActor :type Actor%20Object%20Reference) (OtherComp :type Primitive%20Component%20Object%20Reference) (NormalImpulse :type Vector :default "0, 0, 0") (Hit :type Hit%20Result%20Structure%20%28by%20ref%29))
  (Networking|SwitchHasAuthority
    (:Authority
      (if (>= (Variables|Default|GetReplicatedHealth) (Variables|Default|GetMinHealthToActivate))
        (bind _asadvanced_character (Utilities|Casting|CastToAdvancedCharacter OtherActor))
        (bind _asadvanced_character_movement (Utilities|Casting|CastToAdvancedCharacterMovement (Pawn|GetMovementComponent _asadvanced_character)))
        (if (not (Class|AdvancedCharacter|GetIsDead _asadvanced_character))
          (bind _asmordhau_character (Utilities|Casting|CastToMordhauCharacter _asadvanced_character)
            (:then
              (Utilities|Casting|CastToBlockedMotion (Variables|/Script/Mordhau.MordhauCharacter|GetMotion _asmordhau_character)
                (:then
                  (CallFunction|HandleCollision _asadvanced_character (* (.X (Math|Vector|BreakVector (Math|Vector|UnrotateVector (Variables|/Script/Mordhau.AdvancedCharacterMovement|GetPreviousVelocity _asadvanced_character_movement) (Transformation|GetWorldRotation (Variables|Default|GetBox))))) -1.0) 0.05 :!label _label))
                (:CastFailed
                  (Utilities|Casting|CastToAttackMotion (Variables|/Script/Mordhau.MordhauCharacter|GetMotion _asmordhau_character)
                    (:then
                      (goto _label))
                    (:CastFailed
                      (Utilities|Casting|CastToParryMotion (Variables|/Script/Mordhau.MordhauCharacter|GetMotion _asmordhau_character)
                        (:then
                          (goto _label))
                        (:CastFailed
                          (Utilities|Casting|CastToDisarmedMotion (Variables|/Script/Mordhau.MordhauCharacter|GetMotion _asmordhau_character)
                            (:then
                              (goto _label))
                            (:CastFailed
                              (CallFunction|HandleCollision _asadvanced_character (* (.X (Math|Vector|BreakVector (Math|Vector|UnrotateVector (Variables|/Script/Mordhau.AdvancedCharacterMovement|GetPreviousVelocity _asadvanced_character_movement) (Transformation|GetWorldRotation (Variables|Default|GetBox))))) -1.0) 1.0))))))))))
            (:CastFailed
              (Utilities|Casting|CastToHorse _asadvanced_character)
              (CallFunction|HandleCollision _asadvanced_character (* (.X (Math|Vector|BreakVector (Math|Vector|UnrotateVector (Variables|/Script/Mordhau.AdvancedCharacterMovement|GetPreviousVelocity _asadvanced_character_movement) (Transformation|GetWorldRotation (Variables|Default|GetBox))))) -1.0) (Variables|Default|GetHorseDamageFactor)))))))))

(event EventBeginPlay
  (|CallParentFunction) ; This node is disabled and will not be called.\nDrag off pins to build functionality.
)

(event Collision|EventActorBeginOverlap
  (params (OtherActor :type Actor%20Object%20Reference))
  (|CallParentFunction OtherActor) ; This node is disabled and will not be called.\nDrag off pins to build functionality.
)

(event EventTick
  (params (DeltaSeconds :type Float%20%28single-precision%29))
  (|CallParentFunction DeltaSeconds) ; This node is disabled and will not be called.\nDrag off pins to build functionality.
)

(event EventOnUsedtoKillOther
  (params (Character :type Advanced%20Character%20Object%20Reference) (Type :type EMordhauDamageType%20Enum :default "Generic") (SubType :type Byte :default 0) (bone :type Name%20%28by%20ref%29 :default "None") (Point :type Vector%20%28by%20ref%29 :default "0, 0, 0") (Source :type Actor%20Object%20Reference))
  (Networking|CanExecuteCosmeticEvents
    (:True
      (Utilities|IsValid Character
        (:Is%20Valid
          (CallFunction|Impale Character))))))

(event EventOnReplicatedHealthChanged
  (bind _box (Variables|Default|GetBox))
  (Utilities|FlowControl|Sequence
    (:then_0
      (if (<= (Variables|Default|GetReplicatedHealth) 20)
        (if (!= (Collision|GetCollisionEnabled _box) (Utilities|Enum|LiteralenumECollisionEnabled "NoCollision"))
          (Collision|SetCollisionEnabled _box "NoCollision"))
        (elif (!= (Collision|GetCollisionEnabled _box) (Utilities|Enum|LiteralenumECollisionEnabled "QueryAndPhysics"))
          (Collision|SetCollisionEnabled _box "QueryAndPhysics"))))
    (:then_1
      (|CallParentFunction))))

(fn ConstructionScript
  (|CallParentFunction))

(fn Impale
  (params (Character :type Advanced%20Character%20Object%20Reference))
  (bind _physicshandle (Variables|Default|GetPhysicsHandle))
  (bind _impalementsound (Variables|Default|GetImpalementSound))
  (bind _mesh (Variables|/Script/Engine.Character|GetMesh Character))
  (if (>= (Variables|Default|GetReplicatedHealth) (Variables|Default|GetMinHealthToActivate))
    (Utilities|FlowControl|Sequence
      (:then_0
        (Utilities|Casting|CastToMordhauCharacter Character
          (:then
            (LocalVariables|SetBoneToSticky "Spine1"))
          (:CastFailed
            (Utilities|Casting|CastToHorse Character
              (:then
                (LocalVariables|SetBoneToSticky "Neck2"))
              (:CastFailed
                (return))))))
      (:then_1
        (Physics|Components|PhysicsHandle|ReleaseComponent _physicshandle)
        (Class|AdvancedCharacter|StartRagdoll Character)
        (Physics|Components|PhysicsHandle|GrabComponentatLocationwithRotation _physicshandle _mesh (LocalVariables|GetBoneToSticky) (Transformation|GetSocketLocation _mesh (LocalVariables|GetBoneToSticky)) (Transformation|GetSocketRotation _mesh (LocalVariables|GetBoneToSticky)))
        (Physics|Components|PhysicsHandle|SetTargetLocation _physicshandle (Transformation|GetWorldLocation (Variables|Default|GetImpalePoint))))
      (:then_2
        (Utilities|IsValid _impalementsound
          (:Is%20Valid
            (Audio|PlaySoundatLocation _impalementsound (Transformation|GetWorldLocation (Variables|Default|GetImpalePoint)) "0, 0, 0" 1.0 1.0 0.0 0 0 0)))))))

(fn HandleCollision
  (params (Char :type Advanced%20Character%20Object%20Reference) (Velocity :type Float%20%28single-precision%29) (DamageFactor :type Float%20%28single-precision%29))
  (bind _plantercontroller (Variables|Default|GetPlanterController))
  (if (Variables|/Script/Mordhau.AdvancedCharacter|GetbIsRagdollFalling Char)
    (LocalVariables|SetDamageToDeal 1e+03)
    (else
      (LocalVariables|SetDamageToDeal (* (- Velocity (Variables|Default|GetMinVelocityToTrigger)) (Variables|Default|GetVelocityDamageFactor) DamageFactor))))
  (if (> (LocalVariables|GetDamageToDeal) 1.0)
    (Utilities|FlowControl|Sequence
      (:then_0
        (bind _asmordhau_character (Utilities|Casting|CastToMordhauCharacter Char))
        (bind _asmordhau_game_state (Utilities|Casting|CastToMordhauGameState (Game|GetGameState)))
        (bind _returnvalue (Class|MordhauCharacter|FindBestKiller _asmordhau_character 0.5))
        (Utilities|IsValid _returnvalue
          (:Is%20Not%20Valid
            (Utilities|IsValid _plantercontroller
              (:Is%20Valid
                (bind _returnvalue_2 (Class|MordhauGameState|IsFriendly _asmordhau_game_state _asmordhau_character _plantercontroller))
                (if _returnvalue_2
                  (LocalVariables|SetFriendly true)
                  (else
                    (LocalVariables|SetInstigatorController _plantercontroller))))))))
      (:then_1
        (if (LocalVariables|GetFriendly)
          (LocalVariables|SetDamageToDeal (Math|Float|Min(Float) (LocalVariables|GetDamageToDeal) 25.0))))
      (:then_2
        (Class|AdvancedCharacter|MordhauTakeDamage Char (LocalVariables|GetDamageToDeal) (Collision|MakeHitResult false false 0.0 0.0 "0, 0, 0" "0, 0, 0" "0,0,1" "0,0,1" 0 0) "Generic" 0 Char self (LocalVariables|GetInstigatorController))
        (if (not (Class|AdvancedCharacter|GetIsDead Char))
          (Class|AdvancedCharacter|Knockback Char (* (Transformation|GetActorForwardVector) 8e+02)))))))