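; Interactable swinging door that opens away or toward either side, closes on use, and can be kicked open or shut at high speed.
; A DoorState RepNotify sets target yaw and speed, then enables Tick to interpolate rotation until done.
; While moving, the server damages overlapped world-static Mordhau actors other than doors.
; Blocking characters make it close or get pushed; fast swings ragdoll and knock back those mid-attack, blocked or feinting, sparing the kicker.
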(event EventBeginPlay
  (|CallParentFunction)
  (Variables|Default|SetHasBegunPlay true))

(event Collision|EventActorBeginOverlap
  (params (OtherActor :type Actor%20Object%20Reference))
  (|CallParentFunction OtherActor) ; This node is disabled and will not be called.\nDrag off pins to build functionality.
)

(event Game|Damage|EventAnyDamage
  (params (Damage :type Float%20%28single-precision%29) (DamageType :type Damage%20Type%20Object%20Reference) (InstigatedBy :type Controller%20Object%20Reference) (DamageCauser :type Actor%20Object%20Reference))
  (if (Variables|Default|GetCanBeKickedOpen)
    (bind _asmordhau_character (Utilities|Casting|CastToMordhauCharacter DamageCauser)
      (:then
        (bind _asattack_motion (Utilities|Casting|CastToAttackMotion (Variables|/Script/Mordhau.MordhauCharacter|GetMotion _asmordhau_character))
          (:then
            (if (Utilities|Enum|Equal(Enum) (Variables|/Script/Mordhau.AttackMotion|GetMove _asattack_motion) "Kick")
              (bind _angledegrees (CallFunction|GetDoortoActorAngle _asmordhau_character))
              (if (>= _angledegrees 9e+01)
                (if (>= _angledegrees 1.2e+02)
                  (if (and (!= (Variables|Default|GetDoorState) 2) (!= (Variables|Default|GetDoorState) 1))
                    (if (or (== (Variables|Default|GetDoorState) 0) (== (Variables|Default|GetDoorState) 5))
                      (if (Variables|Default|GetCanOpenForwards)
                        (Variables|Default|SetDoorState 2)
                        (Variables|Default|SetKicker _asmordhau_character :!label _label)
                        (else
                          (|CallParentFunction Damage DamageType InstigatedBy DamageCauser :!label _label_2)))
                      (else
                        (Variables|Default|SetDoorState 5)
                        (goto _label)))
                    (else
                      (goto _label_2)))
                  (else
                    (goto _label_2)))
                (elif (<= _angledegrees 6e+01)
                  (if (and (!= (Variables|Default|GetDoorState) 4) (!= (Variables|Default|GetDoorState) 3))
                    (if (or (== (Variables|Default|GetDoorState) 0) (== (Variables|Default|GetDoorState) 5))
                      (if (Variables|Default|GetCanOpenBackwards)
                        (Variables|Default|SetDoorState 4)
                        (goto _label)
                        (else
                          (goto _label_2)))
                      (else
                        (Variables|Default|SetDoorState 5)
                        (goto _label)))
                    (else
                      (goto _label_2)))
                  (else
                    (goto _label_2))))
              (else
                (goto _label_2))))
          (:CastFailed
            (goto _label_2))))
      (:CastFailed
        (goto _label_2)))
    (else
      (goto _label_2))))

(event EventOnInteractionStart
  (params (Character :type Mordhau%20Character%20Object%20Reference))
  (bind _angledegrees (CallFunction|GetDoortoActorAngle Character))
  (if (and (!= (Variables|Default|GetDoorState) 0) (!= (Variables|Default|GetDoorState) 5))
    (Variables|Default|SetDoorState 0)
    (elif (and (or (>= _angledegrees 9e+01) (not (Variables|Default|GetCanOpenBackwards))) (Variables|Default|GetCanOpenForwards))
      (if (and (!= (Variables|Default|GetDoorState) 1) (!= (Variables|Default|GetDoorState) 2))
        (Variables|Default|SetDoorState 1))
      (elif (Math|Boolean|ANDBoolean (!= (Variables|Default|GetDoorState) 3) (!= (Variables|Default|GetDoorState) 4) (Variables|Default|GetCanOpenBackwards))
        (Variables|Default|SetDoorState 3)))))

(event EventTick
  (params (DeltaSeconds :type Float%20%28single-precision%29))
  (bind _staticmesh (Variables|Default|GetStaticMesh))
  (bind _audio (Variables|Default|GetAudio))
  (bind _audio_2 (Variables|Default|GetAudio))
  (bind _staticmesh_2 (Variables|Default|GetStaticMesh))
  (bind _closesound (Variables|Default|GetCloseSound))
  (bind _fastopenstopsound (Variables|Default|GetFastOpenStopSound))
  (bind _returnvalue (Transformation|GetWorldTransform _staticmesh_2))
  (|CallParentFunction DeltaSeconds)
  (if (Math|Float|NearlyEqual(Float) (Variables|Default|GetSmoothedDoorRotation) (Variables|Default|GetSmoothedDoorRotationTarget) 1e-06)
    (bind _output_get (Variables|Default|SetLastCompletedDoorState (Variables|Default|GetDoorState)))
    (Actor|Tick|SetActorTickEnabled false)
    (Utilities|FlowControl|Sequence
      (:then_0
        (Networking|SwitchHasAuthority
          (:Authority
            (bind _outactors (Collision|ComponentOverlapActors _staticmesh (Transformation|GetWorldTransform _staticmesh) (Variables|Default|GetObjectsThatPreventMovement) "/Script/Mordhau.AdvancedCharacter"))
            (for _array_element _outactors
              (bind _asmordhau_character (Utilities|Casting|CastToMordhauCharacter _array_element)
                (:then
                  (Utilities|IsValid (Variables|/Script/Mordhau.MordhauCharacter|GetCurrentVehicle _asmordhau_character)
                    (:Is%20Not%20Valid
                      _)))
                (:CastFailed
                  _))
              (bind _asadvanced_character (Utilities|Casting|CastToAdvancedCharacter _array_element))
              (Transformation|Teleport _asadvanced_character (Transformation|GetActorLocation _asadvanced_character) (Transformation|GetActorRotation _asadvanced_character))))))
      (:then_1
        (Networking|CanExecuteCosmeticEvents
          (:True
            (switch int (Math|Conversions|ToInteger(Byte) _output_get)
              (:0
                (Utilities|IsValid _closesound :!label _label
                  (:Is%20Valid
                    (Audio|Components|Audio|SetSound _audio_2 _closesound)
                    (Audio|Components|Audio|Play _audio_2 0.0))))
              (:2
                (Utilities|IsValid _fastopenstopsound :!label _label_2
                  (:Is%20Valid
                    (Audio|Components|Audio|SetSound _audio _fastopenstopsound)
                    (Audio|Components|Audio|Play _audio 0.0))))
              (:4
                (goto _label_2))
              (:5
                (goto _label)))))))
    (else
      (bind _output_get_2 (Variables|Default|SetSmoothedDoorRotation (Math|Interpolation|FInterptoConstant (Variables|Default|GetSmoothedDoorRotation) (Variables|Default|GetSmoothedDoorRotationTarget) DeltaSeconds (Variables|Default|GetSmoothedDoorRotationSpeed))))
      (Transformation|SetRelativeRotation (Variables|Default|GetStaticMesh) (Math|Rotator|MakeRotator 0.0 0.0 _output_get_2) false false)
      (Networking|SwitchHasAuthority
        (:Authority
          (Utilities|FlowControl|Sequence
            (:then_0
              (bind _outactors_2 (Collision|ComponentOverlapActors _staticmesh_2 _returnvalue (Utilities|Array|MakeArray "ObjectTypeQuery1") "/Script/Mordhau.MordhauActor" (Utilities|Array|MakeArray self)))
              (bind _array_element_2 (Utilities|Array|ForEachLoopwithBreak _outactors_2)
                (:LoopBody
                  (Utilities|Casting|CastToBP_Door _array_element_2
                    (:CastFailed
                      (Game|Damage|ApplyDamage 0 1e+03 0 0))))))
            (:then_1
              (bind (_outactors_3 _returnvalue_2) (Collision|ComponentOverlapActors _staticmesh_2 _returnvalue (Variables|Default|GetObjectsThatPreventMovement) "/Script/Mordhau.AdvancedCharacter"))
              (if _returnvalue_2
                (if (Math|Boolean|ORBoolean (== (Variables|Default|GetDoorState) 2) (== (Variables|Default|GetDoorState) 4) (== (Variables|Default|GetDoorState) 5))
                  (for _array_element_3 _outactors_3
                    (bind _asmordhau_character_2 (Utilities|Casting|CastToMordhauCharacter _array_element_3)
                      (:then
                        (if (not (== _asmordhau_character_2 (Variables|Default|GetKicker)))
                          (Utilities|IsValid (Variables|/Script/Mordhau.MordhauCharacter|GetCurrentVehicle _asmordhau_character_2)
                            (:Is%20Valid
                              (if (!= (Variables|Default|GetDoorState) 0) :!label _label_3
                                (Variables|Default|SetDoorState 0)))
                            (:Is%20Not%20Valid
                              (bind _asmordhau_movement_component (Utilities|Casting|CastToMordhauMovementComponent (Pawn|GetMovementComponent _asmordhau_character_2))
                                (:then
                                  (if (not (stale _returnvalue))
                                    (if (not (Variables|/Script/Mordhau.AdvancedCharacter|GetbIsRagdollFalling _asmordhau_character_2))
                                      (Utilities|Casting|CastToAttackMotion (Variables|/Script/Mordhau.MordhauCharacter|GetMotion _asmordhau_character_2)
                                        (:then
                                          _)
                                        (:CastFailed
                                          (Utilities|Casting|CastToBlockedMotion (Variables|/Script/Mordhau.MordhauCharacter|GetMotion _asmordhau_character_2)
                                            (:then
                                              _)
                                            (:CastFailed
                                              (Utilities|Casting|CastToFeintedMotion (Variables|/Script/Mordhau.MordhauCharacter|GetMotion _asmordhau_character_2)
                                                (:then
                                                  _)
                                                (:CastFailed
                                                  (goto _label_3)))))))
                                      (Class|AdvancedCharacter|SetIsRagdollFalling _asmordhau_character_2 true)
                                      (Class|AdvancedCharacter|Knockback _asmordhau_character_2 (* (Math|Conversions|ToVector(Vector2D) (Math|Vector2D|Normalize2D (Math|Conversions|ToVector2D(Vector) (- (Transformation|GetActorLocation _asmordhau_character_2) (Transformation|GetWorldLocation (Variables|Default|GetDamageParticleTransform)))))) 1.1e+03)))))
                                (:CastFailed
                                  (goto _label_3)))))))
                      (:CastFailed
                        (goto _label_3))))
                  (elif (!= (Variables|Default|GetDoorState) 0)
                    (Variables|Default|SetDoorState 0)
                    (else
                      (for _array_element_4 _outactors_3
                        (bind _asmordhau_character_3 (Utilities|Casting|CastToMordhauCharacter _array_element_4))
                        (Utilities|IsValid (Variables|/Script/Mordhau.MordhauCharacter|GetCurrentVehicle _asmordhau_character_3)
                          (:Is%20Not%20Valid
                            (Class|AdvancedCharacter|Knockback _asmordhau_character_3 (* (* (Math|Conversions|ToVector(Vector2D) (Math|Vector2D|Normalize2D (Math|Conversions|ToVector2D(Vector) (- (Transformation|GetActorLocation _array_element_4) (Transformation|GetWorldLocation (Variables|Default|GetDamageParticleTransform)))))) 4e+03) (Utilities|Time|GetWorldDeltaSeconds)))))))))))))))))

(fn ConstructionScript
  (|CallParentFunction)
  (Utilities|FlowControl|Sequence
    (:then_0
      (switch int (Math|Conversions|ToInteger(Byte) (Variables|Default|GetStartingState))
        (:0
          (Variables|Default|SetDoorState 0)
          (bind _output_get (Variables|Default|SetSmoothedDoorRotation (Variables|Default|GetDoorYawClosed)))
          (Variables|Default|SetSmoothedDoorRotationTarget _output_get))
        (:1
          (Variables|Default|SetDoorState 1)
          (bind _output_get_2 (Variables|Default|SetSmoothedDoorRotation (Variables|Default|GetDoorYawOpenForward)))
          (Variables|Default|SetSmoothedDoorRotationTarget _output_get_2))
        (:2
          (Variables|Default|SetDoorState 3)
          (bind _output_get_3 (Variables|Default|SetSmoothedDoorRotation (Variables|Default|GetDoorYawOpenBackward)))
          (Variables|Default|SetSmoothedDoorRotationTarget _output_get_3))))
    (:then_1
      (Variables|Default|SetLastCompletedDoorState (Variables|Default|GetDoorState))
      (Transformation|SetRelativeRotation (Variables|Default|GetStaticMesh) (Math|Rotator|MakeRotator 0.0 0.0 (Variables|Default|GetSmoothedDoorRotation)) false false))))

(fn OnRepDoorState
  (bind _usesound (Variables|Default|GetUseSound))
  (bind _audio (Variables|Default|GetAudio))
  (bind _dooryawopenforward (Variables|Default|GetDoorYawOpenForward))
  (bind _dooryawopenbackward (Variables|Default|GetDoorYawOpenBackward))
  ;[1 1 1] DoorState
  ; 0 = closed
  ; 1 = open forward (slow)
  ; 2 = open forward (fast)
  ; 3 = open backward (slow)
  ; 4 = open backward (fast)
  (Networking|ForceNetUpdate)
  (Actor|Tick|SetActorTickEnabled true)
  (switch int (Math|Conversions|ToInteger(Byte) (Variables|Default|GetDoorState))
    (:0
      (Variables|Default|SetSmoothedDoorRotationTarget (Variables|Default|GetDoorYawClosed))
      (Variables|Default|SetSmoothedDoorRotationSpeed (Variables|Default|GetDoorCloseSpeed))
      (Networking|CanExecuteCosmeticEvents :!label _label
        (:True
          (if (Variables|Default|GetHasBegunPlay)
            (Utilities|IsValid _usesound
              (:Is%20Valid
                (Audio|Components|Audio|SetSound _audio _usesound)
                (Audio|Components|Audio|Play _audio 0.0)))))))
    (:1
      (Variables|Default|SetSmoothedDoorRotationTarget _dooryawopenforward)
      (Variables|Default|SetSmoothedDoorRotationSpeed (Variables|Default|GetDoorOpenSpeed))
      (goto _label))
    (:2
      (Variables|Default|SetSmoothedDoorRotationTarget _dooryawopenforward)
      (Variables|Default|SetSmoothedDoorRotationSpeed (Variables|Default|GetDoorOpenSpeedFast) :!label _label_2)
      (Variables|Default|SetFastOpenStart (Utilities|Time|GetGameTimeinSeconds)))
    (:3
      (Variables|Default|SetSmoothedDoorRotationTarget _dooryawopenbackward)
      (Variables|Default|SetSmoothedDoorRotationSpeed (Variables|Default|GetDoorOpenSpeed))
      (goto _label))
    (:4
      (Variables|Default|SetSmoothedDoorRotationTarget _dooryawopenbackward)
      (goto _label_2))
    (:5
      (Variables|Default|SetSmoothedDoorRotationTarget (Variables|Default|GetDoorYawClosed))
      (goto _label_2))))

(fn GetDoorForwardVector
  (return (Math|Vector|GetForwardVector (Math|Rotator|CombineRotators (Transformation|GetActorRotation) (Math|Rotator|Delta(Rotator) (Variables|/Script/Engine.SceneComponent|GetRelativeRotation (Variables|Default|GetStaticMesh)) (Math|Rotator|MakeRotator 0.0 0.0 (Variables|Default|GetDoorYawClosed)))))))

(fn GetDoortoActorAngle
  (params (Actor :type Actor%20Object%20Reference))
  (bind _out (CallFunction|GetDoorForwardVector))
  (return (Class|KismetMathLibrary|DegAcos (Math|Vector|DotProduct _out (Transformation|GetActorForwardVector Actor)))))