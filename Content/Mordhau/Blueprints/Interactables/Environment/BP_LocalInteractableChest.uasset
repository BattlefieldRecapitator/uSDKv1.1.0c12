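; Local interactable chest that visually and audibly reflects whether its contents are depleted or refilled.
; Overrides the parent's Refilled and Depleted events to play an open or interact sound respectively, then run the parent logic.
; Both events share one update that shows the contents mesh and sets the AB_Chest animation Blueprint's Opened flag only while not depleted.
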(event EventBeginPlay)

(event Collision|EventActorBeginOverlap
  (params (OtherActor :type Actor%20Object%20Reference)))

(event EventTick
  (params (DeltaSeconds :type Float%20%28single-precision%29)))

(event EventRefilled
  (bind _isdepleted (Variables|Default|GetIsDepleted))
  (bind _audio (Variables|Default|GetAudio))
  (bind _returnvalue (not _isdepleted))
  (Utilities|FlowControl|Sequence
    (:then_0
      (Audio|Components|Audio|SetSound _audio "/Game/Mordhau/Audio/Cues/Misc/SC_Chest_Open.SC_Chest_Open")
      (Audio|Components|Audio|Play _audio 0.0))
    (:then_1
      (Rendering|SetVisibility (Variables|Default|GetContentsMesh) _returnvalue false)
      (bind _asab_chest (Utilities|Casting|CastToAB_Chest (Components|SkeletalMesh|GetAnimInstance (Variables|Default|GetBoxMesh))))
      (Variables|/Game/Mordhau/Animations/Blueprints/AB_Chest.AB_Chest_C|SetOpened _asab_chest _returnvalue))
    (:then_2
      (|CallParentFunction))))

(event EventDepleted
  (bind _isdepleted (Variables|Default|GetIsDepleted))
  (bind _audio (Variables|Default|GetAudio))
  (bind _returnvalue (not _isdepleted))
  (Utilities|FlowControl|Sequence
    (:then_0
      (Audio|Components|Audio|SetSound _audio "/Game/Mordhau/Audio/Cues/Misc/SC_Chest_Interact.SC_Chest_Interact")
      (Audio|Components|Audio|Play _audio 0.0))
    (:then_1
      (Rendering|SetVisibility (Variables|Default|GetContentsMesh) _returnvalue false)
      (bind _asab_chest (Utilities|Casting|CastToAB_Chest (Components|SkeletalMesh|GetAnimInstance (Variables|Default|GetBoxMesh))))
      (Variables|/Game/Mordhau/Animations/Blueprints/AB_Chest.AB_Chest_C|SetOpened _asab_chest _returnvalue))
    (:then_2
      (|CallParentFunction))))

(fn ConstructionScript
  (|CallParentFunction))