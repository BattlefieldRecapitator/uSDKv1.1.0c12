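; BP_ProjectileTrap is an environment trap that is itself a projectile, fired when triggered and optionally by taking damage.
; If ActivateOnDamage is set and it has not yet fired, damage calls TriggerTrap with the instigating controller.
; TriggerTrap initializes the projectile for that controller without local prediction, then calls Fire.
; Fire destroys the trigger collision and switches the collision component to the Projectile profile before running the parent's firing logic.
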(event EventFire
  (Components|DestroyComponent (Variables|Default|GetTriggerCollision))
  (Collision|SetCollisionProfileName (Variables|Default|GetCollisionComp) "Projectile" :!class /Script/Engine.PrimitiveComponent)
  (|CallParentFunction))

(event EventTick
  (params (DeltaSeconds :type Float%20%28single-precision%29)))

(event Game|Damage|EventAnyDamage
  (params (Damage :type Float%20%28single-precision%29) (DamageType :type Damage%20Type%20Object%20Reference) (InstigatedBy :type Controller%20Object%20Reference) (DamageCauser :type Actor%20Object%20Reference))
  (if (and (Variables|Default|GetActivateOnDamage) (not (Variables|Default|GetbHasFired)))
    (CallFunction|TriggerTrap InstigatedBy)))

(fn ConstructionScript)

(fn TriggerTrap
  (params (InInstigatorController :type Controller%20Object%20Reference))
  (Class|MordhauProjectile|InitializeProjectile InInstigatorController false)
  (Class|MordhauProjectile|Fire))