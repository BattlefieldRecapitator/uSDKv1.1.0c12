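; Siege basket interactable that gives visual and audio feedback as its contents are depleted and refilled.
; Both events set the contents mesh's visibility from IsDepleted, swap and play a chest sound, then call the parent implementation.
; The depletion sound is skipped during the first few seconds of game time.
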(event EventBeginPlay)

(event Collision|EventActorBeginOverlap
  (params (OtherActor :type Actor%20Object%20Reference)))

(event EventTick
  (params (DeltaSeconds :type Float%20%28single-precision%29)))

(event EventRefilled
  (bind _audio (Variables|Default|GetAudio))
  (Utilities|FlowControl|Sequence
    (:then_0
      (Audio|Components|Audio|SetSound _audio "/Game/Mordhau/Audio/Cues/Misc/SC_Chest_Open.SC_Chest_Open")
      (Audio|Components|Audio|Play _audio 0.0))
    (:then_1
      (Rendering|SetVisibility (Variables|Default|GetContentsMesh) (not (Variables|Default|GetIsDepleted)) false))
    (:then_2
      (|CallParentFunction))))

(event EventDepleted
  (bind _audio (Variables|Default|GetAudio))
  (Utilities|FlowControl|Sequence
    (:then_0
      (if (> (Utilities|Time|GetTimeSeconds) 3.0)
        (Audio|Components|Audio|SetSound _audio "/Game/Mordhau/Audio/Cues/Misc/SC_Chest_Interact.SC_Chest_Interact")
        (Audio|Components|Audio|Play _audio 0.0)))
    (:then_1
      (Rendering|SetVisibility (Variables|Default|GetContentsMesh) (not (Variables|Default|GetIsDepleted)) false))
    (:then_2
      (|CallParentFunction))))

(fn ConstructionScript
  (|CallParentFunction))