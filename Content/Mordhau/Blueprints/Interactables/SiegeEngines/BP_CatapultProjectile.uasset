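; Projectile launched by the catapult siege engine, with launch speed based on how far the arm is drawn.
; On fire, it casts its creator to BP_Catapult and scales InitialSpeed by the replicated arm value before running the parent fire logic.
; On hit, it plays a distance-attenuated world camera shake, then defers to the parent hit handling.
; The radial damage call here is disconnected, leaving the authority branch without effect.
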(event EventTick
  (params (DeltaSeconds :type Float%20%28single-precision%29)))

(event EventFire
  (bind _projectilemovement (Variables|Default|GetProjectileMovement))
  (Utilities|FlowControl|Sequence
    (:then_0
      (bind _returnvalue (Class|MordhauProjectile|GetProjectileCreator))
      (bind _asbp_catapult (Utilities|Casting|CastToBP_Catapult _returnvalue))
      (Variables|/Script/Engine.ProjectileMovementComponent|SetInitialSpeed _projectilemovement (* (Variables|/Script/Engine.ProjectileMovementComponent|GetInitialSpeed _projectilemovement) (+ 5.0 (* (/ (Math|Conversions|ToFloat(Byte) (Variables|/Game/Mordhau/Blueprints/Interactables/SiegeEngines/BP_Catapult.BP_Catapult_C|GetReplicatedArm _asbp_catapult)) 1e+02) 5.0)))))
    (:then_1
      (|CallParentFunction))))

(event EventOnProjectileHit
  (params (HitLocation :type Vector%20%28by%20ref%29 :default "0, 0, 0") (HitNormal :type Vector%20%28by%20ref%29 :default "0, 0, 0") (BounceForce :type Float%20%28single-precision%29) (Surface :type Byte :default 0) (bHasHitWorld :type Boolean) (bHasStopped :type Boolean))
  (Utilities|FlowControl|Sequence
    (:then_0
      (Camera|PlayWorldCameraShake 0 HitLocation 2.5e+02 7.5e+03 1e+01))
    (:then_1
      (Networking|SwitchHasAuthority
        (:Authority
          (bind _returnvalue (Class|MordhauProjectile|GetProjectileOwningController)))))
    (:then_2
      (|CallParentFunction HitLocation HitNormal BounceForce Surface bHasHitWorld bHasStopped))))

(fn ConstructionScript
  (|CallParentFunction))