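; BP_CatapultSpawner is a server-authoritative spawner that places a catapult at its location on BeginPlay and respawns it after it dies.
; It spawns the catapult far below the world origin, then teleports it into place, using teleport failure as a blocked-space check.
; Failed placements are destroyed and retried after random delays.
; Respawn delay comes from the Mordhau game mode; death is only tracked when that delay is positive.
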(event Custom|OnCatapultDied
  (params (Character :type Advanced%20Character%20Object%20Reference))
  (Utilities|FlowControl|Delay (Variables|CatapultSpawner|GetRespawnTime))
  (CallFunction|Spawn))

(event Custom|Spawn
  (Networking|SwitchHasAuthority
    (:Authority
      (bind _returnvalue (Game|SpawnActorfromClass "/Game/Mordhau/Blueprints/Interactables/SiegeEngines/BP_Catapult.BP_Catapult_C" (Math|Transform|MakeTransform "0, 0,-3000.000000" "0, 0, 0" "1,1,1") "AlwaysSpawn" 0 0))
      (Utilities|FlowControl|Delay (Math|Random|RandomFloatinRange 0.0 0.1))
      (bind _returnvalue_2 (Transformation|Teleport _returnvalue (Transformation|GetActorLocation) (Transformation|GetActorRotation)))
      (if _returnvalue_2
        (if (> (Variables|CatapultSpawner|GetRespawnTime) 0.0)
          (EventDispatchers|AssignOnCharacterDied _returnvalue (delegate Custom|OnCatapultDied)))
        (else
          (Utilities|FlowControl|Delay (Math|Random|RandomFloatinRange 0.1 0.5)) ; Not enough space; destroy actor and retry
          (Actor|DestroyActor _returnvalue)
          (Utilities|FlowControl|Delay (Math|Random|RandomFloatinRange 1.0 3.0))
          (CallFunction|Spawn))))))

(event EventBeginPlay
  (Networking|SwitchHasAuthority
    (:Authority
      (Utilities|FlowControl|Sequence
        (:then_0
          (bind _asmordhau_game_mode (Utilities|Casting|CastToMordhauGameMode (Game|GetGameMode)))
          (Variables|CatapultSpawner|SetRespawnTime (Variables|/Script/Mordhau.MordhauGameMode|GetCatapultRespawnTime _asmordhau_game_mode)))
        (:then_1
          (CallFunction|Spawn))))))

(fn ConstructionScript)