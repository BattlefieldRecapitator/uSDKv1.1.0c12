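; BP_ArcherCover is a drivable archer cover siege engine that can be destroyed.
; Input turns it and feeds secondary turn and look-up, which steer the driver's first-person camera, and lets the driver cycle cameras.
; Its mesh material is registered to dissolve, and cosmetic hits push the mesh with computed ragdoll forces.
; Death ragdolls it with an impact force and stops its nav obstacle affecting navigation.
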(event EventBeginPlay
  (bind _mesh (Variables|Character|GetMesh))
  (bind _returnvalue (Rendering|Material|CreateDynamicMaterialInstance _mesh 0 (Rendering|Material|GetMaterial _mesh 0) "None" :!class /Script/Engine.PrimitiveComponent))
  (Class|AdvancedCharacter|RegisterMaterialtoDissolve _returnvalue))

(event EventOnCosmeticHit
  (params (DamageType :type EMordhauDamageType%20Enum :default "Generic") (SubType :type Byte :default 0) (Hit :type Hit%20Result%20Structure%20%28by%20ref%29) (Agent :type Actor%20Object%20Reference))
  (bind (_bblockinghit _binitialoverlap _time _distance _location _impactpoint _normal _impactnormal _physmat _hitactor _hitcomponent _hitbonename) (Collision|BreakHitResult Hit))
  (bind _self self)
  (|CallParentFunction DamageType SubType Hit Agent)
  (Class|PrimitiveComponent|AddForceatLocation (Variables|Character|GetMesh) (* (CallFunction|ComputeRagdollForce Agent DamageType SubType 0 _self _self) 1e+02) _impactpoint _hitbonename))

(event EventOnDied
  (params (Angle :type Float%20%28single-precision%29) (Type :type EMordhauDamageType%20Enum :default "Generic") (SubType :type Byte :default 0) (bone :type Name%20%28by%20ref%29 :default "None") (Point :type Vector%20%28by%20ref%29 :default "0, 0, 0") (Source :type Actor%20Object%20Reference) (Agent :type Actor%20Object%20Reference))
  (bind _self self)
  (|CallParentFunction Angle Type SubType bone Point Source Agent)
  (Class|AdvancedCharacter|StartRagdoll)
  (Class|PrimitiveComponent|AddForceatLocation (Variables|Character|GetMesh) (* (CallFunction|ComputeRagdollForce Agent Type SubType 0 _self _self) 1e+02) Point bone)
  (Class|MordhauUtilityLibrary|SetCanEverAffectNavigation (Variables|Default|GetNavObstacle1) false))

(event EventUpdateFPCamerafor
  (params (Character :type Mordhau%20Character%20Object%20Reference) (DeltaSeconds :type Float%20%28single-precision%29) (bRotationOnly :type Boolean))
  (|CallParentFunction Character DeltaSeconds bRotationOnly)
  (Class|MordhauCharacter|UpdateFPCamera Character DeltaSeconds (Variables|Default|GetLookUpValue) bRotationOnly (Math|Rotator|MakeRotator 0.0 0.0 (Variables|Default|GetSecondaryTurnValue))))

(event Input|ActionEvents|InputActionFire
  (params (Key :type Key%20Structure)))

(event Input|ActionEvents|InputActionCycleCamera
  (params (Key :type Key%20Structure))
  (bind _driver (Variables|Default|GetDriver))
  (:Pressed
    (Utilities|IsValid _driver
      (:Is%20Valid
        (Class|MordhauCharacter|CycleCamera _driver)))))

(event Input|AxisEvents|InputAxisMoveRight
  (params (AxisValue :type Float%20%28single-precision%29))
  (Class|AdvancedCharacter|Turn AxisValue false))

(event Input|AxisEvents|InputAxisLookUp
  (params (AxisValue :type Float%20%28single-precision%29))
  (Class|AdvancedCharacter|LookUp AxisValue false))

(event Input|AxisEvents|InputAxisTurnRight
  (params (AxisValue :type Float%20%28single-precision%29))
  (Class|MordhauVehicle|SecondaryTurn AxisValue false))

(fn ConstructionScript
  (|CallParentFunction))