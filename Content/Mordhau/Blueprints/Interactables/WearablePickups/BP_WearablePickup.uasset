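; Interactable armor pickup that puts wearables on the character who interacts with it, then destroys itself.
; On authority it expires after a short lifespan unless the game mode disables equipment despawning.
; Equip uses the player's default customization for its slot and tier, falling back to its own Wearables, and merges these into the replicated profile.
; EquipIfUpgrade gates Battle Royale characters through IsAnUpgrade, which always returns true here.
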(event EventBeginPlay
  (Networking|SwitchHasAuthority
    (:Authority
      (bind _asbp_mordhau_game_mode (Utilities|Casting|CastToBP_MordhauGameMode (Game|GetGameMode)))
      (if (not (Variables|/Script/Mordhau.MordhauGameMode|GetbEquipmentDoesNotDespawn _asbp_mordhau_game_mode))
        (Actor|SetLifeSpan 2e+01)))))

(event Collision|EventActorBeginOverlap
  (params (OtherActor :type Actor%20Object%20Reference)))

(event EventOnInteractionStart
  (params (Character :type Mordhau%20Character%20Object%20Reference))
  (CallFunction|Equip Character))

(event EventTick
  (params (DeltaSeconds :type Float%20%28single-precision%29)))

(fn ConstructionScript
  (|CallParentFunction))

(fn AssigntoCharacter
  (params (Character :type Mordhau%20Character%20Object%20Reference) (CustomizatonReplicationActor :type Customization%20Replication%20Actor%20Object%20Reference))
  (bind _lastassignedprofile (Variables|/Script/Mordhau.CustomizationReplicationActor|GetLastAssignedProfile CustomizatonReplicationActor))
  (bind (_name _gearcustomization _appearancecustomization _facecustomization _skillscustomization) (Utilities|Struct|BreakCharacterProfile _lastassignedprofile))
  (bind (_wearables _equipment) (Utilities|Struct|BreakCharacterGearCustomization _gearcustomization))
  (bind _asmordhau_player_controller (Utilities|Casting|CastToMordhauPlayerController (Pawn|GetController Character))
    (:then
      (bind (_outmap _returnvalue) (Class|MordhauPlayerController|GetDefaultTierCustomizationforSlot _asmordhau_player_controller (Variables|Default|GetMainSlot) (Math|Conversions|ToByte(Integer) (Variables|Default|GetTier))))
      (if _returnvalue
        (LocalVariables|SetWearablesToUse _outmap)
        (else
          (LocalVariables|SetWearablesToUse (Variables|Default|GetWearables) :!label _label))))
    (:CastFailed
      (goto _label)))
  (bind _output_get (LocalVariables|SetNewWearables _wearables))
  (bind _keys (Utilities|Map|Keys (LocalVariables|GetWearablesToUse)))
  (for _array_element _keys
    (if (.ReturnValue (Utilities|Map|Find (LocalVariables|GetWearablesToUse) _array_element))
      (Utilities|Array|SetArrayElem _output_get (Math|Conversions|ToInteger(Byte) _array_element) (.Value (Utilities|Map|Find (LocalVariables|GetWearablesToUse) _array_element)))))
  (Class|CustomizationReplicationActor|AssignDatafromProfile CustomizatonReplicationActor (Utilities|Struct|MakeCharacterProfile _name (Utilities|Struct|MakeCharacterGearCustomization (LocalVariables|GetNewWearables) _equipment) _appearancecustomization _facecustomization _skillscustomization)))

(fn IsAnUpgrade
  (params (Char :type BP%20Battle%20Royale%20Character%20Object%20Reference))
  (return true))

(fn Equip
  (params (Char :type Mordhau%20Character%20Object%20Reference))
  (bind _returnvalue (Class|MordhauCharacter|GetCustomizationReplicationActor Char))
  (Utilities|IsValid _returnvalue
    (:Is%20Valid
      (if (Ability|HasAuthority _returnvalue)
        (CallFunction|AssigntoCharacter Char _returnvalue)
        (Actor|DestroyActor)))))

(fn EquipifUpgrade
  (params (Char :type Mordhau%20Character%20Object%20Reference))
  (bind _asbp_battle_royale_character (Utilities|Casting|CastToBP_BattleRoyaleCharacter Char)
    (:then
      (if (CallFunction|IsAnUpgrade _asbp_battle_royale_character)
        (CallFunction|Equip Char :!label _label)))
    (:CastFailed
      (goto _label))))